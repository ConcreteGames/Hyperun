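; BP_PaletteManager controls the game's color palette by writing parameters to the MPC_Palette Material Parameter Collection.
; RandomPalette gives Bike, Road and Background random RGB colors and picks a random HueShift.
; Two other functions add to or set the stored HueShift, wrap it with modulo 1, and push it to the collection.
; It has no active event logic, so palette changes depend on these functions being called.
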(event EventBeginPlay)

(event EventActorBeginOverlap
  (params (OtherActor :type Actor%20Object%20Reference)))

(event EventTick
  (params (DeltaSeconds :type Float%20%28single-precision%29)))

(fn ConstructionScript)

(fn RandomPalette
  (Rendering|Material|SetVectorParameterValue "/Game/Coco/MPC_Palette.MPC_Palette" "Bike" (Utilities|Struct|MakeLinearColor (Math|Random|RandomFloatinRange 0.0 1.0) (Math|Random|RandomFloatinRange 0.0 1.0) (Math|Random|RandomFloatinRange 0.0 1.0) 1.0) :!class /Script/Engine.KismetMaterialLibrary)
  (Rendering|Material|SetVectorParameterValue "/Game/Coco/MPC_Palette.MPC_Palette" "Road" (Utilities|Struct|MakeLinearColor (Math|Random|RandomFloatinRange 0.0 1.0) (Math|Random|RandomFloatinRange 0.0 1.0) (Math|Random|RandomFloatinRange 0.0 1.0) 1.0) :!class /Script/Engine.KismetMaterialLibrary)
  (Rendering|Material|SetVectorParameterValue "/Game/Coco/MPC_Palette.MPC_Palette" "Background" (Utilities|Struct|MakeLinearColor (Math|Random|RandomFloatinRange 0.0 1.0) (Math|Random|RandomFloatinRange 0.0 1.0) (Math|Random|RandomFloatinRange 0.0 1.0) 1.0) :!class /Script/Engine.KismetMaterialLibrary)
  (Variables|Default|SetHueShift (Math|Random|RandomFloatinRange 0.0 1.0))
  (Rendering|Material|SetScalarParameterValue "/Game/Coco/MPC_Palette.MPC_Palette" "HueShift" (Variables|Default|GetHueShift) :!class /Script/Engine.KismetMaterialLibrary))

(fn ChangePaletteAddHueShift
  (params (AddHueShift :type Float%20%28single-precision%29))
  (Variables|Default|SetHueShift (Math|Float|%(Float) (+ AddHueShift (Variables|Default|GetHueShift)) 1.0))
  (Rendering|Material|SetScalarParameterValue "/Game/Coco/MPC_Palette.MPC_Palette" "HueShift" (Variables|Default|GetHueShift) :!class /Script/Engine.KismetMaterialLibrary))

(fn ChangePaletteSetHueShift
  (params (SetHueShift :type Float%20%28single-precision%29))
  (Variables|Default|SetHueShift (Math|Float|%(Float) SetHueShift 1.0))
  (Rendering|Material|SetScalarParameterValue "/Game/Coco/MPC_Palette.MPC_Palette" "HueShift" (Variables|Default|GetHueShift) :!class /Script/Engine.KismetMaterialLibrary))