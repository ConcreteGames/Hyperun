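; Post-process controller actor that switches the game's screen effects through events across master, fog-without-noise, radial blur and intense components.
; Events toggle these components and rebuild the master settings' weighted blendables, trading the first material against no-noise fog and raising the second for god mode.
; DivideMoblur feeds an amount into the intense settings, and BeginPlay captures the cube scene once.
; Vignette and BloomBoost are empty, with their logic left disconnected.
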(event Custom|Vignette)

(event Custom|NoPP
  (params (ActivateAll :type Boolean))
  (bind _postprocessmaster (Variables|Default|GetPostProcessMaster))
  (Variables|/Script/Engine.PostProcessComponent|SetbEnabled (Variables|Default|GetPostProcessFogNoNoise) false) ; not
  (Variables|/Script/Engine.PostProcessComponent|SetbEnabled (Variables|Default|GetPostProcessMaster) ActivateAll)
  (Variables|/Script/Engine.PostProcessComponent|SetbEnabled (Variables|Default|GetPostProcessRadialBlur) ActivateAll)
  (Variables|/Script/Engine.PostProcessComponent|SetbEnabled (Variables|Default|GetPostProcessIntense) ActivateAll)
  (Variables|/Script/Engine.PostProcessComponent|SetSettings _postprocessmaster (Utilities|Struct|MakePostProcessSettings 1.0 (Utilities|Struct|MakeWeightedBlendables (Utilities|Array|MakeArray (Utilities|Struct|MakeWeightedBlendable 1.0 (.Object (Utilities|Struct|BreakWeightedBlendable (Utilities|Array|Get(acopy) (Utilities|Struct|BreakWeightedBlendables (Utilities|Struct|BreakPostProcessSettings (Variables|/Script/Engine.PostProcessComponent|GetSettings _postprocessmaster))))))) (Utilities|Struct|MakeWeightedBlendable (.Weight (Utilities|Struct|BreakWeightedBlendable (Utilities|Array|Get(acopy) (Utilities|Struct|BreakWeightedBlendables (Utilities|Struct|BreakPostProcessSettings (Variables|/Script/Engine.PostProcessComponent|GetSettings _postprocessmaster))) 1))) (.Object (Utilities|Struct|BreakWeightedBlendable (Utilities|Array|Get(acopy) (Utilities|Struct|BreakWeightedBlendables (Utilities|Struct|BreakPostProcessSettings (Variables|/Script/Engine.PostProcessComponent|GetSettings _postprocessmaster))) 1)))))))))

(event Custom|GodMode
  (bind _postprocessmaster (Variables|Default|GetPostProcessMaster))
  (Variables|/Script/Engine.PostProcessComponent|SetSettings _postprocessmaster (Utilities|Struct|MakePostProcessSettings (Utilities|Struct|MakeWeightedBlendables (Utilities|Array|MakeArray (Utilities|Array|Get(acopy) (Utilities|Struct|BreakWeightedBlendables (Utilities|Struct|BreakPostProcessSettings (Variables|/Script/Engine.PostProcessComponent|GetSettings _postprocessmaster)))) (Utilities|Struct|MakeWeightedBlendable 1.0 (.Object (Utilities|Struct|BreakWeightedBlendable (Utilities|Array|Get(acopy) (Utilities|Struct|BreakWeightedBlendables (Utilities|Struct|BreakPostProcessSettings (Variables|/Script/Engine.PostProcessComponent|GetSettings _postprocessmaster))) 1)))))))))

(event Custom|DivideMoblur
  (params (Amount :type Float%20%28single-precision%29))
  (Variables|/Script/Engine.PostProcessComponent|SetSettings (Variables|Default|GetPostProcessIntense) (Utilities|Struct|MakePostProcessSettings Amount)))

(event Custom|RadialBlurActivate
  (params (SetActive :type Boolean))
  (Variables|/Script/Engine.PostProcessComponent|SetbEnabled (Variables|Default|GetPostProcessRadialBlur) SetActive)
  (Variables|/Script/Engine.PostProcessComponent|SetbEnabled (Variables|Default|GetPostProcessIntense) SetActive))

(event Custom|BloomBoost
  (params (BoostMultiplier :type Float%20%28single-precision%29)))

(event Custom|FogNoNoiseActivate
  (params (SetActive :type Boolean))
  (bind _postprocessmaster (Variables|Default|GetPostProcessMaster))
  (Variables|/Script/Engine.PostProcessComponent|SetbEnabled (Variables|Default|GetPostProcessFogNoNoise) SetActive)
  (Variables|/Script/Engine.PostProcessComponent|SetSettings _postprocessmaster (Utilities|Struct|MakePostProcessSettings 1.0 (Utilities|Struct|MakeWeightedBlendables (Utilities|Array|MakeArray (Utilities|Struct|MakeWeightedBlendable (select SetActive 0.0 1.0) (.Object (Utilities|Struct|BreakWeightedBlendable (Utilities|Array|Get(acopy) (Utilities|Struct|BreakWeightedBlendables (Utilities|Struct|BreakPostProcessSettings (Variables|/Script/Engine.PostProcessComponent|GetSettings _postprocessmaster))))))) (Utilities|Struct|MakeWeightedBlendable (.Weight (Utilities|Struct|BreakWeightedBlendable (Utilities|Array|Get(acopy) (Utilities|Struct|BreakWeightedBlendables (Utilities|Struct|BreakPostProcessSettings (Variables|/Script/Engine.PostProcessComponent|GetSettings _postprocessmaster))) 1))) (.Object (Utilities|Struct|BreakWeightedBlendable (Utilities|Array|Get(acopy) (Utilities|Struct|BreakWeightedBlendables (Utilities|Struct|BreakPostProcessSettings (Variables|/Script/Engine.PostProcessComponent|GetSettings _postprocessmaster))) 1)))))))))

(event EventBeginPlay
  (Rendering|SceneCapture|CaptureScene (Variables|Default|GetSceneCaptureComponentCube) :!class /Script/Engine.SceneCaptureComponentCube))

(fn ConstructionScript)