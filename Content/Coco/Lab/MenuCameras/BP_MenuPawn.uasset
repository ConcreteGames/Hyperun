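; BP_MenuPawn is a menu pawn that gives its Camera a continuous, randomized idle wobble.
; On BeginPlay it starts ManualWobble, which eases the camera to a random relative Y/Z offset and pitch/yaw over a random duration.
; WobblePower scales both ranges, with rotation at a fifth of the positional amount.
; The event calls itself after each latent MoveComponentTo, forming an endless loop without Tick.
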(event Custom|ManualWobble
  (bind _wobblepower (Variables|Default|GetWobblePower))
  (bind _returnvalue (* _wobblepower -1.0))
  (bind _returnvalue_2 (* _wobblepower 0.2))
  (bind _returnvalue_3 (* _returnvalue_2 -1.0))
  (Components|MoveComponentTo (Variables|Default|GetCamera) (Math|Vector|MakeVector 0.0 (Math|Random|RandomFloatinRange _returnvalue _wobblepower) (Math|Random|RandomFloatinRange _returnvalue _wobblepower)) (Math|Rotator|MakeRotator 0.0 (Math|Random|RandomFloatinRange _returnvalue_3 _returnvalue_2) (Math|Random|RandomFloatinRange _returnvalue_3 _returnvalue_2)) true true (Math|Random|RandomFloatinRange 1.0 2.5) false)
  (CallFunction|ManualWobble))

(event EventBeginPlay
  (CallFunction|ManualWobble))

(event Collision|EventActorBeginOverlap
  (params (OtherActor :type Actor%20Object%20Reference)))

(event EventTick
  (params (DeltaSeconds :type Float%20%28single-precision%29)))

(fn ConstructionScript)