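; BP_MenuCameras is the main menu camera rig, moving the player's view between preset cameras for each menu screen and slider item.
; Each tick, nested Selects on BP_MenuManager's current flow and slider states pick a target camera component.
; The BP_MenuPawn's location, rotation and FOV interpolate toward that camera, so the pawn moves instead of switching view targets.
; Tick also spins RotateBody; UpdateCurrentMenuItem stores a clamped index that camera selection ignores.
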(event Custom|UpdateCurrentMenuItem
  (params (Value :type Integer))
  (Variables|Default|SetCurrentMenuItem (Math|Integer|Clamp(Integer) Value 0 5)))

(event EventBeginPlay
  ;[1 1 1] MenuPawn Ref
  (bind _asbp_menu_pawn (Utilities|Casting|CastToBP_MenuPawn (Game|Player|GetPlayerPawn 0)))
  (Variables|Default|SetMenuPawnRef _asbp_menu_pawn)
  ;[1 1 1] menu manager ref
  (bind _outactors (Actor|GetAllActorsOfClass "/Game/UI/Menus/BP_MenuManager.BP_MenuManager_C"))
  (Variables|Default|SetMenuManagerRef (Utilities|Array|Get(acopy) _outactors)))

(event EventTick
  (params (DeltaSeconds :type Float%20%28single-precision%29))
  (bind _returnvalue (Utilities|Time|GetWorldDeltaSeconds))
  (bind _cameratime (Variables|Default|GetCameraTime))
  (bind _cameracusto_tyres (Variables|Default|GetCameraCusto_Tyres))
  (bind _cameracusto_rims (Variables|Default|GetCameraCusto_Rims))
  (bind _cameracusto_sponsor (Variables|Default|GetCameraCusto_Sponsor))
  (bind _cameralb_fsp (Variables|Default|GetCameraLB_FSp))
  (bind _cameralb_wsc (Variables|Default|GetCameraLB_WSc))
  (bind _cameralb_fsc (Variables|Default|GetCameraLB_FSc))
  (bind _cameralb_wsp (Variables|Default|GetCameraLB_WSp))
  (bind _cameralb_overview (Variables|Default|GetCameraLB_Overview))
  (bind _menumanagerref (Variables|Default|GetMenuManagerRef))
  (bind _camerastart (Variables|Default|GetCameraStart))
  (bind _cameracusto (Variables|Default|GetCameraCusto))
  (bind _cameralb (Variables|Default|GetCameraLB))
  (bind _cameraoptions (Variables|Default|GetCameraOptions))
  (bind _cameraexit (Variables|Default|GetCameraExit))
  (bind _cameracusto_body (Variables|Default|GetCameraCusto_Body))
  (bind _cameracusto_exhausts (Variables|Default|GetCameraCusto_Exhausts))
  (bind _cameracusto_lights (Variables|Default|GetCameraCusto_Lights))
  (bind _menupawnref (Variables|Default|GetMenuPawnRef))
  (bind _cameraoptions_2 (Variables|Default|GetCameraOptions))
  (bind _returnvalue_2 (Transformation|GetActorTransform _menupawnref))
  (bind _flow_mainmenu_current (Variables|/Game/UI/Menus/BP_MenuManager.BP_MenuManager_C|GetFlow_MainMenu_Current _menumanagerref))
  (bind _slider_customise_current (Variables|/Game/UI/Menus/BP_MenuManager.BP_MenuManager_C|GetSlider_Customise_Current _menumanagerref))
  (bind _slider_leaderboards_current (Variables|/Game/UI/Menus/BP_MenuManager.BP_MenuManager_C|GetSlider_Leaderboards_Current _menumanagerref))
  (bind _slider_mainmenu_current (Variables|/Game/UI/Menus/BP_MenuManager.BP_MenuManager_C|GetSlider_MainMenu_Current _menumanagerref))
  (bind _camera (Variables|/Game/Coco/Lab/MenuCameras/BP_MenuPawn.BP_MenuPawn_C|GetCamera _menupawnref))
  (bind _returnvalue_3 (Utilities|Select :Index _slider_mainmenu_current :NewEnumerator0 _camerastart :NewEnumerator1 _cameracusto :NewEnumerator2 _cameralb :NewEnumerator3 _cameraoptions_2 :NewEnumerator4 _cameraexit))
  (bind _returnvalue_4 (Utilities|Select :Index _slider_leaderboards_current :NewEnumerator6 _cameralb_wsp :NewEnumerator0 _cameralb_wsc :NewEnumerator1 _cameralb_fsp :NewEnumerator2 _cameralb_fsc :NewEnumerator5 _cameralb_overview))
  (bind _returnvalue_5 (Utilities|Select :Index _slider_customise_current :NewEnumerator0 _cameracusto_body :NewEnumerator1 _cameracusto_body :NewEnumerator5 _cameracusto_body :NewEnumerator6 _cameracusto_body :NewEnumerator7 _cameracusto_exhausts :NewEnumerator8 _cameracusto_lights :NewEnumerator9 _cameracusto_tyres :NewEnumerator10 _cameracusto_tyres :NewEnumerator11 _cameracusto_rims :NewEnumerator12 _cameracusto_rims :NewEnumerator13 _cameracusto_sponsor))
  (bind _returnvalue_6 (Utilities|Select :Index _flow_mainmenu_current :NewEnumerator0 _returnvalue_3 :NewEnumerator5 _cameratime :NewEnumerator2 _returnvalue_5 :NewEnumerator4 _returnvalue_4 :NewEnumerator6 _cameraoptions :NewEnumerator9 _cameraoptions :NewEnumerator10 _cameraoptions :NewEnumerator8 _cameraoptions :NewEnumerator12 _cameraoptions))
  (bind _returnvalue_7 (Transformation|GetWorldTransform _returnvalue_6))
  (Transformation|AddRelativeRotation (Variables|Default|GetRotateBody) (Math|Rotator|MakeRotator 0.0 0.0 (* DeltaSeconds -2e+01)) false false)
  (Utilities|IsValid _menupawnref
    (:Is%20Valid
      (Transformation|SetActorLocationAndRotation _menupawnref (Math|Interpolation|VInterpTo (.location _returnvalue_2) (.location _returnvalue_7) _returnvalue 15.0) (Math|Interpolation|RInterpTo (.rotation _returnvalue_2) (.rotation _returnvalue_7) _returnvalue 15.0))
      (Camera|SetFieldOfView _camera (Math|Interpolation|FInterpTo (Variables|/Script/Engine.CameraComponent|GetFieldOfView _camera) (Variables|/Script/Engine.CameraComponent|GetFieldOfView (.AsCamera%20Component (Utilities|Casting|CastToCameraComponent _returnvalue_6))) _returnvalue 15.0)))))

(fn ConstructionScript)