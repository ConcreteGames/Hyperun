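; BP_NearPropMaster is a randomized near-prop container that becomes one of eight props, including cat balloon, circle variants, 3D text and Ganesh.
; The construction script randomly tilts the Scene component, then adds a Child Actor of a random class at the Arrow's location with random yaw and scale.
; When anything overlaps its Box, it prints that actor's name and, once only, sets a near-zero lifespan to destroy itself.
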(event OnComponentBeginOverlap(Box)
  (params (OverlappedComponent :type Primitive%20Component%20Object%20Reference) (OtherActor :type Actor%20Object%20Reference) (OtherComp :type Primitive%20Component%20Object%20Reference) (OtherBodyIndex :type Integer) (bFromSweep :type Boolean) (SweepResult :type Hit%20Result%20Structure%20%28by%20ref%29))
  (Development|PrintString (Utilities|GetDisplayName OtherActor) true true "(R=1.000000,G=1.000000,B=1.000000,A=1.000000)" 4.0)
  (Utilities|FlowControl|DoOnce false
    (:Completed
      (Actor|SetLifeSpan 0.01))))

(event EventBeginPlay)

(event Collision|EventActorBeginOverlap
  (params (OtherActor :type Actor%20Object%20Reference)))

(event EventTick
  (params (DeltaSeconds :type Float%20%28single-precision%29)))

(fn ConstructionScript
  (bind _returnvalue (Math|Random|RandomFloatinRange 2.0 2.5))
  (Transformation|SetRelativeRotation (Variables|Default|GetScene) (Math|Rotator|MakeRotator (Math|Random|RandomFloatinRange -65.0 65.0) (Math|Random|RandomFloatinRange -65.0 65.0) 0.0) false false)
  (bind _returnvalue_2 (AddComponent|AddChildActorComponent false (Math|Transform|MakeTransform "0, 0, 0" (Math|Rotator|MakeRotator 0.0 0.0 (Math|Random|RandomFloatinRange 0.0 3.6e+02)) (Math|Vector|MakeVector _returnvalue _returnvalue _returnvalue))))
  (Transformation|SetWorldLocation _returnvalue_2 (Transformation|GetWorldLocation (Variables|Default|GetArrow)) false false)
  (ChildActorComponent|SetChildActorClass _returnvalue_2 (Utilities|Select :Index (Math|Random|RandomIntegerinRange 0 7) :Option%200 "/Game/Coco/Lab/Props/NearProps/BP_CatBaloon.BP_CatBaloon_C" :Option%201 "/Game/Coco/Lab/Props/NearProps/BP_NearCircle_1.BP_NearCircle_1_C" :Option%202 "/Game/Coco/Lab/Props/NearProps/BP_NearCircle_2.BP_NearCircle_2_C" :Option%203 "/Game/Coco/Lab/Props/NearProps/BP_NearCircle_3.BP_NearCircle_3_C" :Option%204 "/Game/Coco/Lab/Props/NearProps/BP_NearCircle_4.BP_NearCircle_4_C" :Option%205 "/Game/Coco/Lab/Props/NearProps/BP_NearCircle_5.BP_NearCircle_5_C" :Option%206 "/Game/Coco/Lab/Props/NearProps/BP_Text3D.BP_Text3D_C" :Option%207 "/Game/Coco/Lab/Props/NearProps/Budha/BP_Ganesh.BP_Ganesh_C")))