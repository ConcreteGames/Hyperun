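; BP_Ganesh is a Buddha statue prop that randomizes its look, with no active gameplay logic.
; Its construction script randomly hides the yin-yang mesh and, separately, the holo-ad together with another static mesh.
; It occasionally swaps the Buddha's material to M_Buddha_Inst and gives the Scene component a random scale on each axis, so placed copies vary.
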(event EventBeginPlay)

(event Collision|EventActorBeginOverlap
  (params (OtherActor :type Actor%20Object%20Reference)))

(event EventTick
  (params (DeltaSeconds :type Float%20%28single-precision%29)))

(fn ConstructionScript
  (bind _returnvalue (Math|Random|RandomFloatinRange 0.25 0.5))
  (Utilities|FlowControl|Sequence
    (:then_0
      (if (Math|Random|RandomBool)
        (Rendering|SetVisibility (Variables|Default|GetSM_YinYang) false false)))
    (:then_1
      (if (Math|Random|RandomBool)
        (Rendering|SetVisibility (Variables|Default|GetStaticMesh) false false)))
    (:then_2
      (if (Math|Random|RandomBoolwithWeight 0.2)
        (Rendering|Material|SetMaterial (Variables|Default|GetSM_Buddha) 0 "/Game/Coco/Lab/Props/NearProps/Budha/M_Buddha_Inst.M_Buddha_Inst")))
    (:then_3
      (Transformation|SetRelativeScale3D (Variables|Default|GetScene) (Math|Vector|MakeVector _returnvalue _returnvalue _returnvalue)))))