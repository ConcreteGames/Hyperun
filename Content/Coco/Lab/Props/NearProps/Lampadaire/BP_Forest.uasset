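; BP_Forest is a prop Blueprint that scatters static mesh instances, by its name a forest, along both sides of a central corridor.
; Its construction script adds a fixed number of separate static mesh components in a loop, each randomly placed along X and pushed to either side in Y at a lowered height.
; Random slight tilt, full yaw and small per-axis scale changes vary each copy, using unseeded randomness with no runtime logic.
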(event EventBeginPlay)

(event Collision|EventActorBeginOverlap
  (params (OtherActor :type Actor%20Object%20Reference)))

(event EventTick
  (params (DeltaSeconds :type Float%20%28single-precision%29)))

(fn ConstructionScript
  (bind _returnvalue (Math|Random|RandomFloatinRange 1.0 1.2))
  (for _index (range 0 12)
    (AddComponent|AddStaticMeshComponent false (Math|Transform|MakeTransform (Math|Vector|MakeVector (Math|Random|RandomFloatinRange 0.0 1.5e+03) (* (Math|Random|RandomFloatinRange 1.3e+03 3e+03) (select (Math|Random|RandomBool) -1.0 1.0)) -8e+02) (Math|Rotator|MakeRotator (Math|Random|RandomFloatinRange -5.0 5.0) (Math|Random|RandomFloatinRange -5.0 5.0) (Math|Random|RandomFloatinRange 0.0 3.6e+02)) (Math|Vector|MakeVector _returnvalue _returnvalue _returnvalue)))))