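; Flag prop that plays pass-by whoosh sounds, with pitch or character driven by the bike's speed through a "Speed" parameter.
; Each of four trigger boxes plays its own whoosh on overlap, after CallSpeed maps the first BP_Bike_Parent's speed onto all four sounds.
; The construction script also scales the boxes' X extent from that speed, so trigger length is set at construction rather than updated live.
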(event OnComponentBeginOverlap(Box)
  (params (OverlappedComponent :type Primitive%20Component%20Object%20Reference) (OtherActor :type Actor%20Object%20Reference) (OtherComp :type Primitive%20Component%20Object%20Reference) (OtherBodyIndex :type Integer) (bFromSweep :type Boolean) (SweepResult :type Hit%20Result%20Structure%20%28by%20ref%29))
  (CallFunction|CallSpeed)
  (Class|FMODAudioComponent|Play (Variables|Default|GetWoosh1)))

(event OnComponentBeginOverlap(Box1)
  (params (OverlappedComponent :type Primitive%20Component%20Object%20Reference) (OtherActor :type Actor%20Object%20Reference) (OtherComp :type Primitive%20Component%20Object%20Reference) (OtherBodyIndex :type Integer) (bFromSweep :type Boolean) (SweepResult :type Hit%20Result%20Structure%20%28by%20ref%29))
  (CallFunction|CallSpeed)
  (Class|FMODAudioComponent|Play (Variables|Default|GetWoosh2)))

(event OnComponentBeginOverlap(Box2)
  (params (OverlappedComponent :type Primitive%20Component%20Object%20Reference) (OtherActor :type Actor%20Object%20Reference) (OtherComp :type Primitive%20Component%20Object%20Reference) (OtherBodyIndex :type Integer) (bFromSweep :type Boolean) (SweepResult :type Hit%20Result%20Structure%20%28by%20ref%29))
  (CallFunction|CallSpeed)
  (Class|FMODAudioComponent|Play (Variables|Default|GetWoosh3)))

(event OnComponentBeginOverlap(Box3)
  (params (OverlappedComponent :type Primitive%20Component%20Object%20Reference) (OtherActor :type Actor%20Object%20Reference) (OtherComp :type Primitive%20Component%20Object%20Reference) (OtherBodyIndex :type Integer) (bFromSweep :type Boolean) (SweepResult :type Hit%20Result%20Structure%20%28by%20ref%29))
  (CallFunction|CallSpeed)
  (Class|FMODAudioComponent|Play (Variables|Default|GetWoosh4)))

(event EventBeginPlay)

(event Collision|EventActorBeginOverlap
  (params (OtherActor :type Actor%20Object%20Reference)))

(event EventTick
  (params (DeltaSeconds :type Float%20%28single-precision%29)))

(fn ConstructionScript
  (bind _outactors (Actor|GetAllActorsOfClass "/Game/Bikes/BP_Bike_Parent.BP_Bike_Parent_C"))
  (Components|Box|SetBoxExtent (Variables|Default|GetBox1) (Math|Vector|MakeVector (Math|Float|MapRangeClamped (Variables|/Game/Bikes/BP_Bike_Parent.BP_Bike_Parent_C|GetSpeedWithFactor (Utilities|Array|Get(acopy) _outactors)) 1e+02 1.1e+03 2e+02 1.4e+03) 2e+03 2e+03) true))

(fn CallSpeed
  (bind _outactors (Actor|GetAllActorsOfClass "/Game/Bikes/BP_Bike_Parent.BP_Bike_Parent_C"))
  (Class|FMODAudioComponent|SetParameter (Variables|Default|GetWoosh3) "Speed" (Math|Float|MapRangeClamped (Variables|/Game/Bikes/BP_Bike_Parent.BP_Bike_Parent_C|GetSpeedWithFactor (Utilities|Array|Get(acopy) _outactors)) 1e+02 1.1e+03 0.0 1.0)))