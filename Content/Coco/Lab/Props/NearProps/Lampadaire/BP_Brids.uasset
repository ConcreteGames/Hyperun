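; BP_Brids is a lamppost prop Blueprint whose BirdLauncher event moves pooled bird effects to its location.
; BirdLauncher gathers all BP_birdsPool actors, moves a random one to this root, then resets the Birds component's transform and calls SetActive false with reset.
; The random index is re-evaluated per access, so those steps can hit different pool actors.
; An unconnected PS_Birds emitter spawn and debug prints remain unused.
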(event Custom|BirdLauncher
  (bind _outactors (Actor|GetAllActorsOfClass "/Game/Coco/Lab/Props/NearProps/Lampadaire/BP_birdsPool.BP_birdsPool_C"))
  (Transformation|SetActorLocation (Utilities|Array|Get(acopy) _outactors (Math|Random|RandomIntegerinRange 0 (- (Utilities|Array|Length _outactors) 1))) (Transformation|GetWorldLocation (Variables|Default|GetDefaultSceneRoot)) false false)
  (Transformation|ResetRelativeTransform (Variables|/Game/Coco/Lab/Props/NearProps/Lampadaire/BP_birdsPool.BP_birdsPool_C|GetBirds (Utilities|Array|Get(acopy) _outactors (Math|Random|RandomIntegerinRange 0 (- (Utilities|Array|Length _outactors) 1)))))
  (Components|Activation|SetActive (Variables|/Game/Coco/Lab/Props/NearProps/Lampadaire/BP_birdsPool.BP_birdsPool_C|GetBirds (Utilities|Array|Get(acopy) _outactors (Math|Random|RandomIntegerinRange 0 (- (Utilities|Array|Length _outactors) 1)))) false true))

(event EventBeginPlay)

(event Collision|EventActorBeginOverlap
  (params (OtherActor :type Actor%20Object%20Reference)))

(event EventTick
  (params (DeltaSeconds :type Float%20%28single-precision%29)))

(fn ConstructionScript)