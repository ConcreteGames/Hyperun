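; BP_Armature is a procedural far-background lab prop that builds a vertical armature structure from static meshes, sized by Height.
; The construction script stacks segments every 400 units, mirroring alternate ones on Y with a matching offset so the pattern zigzags without separate meshes.
; A vertically squashed mesh caps the top, and the event graph has no runtime logic.
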(event EventBeginPlay)

(event Collision|EventActorBeginOverlap
  (params (OtherActor :type Actor%20Object%20Reference)))

(event EventTick
  (params (DeltaSeconds :type Float%20%28single-precision%29)))

(fn ConstructionScript
  (bind _height (Variables|Default|GetHeight))
  (for _index (range 0 _height)
    (AddComponent|AddStaticMeshComponent false (Math|Transform|MakeTransform (Math|Vector|MakeVector 0.0 (Math|Float|SelectFloat 0.0 4e+02 (Math|Conversions|ToBoolean(Integer) (Math|Integer|%(Integer) _index 2))) (* _index 4e+02)) "0, 0, 0" (Math|Vector|MakeVector 1.0 (Math|Float|SelectFloat 1.0 -1.0 (Math|Conversions|ToBoolean(Integer) (Math|Integer|%(Integer) _index 2))) 1.0))))
  (AddComponent|AddStaticMeshComponent false (Math|Transform|MakeTransform (Math|Vector|MakeVector 0.0 0.0 (+ (* (+ _height 1) 4e+02) 25.0)) "0, 0, 0" "1.0,1,0.250000")))