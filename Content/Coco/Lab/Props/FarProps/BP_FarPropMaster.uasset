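; Spawner actor that scatters random distant background props (big and small platforms, antennas, a zeppelin) around the Lab level.
; The construction script adds child actor components at four arrow markers: two always, the other two each on a coin flip.
; Each child gets an independently random class and random yaw.
; Randomness is unseeded, so the layout rerolls whenever construction reruns; the event graph is empty.
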(event EventBeginPlay)

(event Collision|EventActorBeginOverlap
  (params (OtherActor :type Actor%20Object%20Reference)))

(event EventTick
  (params (DeltaSeconds :type Float%20%28single-precision%29)))

(fn ConstructionScript
  (bind _returnvalue (AddComponent|AddChildActorComponent false (Math|Transform|MakeTransform (Variables|/Script/Engine.SceneComponent|GetRelativeLocation (Variables|Default|GetArrow1)) (Math|Rotator|MakeRotator 0.0 0.0 (Math|Random|RandomFloatinRange 0.0 3.6e+02)) "1,1,1")))
  (ChildActorComponent|SetChildActorClass _returnvalue (Utilities|Select :Index (Math|Random|RandomIntegerinRange 0 11) :Option%200 "/Game/Coco/Lab/Props/FarProps/BP_FarProp_PlatformBig_1.BP_FarProp_PlatformBig_1_C" :Option%201 "/Game/Coco/Lab/Props/FarProps/BP_FarProp_PlatformBig_2.BP_FarProp_PlatformBig_2_C" :Option%202 "/Game/Coco/Lab/Props/FarProps/BP_FarProp_PlatformBig_3.BP_FarProp_PlatformBig_3_C" :Option%203 "/Game/Coco/Lab/Props/FarProps/BP_FarProp_PlatformBig_4.BP_FarProp_PlatformBig_4_C" :Option%204 "/Game/Coco/Lab/Props/FarProps/BP_FarProp_PlatformSmall_1.BP_FarProp_PlatformSmall_1_C" :Option%205 "/Game/Coco/Lab/Props/FarProps/BP_FarProp_PlatformSmall_2.BP_FarProp_PlatformSmall_2_C" :Option%206 "/Game/Coco/Lab/Props/FarProps/BP_FarProp_PlatformSmall_3.BP_FarProp_PlatformSmall_3_C" :Option%207 "/Game/Coco/Lab/Props/FarProps/BP_FarProp_PlatformSmall_4.BP_FarProp_PlatformSmall_4_C" :Option%208 "/Game/Coco/Lab/Props/FarProps/BP_FarProp_PlatformSmall_5.BP_FarProp_PlatformSmall_5_C" :Option%209 "/Game/Coco/Lab/Props/FarProps/Antenna/BP_Antenna.BP_Antenna_C" :Option%2010 "/Game/Coco/Lab/Props/FarProps/Antenna/BP_Antenna2.BP_Antenna2_C" :Option%2011 "/Game/Coco/Lab/Props/FarProps/Zepplin/BP_Zepplin.BP_Zepplin_C"))
  (bind _returnvalue_2 (AddComponent|AddChildActorComponent false (Math|Transform|MakeTransform (Variables|/Script/Engine.SceneComponent|GetRelativeLocation (Variables|Default|GetArrow)) (Math|Rotator|MakeRotator 0.0 0.0 (Math|Random|RandomFloatinRange 0.0 3.6e+02)) "1,1,1")))
  (ChildActorComponent|SetChildActorClass _returnvalue_2 (Utilities|Select :Index (Math|Random|RandomIntegerinRange 0 11) :Option%200 "/Game/Coco/Lab/Props/FarProps/BP_FarProp_PlatformBig_1.BP_FarProp_PlatformBig_1_C" :Option%201 "/Game/Coco/Lab/Props/FarProps/BP_FarProp_PlatformBig_2.BP_FarProp_PlatformBig_2_C" :Option%202 "/Game/Coco/Lab/Props/FarProps/BP_FarProp_PlatformBig_3.BP_FarProp_PlatformBig_3_C" :Option%203 "/Game/Coco/Lab/Props/FarProps/BP_FarProp_PlatformBig_4.BP_FarProp_PlatformBig_4_C" :Option%204 "/Game/Coco/Lab/Props/FarProps/BP_FarProp_PlatformSmall_1.BP_FarProp_PlatformSmall_1_C" :Option%205 "/Game/Coco/Lab/Props/FarProps/BP_FarProp_PlatformSmall_2.BP_FarProp_PlatformSmall_2_C" :Option%206 "/Game/Coco/Lab/Props/FarProps/BP_FarProp_PlatformSmall_3.BP_FarProp_PlatformSmall_3_C" :Option%207 "/Game/Coco/Lab/Props/FarProps/BP_FarProp_PlatformSmall_4.BP_FarProp_PlatformSmall_4_C" :Option%208 "/Game/Coco/Lab/Props/FarProps/BP_FarProp_PlatformSmall_5.BP_FarProp_PlatformSmall_5_C" :Option%209 "/Game/Coco/Lab/Props/FarProps/Antenna/BP_Antenna.BP_Antenna_C" :Option%2010 "/Game/Coco/Lab/Props/FarProps/Antenna/BP_Antenna2.BP_Antenna2_C" :Option%2011 "/Game/Coco/Lab/Props/FarProps/Zepplin/BP_Zepplin.BP_Zepplin_C"))
  (Utilities|FlowControl|Sequence
    (:then_0
      (if (Math|Random|RandomBool)
        (bind _returnvalue_3 (AddComponent|AddChildActorComponent false (Math|Transform|MakeTransform (Variables|/Script/Engine.SceneComponent|GetRelativeLocation (Variables|Default|GetArrow2)) (Math|Rotator|MakeRotator 0.0 0.0 (Math|Random|RandomFloatinRange 0.0 3.6e+02)) "1,1,1")))
        (ChildActorComponent|SetChildActorClass _returnvalue_3 (Utilities|Select :Index (Math|Random|RandomIntegerinRange 0 11) :Option%200 "/Game/Coco/Lab/Props/FarProps/BP_FarProp_PlatformBig_1.BP_FarProp_PlatformBig_1_C" :Option%201 "/Game/Coco/Lab/Props/FarProps/BP_FarProp_PlatformBig_2.BP_FarProp_PlatformBig_2_C" :Option%202 "/Game/Coco/Lab/Props/FarProps/BP_FarProp_PlatformBig_3.BP_FarProp_PlatformBig_3_C" :Option%203 "/Game/Coco/Lab/Props/FarProps/BP_FarProp_PlatformBig_4.BP_FarProp_PlatformBig_4_C" :Option%204 "/Game/Coco/Lab/Props/FarProps/BP_FarProp_PlatformSmall_1.BP_FarProp_PlatformSmall_1_C" :Option%205 "/Game/Coco/Lab/Props/FarProps/BP_FarProp_PlatformSmall_2.BP_FarProp_PlatformSmall_2_C" :Option%206 "/Game/Coco/Lab/Props/FarProps/BP_FarProp_PlatformSmall_3.BP_FarProp_PlatformSmall_3_C" :Option%207 "/Game/Coco/Lab/Props/FarProps/BP_FarProp_PlatformSmall_4.BP_FarProp_PlatformSmall_4_C" :Option%208 "/Game/Coco/Lab/Props/FarProps/BP_FarProp_PlatformSmall_5.BP_FarProp_PlatformSmall_5_C" :Option%209 "/Game/Coco/Lab/Props/FarProps/Antenna/BP_Antenna.BP_Antenna_C" :Option%2010 "/Game/Coco/Lab/Props/FarProps/Antenna/BP_Antenna2.BP_Antenna2_C" :Option%2011 "/Game/Coco/Lab/Props/FarProps/Zepplin/BP_Zepplin.BP_Zepplin_C"))))
    (:then_1
      (if (Math|Random|RandomBool)
        (bind _returnvalue_4 (AddComponent|AddChildActorComponent false (Math|Transform|MakeTransform (Variables|/Script/Engine.SceneComponent|GetRelativeLocation (Variables|Default|GetArrow3)) (Math|Rotator|MakeRotator 0.0 0.0 (Math|Random|RandomFloatinRange 0.0 3.6e+02)) "1,1,1")))
        (ChildActorComponent|SetChildActorClass _returnvalue_4 (Utilities|Select :Index (Math|Random|RandomIntegerinRange 0 11) :Option%200 "/Game/Coco/Lab/Props/FarProps/BP_FarProp_PlatformBig_1.BP_FarProp_PlatformBig_1_C" :Option%201 "/Game/Coco/Lab/Props/FarProps/BP_FarProp_PlatformBig_2.BP_FarProp_PlatformBig_2_C" :Option%202 "/Game/Coco/Lab/Props/FarProps/BP_FarProp_PlatformBig_3.BP_FarProp_PlatformBig_3_C" :Option%203 "/Game/Coco/Lab/Props/FarProps/BP_FarProp_PlatformBig_4.BP_FarProp_PlatformBig_4_C" :Option%204 "/Game/Coco/Lab/Props/FarProps/BP_FarProp_PlatformSmall_1.BP_FarProp_PlatformSmall_1_C" :Option%205 "/Game/Coco/Lab/Props/FarProps/BP_FarProp_PlatformSmall_2.BP_FarProp_PlatformSmall_2_C" :Option%206 "/Game/Coco/Lab/Props/FarProps/BP_FarProp_PlatformSmall_3.BP_FarProp_PlatformSmall_3_C" :Option%207 "/Game/Coco/Lab/Props/FarProps/BP_FarProp_PlatformSmall_4.BP_FarProp_PlatformSmall_4_C" :Option%208 "/Game/Coco/Lab/Props/FarProps/BP_FarProp_PlatformSmall_5.BP_FarProp_PlatformSmall_5_C" :Option%209 "/Game/Coco/Lab/Props/FarProps/Antenna/BP_Antenna.BP_Antenna_C" :Option%2010 "/Game/Coco/Lab/Props/FarProps/Antenna/BP_Antenna2.BP_Antenna2_C" :Option%2011 "/Game/Coco/Lab/Props/FarProps/Zepplin/BP_Zepplin.BP_Zepplin_C"))))))