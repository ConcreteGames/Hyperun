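; Far-prop master actor that builds a randomized cluster of background props and a branded zeppelin, with all logic in the Construction Script.
; It adds static mesh components at four Arrow markers, each with a random mesh from six far-prop variants and a random yaw.
; The zeppelin gets a random yaw and one stored random brand index, which keeps its logo and body materials matched across five slots.
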(event EventBeginPlay)

(event Collision|EventActorBeginOverlap
  (params (OtherActor :type Actor%20Object%20Reference)))

(event EventTick
  (params (DeltaSeconds :type Float%20%28single-precision%29)))

(fn ConstructionScript
  (bind _sm_zeppelin (Variables|Default|GetSM_Zeppelin))
  (bind _sm_zeppelin_2 (Variables|Default|GetSM_Zeppelin))
  (bind _returnvalue (AddComponent|AddStaticMeshComponent false (Math|Transform|MakeTransform (Variables|/Script/Engine.SceneComponent|GetRelativeLocation (Variables|Default|GetArrow1)) (Math|Rotator|MakeRotator 0.0 0.0 (Math|Random|RandomFloatinRange 0.0 3.6e+02)) "1,1,1")))
  (Components|StaticMesh|SetStaticMesh _returnvalue (Utilities|Select :Index (Math|Random|RandomIntegerinRange 0 5) :Option%200 "/Game/Coco/Lab/Props/FarProps/OptiFarP/SM_FP_1.SM_FP_1" :Option%201 "/Game/Coco/Lab/Props/FarProps/OptiFarP/SM_FP_2.SM_FP_2" :Option%202 "/Game/Coco/Lab/Props/FarProps/OptiFarP/SM_FP_3.SM_FP_3" :Option%203 "/Game/Coco/Lab/Props/FarProps/OptiFarP/SM_FP_4.SM_FP_4" :Option%204 "/Game/Coco/Lab/Props/FarProps/OptiFarP/SM_FP_5.SM_FP_5" :Option%205 "/Game/Coco/Lab/Props/FarProps/OptiFarP/SM_FP_6.SM_FP_6"))
  (bind _returnvalue_2 (AddComponent|AddStaticMeshComponent false (Math|Transform|MakeTransform (Variables|/Script/Engine.SceneComponent|GetRelativeLocation (Variables|Default|GetArrow2)) (Math|Rotator|MakeRotator 0.0 0.0 (Math|Random|RandomFloatinRange 0.0 3.6e+02)) "1,1,1")))
  (Components|StaticMesh|SetStaticMesh _returnvalue_2 (Utilities|Select :Index (Math|Random|RandomIntegerinRange 0 5) :Option%200 "/Game/Coco/Lab/Props/FarProps/OptiFarP/SM_FP_1.SM_FP_1" :Option%201 "/Game/Coco/Lab/Props/FarProps/OptiFarP/SM_FP_2.SM_FP_2" :Option%202 "/Game/Coco/Lab/Props/FarProps/OptiFarP/SM_FP_3.SM_FP_3" :Option%203 "/Game/Coco/Lab/Props/FarProps/OptiFarP/SM_FP_4.SM_FP_4" :Option%204 "/Game/Coco/Lab/Props/FarProps/OptiFarP/SM_FP_5.SM_FP_5" :Option%205 "/Game/Coco/Lab/Props/FarProps/OptiFarP/SM_FP_6.SM_FP_6"))
  (bind _returnvalue_3 (AddComponent|AddStaticMeshComponent false (Math|Transform|MakeTransform (Variables|/Script/Engine.SceneComponent|GetRelativeLocation (Variables|Default|GetArrow3)) (Math|Rotator|MakeRotator 0.0 0.0 (Math|Random|RandomFloatinRange 0.0 3.6e+02)) "1,1,1")))
  (Components|StaticMesh|SetStaticMesh _returnvalue_3 (Utilities|Select :Index (Math|Random|RandomIntegerinRange 0 5) :Option%200 "/Game/Coco/Lab/Props/FarProps/OptiFarP/SM_FP_1.SM_FP_1" :Option%201 "/Game/Coco/Lab/Props/FarProps/OptiFarP/SM_FP_2.SM_FP_2" :Option%202 "/Game/Coco/Lab/Props/FarProps/OptiFarP/SM_FP_3.SM_FP_3" :Option%203 "/Game/Coco/Lab/Props/FarProps/OptiFarP/SM_FP_4.SM_FP_4" :Option%204 "/Game/Coco/Lab/Props/FarProps/OptiFarP/SM_FP_5.SM_FP_5" :Option%205 "/Game/Coco/Lab/Props/FarProps/OptiFarP/SM_FP_6.SM_FP_6"))
  (bind _returnvalue_4 (AddComponent|AddStaticMeshComponent false (Math|Transform|MakeTransform (Variables|/Script/Engine.SceneComponent|GetRelativeLocation (Variables|Default|GetArrow)) (Math|Rotator|MakeRotator 0.0 0.0 (Math|Random|RandomFloatinRange 0.0 3.6e+02)) "1,1,1")))
  (Components|StaticMesh|SetStaticMesh _returnvalue_4 (Utilities|Select :Index (Math|Random|RandomIntegerinRange 0 5) :Option%200 "/Game/Coco/Lab/Props/FarProps/OptiFarP/SM_FP_1.SM_FP_1" :Option%201 "/Game/Coco/Lab/Props/FarProps/OptiFarP/SM_FP_2.SM_FP_2" :Option%202 "/Game/Coco/Lab/Props/FarProps/OptiFarP/SM_FP_3.SM_FP_3" :Option%203 "/Game/Coco/Lab/Props/FarProps/OptiFarP/SM_FP_4.SM_FP_4" :Option%204 "/Game/Coco/Lab/Props/FarProps/OptiFarP/SM_FP_5.SM_FP_5" :Option%205 "/Game/Coco/Lab/Props/FarProps/OptiFarP/SM_FP_6.SM_FP_6"))
  ;[1 1 1] Zeppelin
  (Transformation|SetRelativeRotation (Variables|Default|GetSM_Zeppelin) (Math|Rotator|MakeRotator 0.0 0.0 (Math|Random|RandomFloatinRange 0.0 3.6e+02)) false false)
  (Variables|Default|SetRandBrand (Math|Random|RandomIntegerinRange 0 5))
  (Rendering|Material|SetMaterial (Variables|Default|GetSM_Zeppelin) 2 (Utilities|Select :Index (Variables|Default|GetRandBrand) :Option%200 "/Game/Coco/Lab/Props/FarProps/Zepplin/M_Zeppelinbrand.M_Zeppelinbrand" :Option%201 "/Game/Coco/Lab/Props/FarProps/Zepplin/M_Zeppelinbrand_Archibald.M_Zeppelinbrand_Archibald" :Option%202 "/Game/Coco/Lab/Props/FarProps/Zepplin/M_Zeppelinbrand_dAcOSTA.M_Zeppelinbrand_DaCosta" :Option%203 "/Game/Coco/Lab/Props/FarProps/Zepplin/M_Zeppelinbrand_Dexter.M_Zeppelinbrand_Dexter" :Option%204 "/Game/Coco/Lab/Props/FarProps/Zepplin/M_Zeppelinbrand_JIN.M_Zeppelinbrand_JIN" :Option%205 "/Game/Coco/Lab/Props/FarProps/Zepplin/M_Zeppelinbrand_Zero.M_Zeppelinbrand_Zero"))
  (Rendering|Material|SetMaterial _sm_zeppelin 0 (Utilities|Select :Index (Variables|Default|GetRandBrand) :Option%200 "/Game/Coco/Cel/M_SimpleCel_Inst10.M_SimpleCel_Inst10" :Option%201 "/Game/Coco/Cel/M_SimpleCel_Inst2.M_SimpleCel_Inst2" :Option%202 "/Game/Coco/Cel/M_SimpleCel.M_SimpleCel" :Option%203 "/Game/Coco/Cel/M_SimpleCel_Inst12.M_SimpleCel_Inst12" :Option%204 "/Game/Coco/Cel/M_SimpleCel_Inst13.M_SimpleCel_Inst13" :Option%205 "/Game/Coco/Cel/M_SimpleCel_Inst14.M_SimpleCel_Inst14"))
  (Rendering|Material|SetMaterial _sm_zeppelin 4 (Utilities|Select :Index (Variables|Default|GetRandBrand) :Option%200 "/Game/Coco/Cel/M_SimpleCel_Inst10.M_SimpleCel_Inst10" :Option%201 "/Game/Coco/Cel/M_SimpleCel_Inst2.M_SimpleCel_Inst2" :Option%202 "/Game/Coco/Cel/M_SimpleCel.M_SimpleCel" :Option%203 "/Game/Coco/Cel/M_SimpleCel_Inst12.M_SimpleCel_Inst12" :Option%204 "/Game/Coco/Cel/M_SimpleCel_Inst13.M_SimpleCel_Inst13" :Option%205 "/Game/Coco/Cel/M_SimpleCel_Inst14.M_SimpleCel_Inst14"))
  (Rendering|Material|SetMaterial _sm_zeppelin_2 1 (Utilities|Select :Index (Variables|Default|GetRandBrand) :Option%200 "/Game/Coco/Cel/M_SimpleCel_Inst4.M_SimpleCel_Inst4" :Option%201 "/Game/Coco/Cel/M_SimpleCel_Inst11.M_SimpleCel_Inst11" :Option%202 "/Game/Coco/Cel/M_SimpleCel_Inst2.M_SimpleCel_Inst2" :Option%203 "/Game/Coco/Lab/Props/FarProps/Zepplin/M_Zeppelinbrand_Dexter.M_Zeppelinbrand_Dexter" :Option%204 "/Game/Coco/Cel/M_SimpleCel_Inst2.M_SimpleCel_Inst2" :Option%205 "/Game/Coco/Cel/M_SimpleCel.M_SimpleCel"))
  (Rendering|Material|SetMaterial _sm_zeppelin_2 3 (Utilities|Select :Index (Variables|Default|GetRandBrand) :Option%200 "/Game/Coco/Cel/M_SimpleCel_Inst4.M_SimpleCel_Inst4" :Option%201 "/Game/Coco/Cel/M_SimpleCel_Inst11.M_SimpleCel_Inst11" :Option%202 "/Game/Coco/Cel/M_SimpleCel_Inst2.M_SimpleCel_Inst2" :Option%203 "/Game/Coco/Lab/Props/FarProps/Zepplin/M_Zeppelinbrand_Dexter.M_Zeppelinbrand_Dexter" :Option%204 "/Game/Coco/Cel/M_SimpleCel_Inst2.M_SimpleCel_Inst2" :Option%205 "/Game/Coco/Cel/M_SimpleCel.M_SimpleCel")))