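; Zeppelin prop that gets a randomly chosen brand livery.
; The Construction Script rolls a brand index, which drives Select nodes that assign materials to five slots on the zeppelin mesh component.
; One slot gets the brand material, while two pairs of slots share matching, mostly cel-shaded colour materials.
; The roll is unseeded, so the livery can change whenever construction reruns.
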(fn ConstructionScript
  (bind _sm_zeppelinco (Variables|Default|GetSM_ZeppelinCo))
  (bind _sm_zeppelinco_2 (Variables|Default|GetSM_ZeppelinCo))
  (Variables|Default|SetRandBrand (Math|Random|RandomIntegerinRange 0 5))
  (Rendering|Material|SetMaterial (Variables|Default|GetSM_ZeppelinCo) 2 (Utilities|Select :Index (Variables|Default|GetRandBrand) :Option%200 "/Game/Coco/Lab/Props/FarProps/Zepplin/M_Zeppelinbrand.M_Zeppelinbrand" :Option%201 "/Game/Coco/Lab/Props/FarProps/Zepplin/M_Zeppelinbrand_Archibald.M_Zeppelinbrand_Archibald" :Option%202 "/Game/Coco/Lab/Props/FarProps/Zepplin/M_Zeppelinbrand_dAcOSTA.M_Zeppelinbrand_DaCosta" :Option%203 "/Game/Coco/Lab/Props/FarProps/Zepplin/M_Zeppelinbrand_Dexter.M_Zeppelinbrand_Dexter" :Option%204 "/Game/Coco/Lab/Props/FarProps/Zepplin/M_Zeppelinbrand_JIN.M_Zeppelinbrand_JIN" :Option%205 "/Game/Coco/Lab/Props/FarProps/Zepplin/M_Zeppelinbrand_Zero.M_Zeppelinbrand_Zero"))
  (Rendering|Material|SetMaterial _sm_zeppelinco_2 0 (Utilities|Select :Index (Variables|Default|GetRandBrand) :Option%200 "/Game/Coco/Cel/M_SimpleCel_Inst10.M_SimpleCel_Inst10" :Option%201 "/Game/Coco/Cel/M_SimpleCel_Inst2.M_SimpleCel_Inst2" :Option%202 "/Game/Coco/Cel/M_SimpleCel.M_SimpleCel" :Option%203 "/Game/Coco/Cel/M_SimpleCel_Inst12.M_SimpleCel_Inst12" :Option%204 "/Game/Coco/Cel/M_SimpleCel_Inst13.M_SimpleCel_Inst13" :Option%205 "/Game/Coco/Cel/M_SimpleCel_Inst14.M_SimpleCel_Inst14"))
  (Rendering|Material|SetMaterial _sm_zeppelinco_2 4 (Utilities|Select :Index (Variables|Default|GetRandBrand) :Option%200 "/Game/Coco/Cel/M_SimpleCel_Inst10.M_SimpleCel_Inst10" :Option%201 "/Game/Coco/Cel/M_SimpleCel_Inst2.M_SimpleCel_Inst2" :Option%202 "/Game/Coco/Cel/M_SimpleCel.M_SimpleCel" :Option%203 "/Game/Coco/Cel/M_SimpleCel_Inst12.M_SimpleCel_Inst12" :Option%204 "/Game/Coco/Cel/M_SimpleCel_Inst13.M_SimpleCel_Inst13" :Option%205 "/Game/Coco/Cel/M_SimpleCel_Inst14.M_SimpleCel_Inst14"))
  (Rendering|Material|SetMaterial _sm_zeppelinco 1 (Utilities|Select :Index (Variables|Default|GetRandBrand) :Option%200 "/Game/Coco/Cel/M_SimpleCel_Inst4.M_SimpleCel_Inst4" :Option%201 "/Game/Coco/Cel/M_SimpleCel_Inst11.M_SimpleCel_Inst11" :Option%202 "/Game/Coco/Cel/M_SimpleCel_Inst2.M_SimpleCel_Inst2" :Option%203 "/Game/Coco/Lab/Props/FarProps/Zepplin/M_Zeppelinbrand_Dexter.M_Zeppelinbrand_Dexter" :Option%204 "/Game/Coco/Cel/M_SimpleCel_Inst2.M_SimpleCel_Inst2" :Option%205 "/Game/Coco/Cel/M_SimpleCel.M_SimpleCel"))
  (Rendering|Material|SetMaterial _sm_zeppelinco 3 (Utilities|Select :Index (Variables|Default|GetRandBrand) :Option%200 "/Game/Coco/Cel/M_SimpleCel_Inst4.M_SimpleCel_Inst4" :Option%201 "/Game/Coco/Cel/M_SimpleCel_Inst11.M_SimpleCel_Inst11" :Option%202 "/Game/Coco/Cel/M_SimpleCel_Inst2.M_SimpleCel_Inst2" :Option%203 "/Game/Coco/Lab/Props/FarProps/Zepplin/M_Zeppelinbrand_Dexter.M_Zeppelinbrand_Dexter" :Option%204 "/Game/Coco/Cel/M_SimpleCel_Inst2.M_SimpleCel_Inst2" :Option%205 "/Game/Coco/Cel/M_SimpleCel.M_SimpleCel")))