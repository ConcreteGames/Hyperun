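; BP_AdCorner is an advertisement corner prop that plays FMOD audio while something overlaps its trigger box.
; On BeginPlay it randomly picks one of three values for the FMOD "ADD" parameter through nested weighted booleans, likely selecting which ad plays.
; Box1 overlap starts the audio and end overlap stops it, with no filtering on the overlapping actor.
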(event OnComponentBeginOverlap(Box1)
  (params (OverlappedComponent :type Primitive%20Component%20Object%20Reference) (OtherActor :type Actor%20Object%20Reference) (OtherComp :type Primitive%20Component%20Object%20Reference) (OtherBodyIndex :type Integer) (bFromSweep :type Boolean) (SweepResult :type Hit%20Result%20Structure%20%28by%20ref%29))
  (Class|FMODAudioComponent|Play (Variables|Default|GetFMODAudio)))

(event OnComponentEndOverlap(Box1)
  (params (OverlappedComponent :type Primitive%20Component%20Object%20Reference) (OtherActor :type Actor%20Object%20Reference) (OtherComp :type Primitive%20Component%20Object%20Reference) (OtherBodyIndex :type Integer))
  (Class|FMODAudioComponent|Stop (Variables|Default|GetFMODAudio)))

(event EventBeginPlay
  (bind _fmodaudio (Variables|Default|GetFMODAudio))
  (if (Math|Random|RandomBoolwithWeight 0.25)
    (Class|FMODAudioComponent|SetParameter _fmodaudio "ADD" 1.0)
    (elif (Math|Random|RandomBoolwithWeight 0.5)
      (Class|FMODAudioComponent|SetParameter _fmodaudio "ADD" 3.0)
      (else
        (Class|FMODAudioComponent|SetParameter _fmodaudio "ADD" 2.0)))))

(event Collision|EventActorBeginOverlap
  (params (OtherActor :type Actor%20Object%20Reference)))

(event EventTick
  (params (DeltaSeconds :type Float%20%28single-precision%29)))

(fn ConstructionScript)