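; BP_Ad1 is an advertising structure prop with two light meshes, an ad screen and FMOD audio.
; The construction script randomly shows or hides each light mesh, picks a screen material and sets the audio's "ADD" parameter.
; Material and parameter come from separate random rolls, so they are not guaranteed to match.
; Box overlap starts the audio, and ending the overlap stops it.
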(event OnComponentBeginOverlap(Box)
  (params (OverlappedComponent :type Primitive%20Component%20Object%20Reference) (OtherActor :type Actor%20Object%20Reference) (OtherComp :type Primitive%20Component%20Object%20Reference) (OtherBodyIndex :type Integer) (bFromSweep :type Boolean) (SweepResult :type Hit%20Result%20Structure%20%28by%20ref%29))
  (Class|FMODAudioComponent|Play (Variables|Default|GetFMODAudio)))

(event OnComponentEndOverlap(Box)
  (params (OverlappedComponent :type Primitive%20Component%20Object%20Reference) (OtherActor :type Actor%20Object%20Reference) (OtherComp :type Primitive%20Component%20Object%20Reference) (OtherBodyIndex :type Integer))
  (Class|FMODAudioComponent|Stop (Variables|Default|GetFMODAudio)))

(event EventBeginPlay)

(event Collision|EventActorBeginOverlap
  (params (OtherActor :type Actor%20Object%20Reference)))

(event EventTick
  (params (DeltaSeconds :type Float%20%28single-precision%29)))

(fn ConstructionScript
  (bind _returnvalue (Math|Random|RandomIntegerinRange 0 5))
  (Rendering|SetVisibility (Variables|Default|GetSM_Lights) (Math|Random|RandomBool) false)
  (Rendering|SetVisibility (Variables|Default|GetSM_Lights2) (Math|Random|RandomBool) false)
  (Rendering|Material|SetMaterial (Variables|Default|GetSM_AdScreen) 0 (Utilities|Select :Index _returnvalue :Option%200 "/Game/Coco/Lab/Ads/M_AdScreen_16Frames.M_AdScreen_16Frames" :Option%201 "/Game/Coco/Lab/Ads/M_AdConcrete.M_AdConcrete" :Option%202 "/Game/Coco/Lab/Ads/M_AdScreen_32Frames.M_AdScreen_32Frames" :Option%203 "/Game/Coco/Lab/Ads/M_AdScreen_32Frames.M_AdScreen_32Frames" :Option%204 "/Game/Coco/Lab/Ads/M_AdScreen.M_AdScreen" :Option%205 "/Game/Coco/Lab/Ads/M_AdScreen_1frame.M_AdScreen_1Frame"))
  (Class|FMODAudioComponent|SetParameter (Variables|Default|GetFMODAudio) "ADD" (Utilities|Select :Index _returnvalue :Option%200 3.0 :Option%201 4.0 :Option%202 1.0 :Option%203 1.0 :Option%204 5.0 :Option%205 0.0)))