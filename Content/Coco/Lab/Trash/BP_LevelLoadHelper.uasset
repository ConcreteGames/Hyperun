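; BP_LevelLoadHelper is a short-lived helper actor that triggers tutorial phase loading in BP_GamemodeRun shortly after BeginPlay.
; The LoadTuto1 flag selects phase 1 or phase 4, and the actor expires after either load.
; For phase 1, an unpassed tutorial save runs BP_Scalability's AutoFPS instead, leaving the load to the ContinueTuto event.
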(event Custom|ContinueTuto
  (Default|LoadTutoPhase1 (.AsBP%20Gamemode%20Run (Utilities|Casting|CastToBP_GamemodeRun (Game|GetGameMode))))
  (Actor|SetLifeSpan 0.01))

(event EventBeginPlay
  (bind _returnvalue (Game|GetGameMode))
  (bind _asbp_gamemode_run (Utilities|Casting|CastToBP_GamemodeRun _returnvalue))
  (Utilities|FlowControl|Delay 0.2)
  (if (Variables|Default|GetLoadTuto1)
    (if (Variables|/Game/Base/Blueprints/BP_Save.BP_Save_C|GetSAVE_TutoPassed (Variables|/Game/Base/Blueprints/BP_GameInstance.BP_GameInstance_C|GetSaveREF (.AsBP%20Game%20Instance (Utilities|Casting|CastToBP_GameInstance (Game|GetGameInstance))))) ; scalability
      (Default|LoadTutoPhase1 _asbp_gamemode_run)
      (Actor|SetLifeSpan 0.01 :!label _label)
      (else
        (bind _outactors (Actor|GetAllActorsOfClass "/Game/UI/Menus/MainMenu/BP_Scalability.BP_Scalability_C"))
        (Default|AutoFPS (Utilities|Array|Get(acopy) _outactors) 57.0)))
    (else
      (Default|LoadTutoPhase4 _asbp_gamemode_run)
      (goto _label))))

(event Collision|EventActorBeginOverlap
  (params (OtherActor :type Actor%20Object%20Reference)))

(event EventTick
  (params (DeltaSeconds :type Float%20%28single-precision%29)))

(fn ConstructionScript)