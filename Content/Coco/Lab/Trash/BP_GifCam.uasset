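; Records a rolling replay of the bike's death for an in-game screen and GIF export, skipped during replay playback.
; Tick copies the bike camera, adding pitch shake, and captures a SceneCapture2D into a ring buffer of render targets.
; Death refreshes a speed and pilot-text canvas, which PlayMat bakes into the frames before looping them on a material.
; CreateGif passes frames to the game instance; alternate cinematic camera logic is disconnected.
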(event Custom|UpdateCanvas
  (params (Canvas :type Canvas%20Object%20Reference) (Width :type Integer) (Height :type Integer))
  ;[1 1 1] Dynamic TV Overlay
  (HUD|DrawText Canvas "/Game/Coco/Lab/Gif/Industry_Ultra_Italic.Industry_Ultra_Italic" (Utilities|String|Append (Utilities|String|LeftChop (Utilities|String|ToString(Float) (Variables|/Game/Bikes/BP_Bike_Parent.BP_Bike_Parent_C|GetSpeedWithFactor (Variables|Default|GetBikeRef))) 4) " km/h") (Math|Vector2D|MakeVector2D (* (.x (Variables|Default|GetTexture%20Size)) 0.5) 1e+01) "(R=1.000000,G=0.000000,B=0.000000,A=1.000000)" 0.0 "(R=0.000000,G=0.000000,B=0.000000,A=0.000000)" "(X=1.000,Y=1.000)" true false false "(R=1.000000,G=0.895436,B=0.000000,A=1.000000)")
  (HUD|DrawText Canvas "/Game/Coco/Lab/Gif/Industry_Bold.Industry_Bold" (Utilities|String|SelectString (Utilities|String|Append "Pilot: " (Utilities|String|ToString(Name) (Variables|/Game/Base/Blueprints/BP_GameInstance.BP_GameInstance_C|GetSteamPlayerName (Variables|Default|GetGameInstaceREF)))) (Utilities|Select :Index (Math|Random|RandomIntegerinRange 0 5) :Option%200 "Insane Speed!" :Option%201 "Try Again!" :Option%202 "No Speed Limit!" :Option%203 "Race to Death!" :Option%204 "Just one more time!" :Option%205 "Reckless!") (Variables|Default|GetLocalSteamConnected)) (Math|Vector2D|MakeVector2D 2e+01 2.2e+02) "(R=1.000000,G=1.000000,B=1.000000,A=1.000000)" 0.0 "(R=0.000000,G=0.000000,B=0.000000,A=0.000000)" "(X=1.000,Y=1.000)" false false true "(R=1.000000,G=0.000000,B=0.000000,A=1.000000)")
  (Rendering|Material|SetScalarParameterValue (Variables|Default|GetGifMaterial) "700" (select (>= (Variables|/Game/Bikes/BP_Bike_Parent.BP_Bike_Parent_C|GetSpeedWithFactor (Variables|Default|GetBikeRef)) 7e+02) 1.0 0.0) :!class /Script/Engine.MaterialInstanceDynamic))

(event Custom|PlaceCamera
  (params (BikeCam :type Boolean) (KeepBikeCam :type Boolean))
  ;[1 1 1] Place camera in world every X sec
)

(event Custom|Wobble
  ;[1 0.0557 0] To kill: Wobble
  (Components|MoveComponentTo (Variables|/Script/Engine.SceneCapture2D|GetCaptureComponent2D (Variables|Default|GetGifCam)) (Math|Vector|MakeVector 0.0 (Math|Random|RandomFloatinRange -1e+01 1e+01) (Math|Random|RandomFloatinRange -1e+01 1e+01)) "0, 0, 0" false false (Math|Random|RandomFloatinRange 0.05 0.5) false)
  (CallFunction|Wobble))

(event Custom|CreateRenderTargets
  (bind _texture_size (Variables|Default|GetTexture%20Size))
  ;[1 1 1] Create Render Targets
  (for _index (range 0 (- (* (Variables|Default|GetGifDuration) (Variables|Default|GetCapturesPerSec)) 1))
    (bind _returnvalue (Rendering|CreateRenderTarget2D (Math|Float|Truncate (.x _texture_size)) (Math|Float|Truncate (.y _texture_size))))
    (Variables|/Script/Engine.Texture|SetCompressionNoAlpha _returnvalue true)
    (Variables|/Script/Engine.Texture|SetCompressionSettings _returnvalue "TC_EditorIcon")
    (Utilities|Array|Add (Variables|Default|GetFrames) _returnvalue)))

(event Custom|HitDeathShake
  ;[1 1 1] Camshake
  (bind _newtrack_0 (Timeline|Timeline_0 PlayFromStart)
    (:Update
      (Variables|Default|SetShakePower (+ _newtrack_0 1.0)))))

(event Custom|Death
  ;[1 1 1] Death: update canvas
  (if (not (Variables|/Game/Base/Blueprints/BP_GameInstance.BP_GameInstance_C|GetTRP_PlayReplay (Variables|Default|GetGameInstaceREF)))
    (Class|CanvasRenderTarget2D|UpdateResource (Variables|Default|GetCanvasRef))
    (CallFunction|HitDeathShake)))

(event Custom|DrawOverlayToFrames
  (bind _gifmaterial (Variables|Default|GetGifMaterial))
  (bind _frames (Variables|Default|GetFrames))
  ;[1 1 1] Draw Overlay to RTs (Frames)
  (for (_array_element _array_index) _frames
    (Rendering|Material|SetTextureParameterValue _gifmaterial "Texture" (Utilities|Array|Get(acopy) _frames (Math|Integer|%(Integer) (+ _array_index 1) (Utilities|Array|Length _frames))))
    (Rendering|Material|SetScalarParameterValue _gifmaterial "CustomTime" (* _array_index 0.0495) :!class /Script/Engine.MaterialInstanceDynamic)
    (Rendering|DrawMaterialtoRenderTarget _array_element _gifmaterial)))

(event Custom|PlayMat
  ;[1 1 1] Playback on material
  (Utilities|FlowControl|DoOnce false
    (:Completed
      (Variables|Default|SetUpdateCaptureBool false)
      (CallFunction|DrawOverlaytoFrames)
      (Rendering|Material|SetTextureParameterValue (Variables|Default|GetUE4Material) "Texture" (Utilities|Array|Get(acopy) (Variables|Default|GetFrames) (Math|Integer|%(Integer) (Variables|Default|GetCurrentFrame) (* (Variables|Default|GetGifDuration) (Variables|Default|GetCapturesPerSec)))) :!label _label)
      (Variables|Default|SetCurrentFrame (+ (Variables|Default|GetCurrentFrame) 1))
      (Utilities|FlowControl|Delay (/ 1.0 (Variables|Default|GetPlaybackFPS)))
      (goto _label))))

(event EventBeginPlay
  (bind _texture_size (Variables|Default|GetTexture%20Size))
  ;[1 1 1] Game Instance Ref
  (bind _asbp_game_instance (Utilities|Casting|CastToBP_GameInstance (Game|GetGameInstance)))
  (bind _output_get (Variables|Default|SetGameInstaceREF _asbp_game_instance))
  (if (not (Variables|/Game/Base/Blueprints/BP_GameInstance.BP_GameInstance_C|GetTRP_PlayReplay _output_get))
    ;[1 1 1] Bike Ref
    (bind _outactors (Actor|GetAllActorsOfClass "/Game/Bikes/BP_Bike_Parent.BP_Bike_Parent_C"))
    (Variables|Default|SetBikeRef (Utilities|Array|Get(acopy) _outactors))
    (CallFunction|GetSteamConnection)
    ;[1 1 1] Dynamic TV Overlay
    (bind _returnvalue (CanvasRenderTarget2D|CreateCanvasRenderTarget2D "/Script/Engine.CanvasRenderTarget2D" (Math|Float|Truncate (.x _texture_size)) (Math|Float|Truncate (.y _texture_size))))
    (bind _output_get_2 (Variables|Default|SetCanvasRef _returnvalue))
    (EventDispatchers|BindEventtoOnCanvasRenderTargetUpdate _output_get_2 (delegate Custom|UpdateCanvas))
    ;[1 1 1] Find 2D capture in level
    (bind _outactors_2 (Actor|GetAllActorsOfClass "/Script/Engine.SceneCapture2D"))
    (bind _output_get_3 (Variables|Default|SetGifCam (Utilities|Array|Get(acopy) _outactors_2)))
    (Transformation|AttachComponentToComponent _output_get_3 (Variables|Default|GetArrow) "None" "SnapToTarget" "SnapToTarget" "KeepRelative" true)
    (CallFunction|CreateRenderTargets)
    (bind _returnvalue_2 (Rendering|Material|CreateDynamicMaterialInstance "/Game/Coco/Lab/Trash/M_GifReplay.M_GifReplay" :!class /Script/Engine.KismetMaterialLibrary))
    (bind _output_get_4 (Variables|Default|SetGifMaterial _returnvalue_2))
    (Rendering|Material|SetTextureParameterValue _output_get_4 "Canvas" (Variables|Default|GetCanvasRef))
    (bind _returnvalue_3 (Rendering|Material|CreateDynamicMaterialInstance "/Game/Coco/Lab/Gif/M_GifUE4Playback.M_GifUE4Playback" :!class /Script/Engine.KismetMaterialLibrary))
    (Variables|Default|SetUE4Material _returnvalue_3)))

(event EventEndPlay
  (params (EndPlayReason :type EEndPlayReason%20Enum :default "Destroyed"))
  ;[1 1 1] If Gif is still generating, close it.
  (bind _returnvalue (Class|DemoGameInstance|IsThreadFinished (Variables|Default|GetGameInstaceREF)))
  (if _returnvalue
    (Class|DemoGameInstance|CloseGif (Variables|Default|GetGameInstaceREF))))

(event EventTick
  (params (DeltaSeconds :type Float%20%28single-precision%29))
  (bind _gifcam (Variables|Default|GetGifCam))
  (bind _gameinstaceref (Variables|Default|GetGameInstaceREF))
  (bind _gifcam_2 (Variables|Default|GetGifCam))
  (bind _bikeref (Variables|Default|GetBikeRef))
  (bind _capturecomponent2d (Variables|/Script/Engine.SceneCapture2D|GetCaptureComponent2D _gifcam))
  (bind _cameratp (Variables|/Game/Bikes/BP_Bike_Parent.BP_Bike_Parent_C|GetCameraTP _bikeref))
  (bind _returnvalue (Transformation|GetWorldTransform _cameratp))
  ;[1 1 1] Tick = update capture
  (if (not (or (Variables|/Game/Base/Blueprints/BP_Save.BP_Save_C|GetSAVE_VS_DisableGIF (Variables|/Game/Base/Blueprints/BP_GameInstance.BP_GameInstance_C|GetSaveREF _gameinstaceref)) (Variables|/Game/Base/Blueprints/BP_GameInstance.BP_GameInstance_C|GetTRP_PlayReplay _gameinstaceref)))
    (if (Variables|Default|GetUpdateCaptureBool)
      (Transformation|SetActorLocationAndRotation _gifcam_2 (.location _returnvalue) (Math|Rotator|MakeRotator (.roll (.rotation _returnvalue)) (+ (.pitch (.rotation _returnvalue)) (* (Math|Trig|Sin(Radians) (* (Actor|GetGameTimeSinceCreation) 1.0 (Variables|Default|GetShakePower))) 3.0 (Variables|Default|GetShakePower))) (.yaw (.rotation _returnvalue))))
      (Variables|/Script/Engine.SceneCaptureComponent2D|SetFOVAngle (Variables|/Script/Engine.SceneCapture2D|GetCaptureComponent2D _gifcam_2) (Variables|/Script/Engine.CameraComponent|GetFieldOfView _cameratp))
      (bind _output_get (Variables|/Script/Engine.SceneCaptureComponent2D|SetTextureTarget _capturecomponent2d (Utilities|Array|Get(acopy) (Variables|Default|GetFrames) (Math|Integer|%(Integer) (Variables|Default|GetCurrentFrame) (* (Variables|Default|GetGifDuration) (Variables|Default|GetCapturesPerSec))))))
      (Rendering|SceneCapture|CaptureScene _capturecomponent2d :!class /Script/Engine.SceneCaptureComponent2D)
      (Rendering|Material|SetTextureParameterValue (Variables|Default|GetGifMaterial) "Texture" _output_get)
      (Variables|Default|SetCurrentFrame (+ (Variables|Default|GetCurrentFrame) 1)))))

(fn ConstructionScript)

(fn CreateGif
  (bind _frames (Variables|Default|GetFrames))
  (bind _item (Utilities|Array|Get(acopy) _frames))
  ;[1 1 1] Change FPS to 50
  (bind (_outgifpath _returnvalue) (Class|DemoGameInstance|CreateGif (Variables|Default|GetGameInstaceREF) (Variables|/Script/Engine.TextureRenderTarget2D|GetSizeX _item) (Variables|/Script/Engine.TextureRenderTarget2D|GetSizeY _item) 50 (Utilities|Array|Length _frames) 0 256 200 false))
  (Variables|Default|SetGifPath _outgifpath)
  (return _returnvalue))

(fn GetSteamConnection
  (bind _outactors (Actor|GetAllActorsOfClass "/Game/Base/Blueprints/BP_SteamManager.BP_SteamManager_C"))
  (Utilities|IsValid (Utilities|Array|Get(acopy) _outactors)
    (:Is%20Valid
      (Variables|Default|SetLocalSteamConnected (Variables|/Game/Base/Blueprints/BP_SteamManager.BP_SteamManager_C|GetConnectedToSteamForThisRun (Utilities|Array|Get(acopy) _outactors))))
    (:Is%20Not%20Valid
      (Variables|Default|SetLocalSteamConnected false))))