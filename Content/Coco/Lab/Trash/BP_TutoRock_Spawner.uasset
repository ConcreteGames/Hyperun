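; BP_TutoRock_Spawner is an editor-time placement actor that lays out a row of BP_BorderRock instances, apparently for a tutorial.
; Its construction script adds child actor components along local X, spaced by Distance over an index loop up to Number.
; Each rock's NeedRedSign flag is set either randomly when Randomize is on or from the shared RedSign value.
; The event graph is empty.
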(event EventBeginPlay)

(event Collision|EventActorBeginOverlap
  (params (OtherActor :type Actor%20Object%20Reference)))

(event EventTick
  (params (DeltaSeconds :type Float%20%28single-precision%29)))

(fn ConstructionScript
  (for _index (range 0 (Variables|Default|GetNumber))
    (bind _returnvalue (AddComponent|AddChildActorComponent false (Math|Transform|MakeTransform (Math|Vector|MakeVector (* _index (Variables|Default|GetDistance)) 0.0 0.0) "0, 0, 0" "1,1,1")))
    (bind _asbp_border_rock (Utilities|Casting|CastToBP_BorderRock (Variables|/Script/Engine.ChildActorComponent|GetChildActor _returnvalue)))
    (Variables|/Game/Gameplay/BreakableProps/Blueprints/BP_BorderRock.BP_BorderRock_C|SetNeedRedSign _asbp_border_rock (select (Variables|Default|GetRandomize) (Math|Random|RandomBool) (Variables|Default|GetRedSign)))))