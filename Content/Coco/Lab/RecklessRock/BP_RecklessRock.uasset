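; BP_RecklessRock is a prop the player's bike can break, with a randomized shape.
; The construction script randomizes the mesh's yaw and height scale; a random rock-or-cactus mesh and material swap exists but is disconnected.
; Its Breakless function calls Breakless on the player's BP_Bike_Parent, spawns a bike-oriented cactus burst and an impact effect, then hides the mesh.
; Nothing in this Blueprint triggers Breakless itself.
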(event EventBeginPlay)

(event Collision|EventActorBeginOverlap
  (params (OtherActor :type Actor%20Object%20Reference)))

(event EventTick
  (params (DeltaSeconds :type Float%20%28single-precision%29)))

(fn ConstructionScript
  (bind _sm_rocksmooth_v2 (Variables|Default|GetSM_RockSmooth_v2))
  (Transformation|SetRelativeRotation _sm_rocksmooth_v2 (Math|Rotator|MakeRotator 0.0 0.0 (Math|Random|RandomFloatinRange 0.0 3.6e+02)) false false)
  (Transformation|SetRelativeScale3D _sm_rocksmooth_v2 (Math|Vector|MakeVector 0.7 0.7 (Math|Random|RandomFloatinRange 0.6 0.9))))

(fn Breakless
  (bind _returnvalue (Game|Player|GetPlayerPawn 0))
  (bind _defaultsceneroot (Variables|Default|GetDefaultSceneRoot))
  (bind _asbp_bike_parent (Utilities|Casting|CastToBP_Bike_Parent _returnvalue))
  (bind _bikescene (Variables|/Game/Bikes/BP_Bike_Parent.BP_Bike_Parent_C|GetBikeScene _asbp_bike_parent))
  (bind _asbp_bike_parent_2 (Utilities|Casting|CastToBP_Bike_Parent (Game|Player|GetPlayerPawn 0)))
  (Default|Breakless _asbp_bike_parent_2)
  (Effects|SpawnEmitterAttached "/Game/Coco/Lab/RecklessRock/PS_RecklessCactus.PS_RecklessCactus" _defaultsceneroot "None" (Transformation|GetWorldLocation _defaultsceneroot) (Math|Rotator|MakeRotfromXZ (Math|Vector|GetForwardVector _bikescene) (Math|Vector|GetUpVector _bikescene)) "KeepWorldPosition")
  (Effects|SpawnEmitterAttached "/Game/Coco/Lab/RecklessRock/PS_bIGImpact.PS_BigImpact" (Variables|Default|GetDefaultSceneRoot) "None")
  (Rendering|SetVisibility (Variables|Default|GetSM_RockSmooth_v2) false false))