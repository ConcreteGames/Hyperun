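; Road tunnel entrance/exit actor that carries twelve child actors for whoosh sound effects near props.
; The construction script casts each child actor to BP_SFX_WooshsNearPropsA and sets all of them to the same PropsType enum value.
; The casts run in one chain, so a failed cast leaves the remaining emitters unset; the event graph holds no logic.
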(event EventBeginPlay)

(event Collision|EventActorBeginOverlap
  (params (OtherActor :type Actor%20Object%20Reference)))

(event EventTick
  (params (DeltaSeconds :type Float%20%28single-precision%29)))

(fn ConstructionScript
  (bind _asbp_sfx_wooshs_near_props_a (Utilities|Casting|CastToBP_SFX_WooshsNearPropsA (Variables|/Script/Engine.ChildActorComponent|GetChildActor (Variables|Default|GetChildActor))))
  (Variables|/Game/Sound/Blueprints/BP_SFX_WooshsNearPropsA.BP_SFX_WooshsNearPropsA_C|SetPropsType _asbp_sfx_wooshs_near_props_a "NewEnumerator5")
  (bind _asbp_sfx_wooshs_near_props_a_2 (Utilities|Casting|CastToBP_SFX_WooshsNearPropsA (Variables|/Script/Engine.ChildActorComponent|GetChildActor (Variables|Default|GetChildActor1))))
  (Variables|/Game/Sound/Blueprints/BP_SFX_WooshsNearPropsA.BP_SFX_WooshsNearPropsA_C|SetPropsType _asbp_sfx_wooshs_near_props_a_2 "NewEnumerator5")
  (bind _asbp_sfx_wooshs_near_props_a_3 (Utilities|Casting|CastToBP_SFX_WooshsNearPropsA (Variables|/Script/Engine.ChildActorComponent|GetChildActor (Variables|Default|GetChildActor2))))
  (Variables|/Game/Sound/Blueprints/BP_SFX_WooshsNearPropsA.BP_SFX_WooshsNearPropsA_C|SetPropsType _asbp_sfx_wooshs_near_props_a_3 "NewEnumerator5")
  (bind _asbp_sfx_wooshs_near_props_a_4 (Utilities|Casting|CastToBP_SFX_WooshsNearPropsA (Variables|/Script/Engine.ChildActorComponent|GetChildActor (Variables|Default|GetChildActor3))))
  (Variables|/Game/Sound/Blueprints/BP_SFX_WooshsNearPropsA.BP_SFX_WooshsNearPropsA_C|SetPropsType _asbp_sfx_wooshs_near_props_a_4 "NewEnumerator5")
  (bind _asbp_sfx_wooshs_near_props_a_5 (Utilities|Casting|CastToBP_SFX_WooshsNearPropsA (Variables|/Script/Engine.ChildActorComponent|GetChildActor (Variables|Default|GetChildActor4))))
  (Variables|/Game/Sound/Blueprints/BP_SFX_WooshsNearPropsA.BP_SFX_WooshsNearPropsA_C|SetPropsType _asbp_sfx_wooshs_near_props_a_5 "NewEnumerator5")
  (bind _asbp_sfx_wooshs_near_props_a_6 (Utilities|Casting|CastToBP_SFX_WooshsNearPropsA (Variables|/Script/Engine.ChildActorComponent|GetChildActor (Variables|Default|GetChildActor5))))
  (Variables|/Game/Sound/Blueprints/BP_SFX_WooshsNearPropsA.BP_SFX_WooshsNearPropsA_C|SetPropsType _asbp_sfx_wooshs_near_props_a_6 "NewEnumerator5")
  (bind _asbp_sfx_wooshs_near_props_a_7 (Utilities|Casting|CastToBP_SFX_WooshsNearPropsA (Variables|/Script/Engine.ChildActorComponent|GetChildActor (Variables|Default|GetChildActor6))))
  (Variables|/Game/Sound/Blueprints/BP_SFX_WooshsNearPropsA.BP_SFX_WooshsNearPropsA_C|SetPropsType _asbp_sfx_wooshs_near_props_a_7 "NewEnumerator5")
  (bind _asbp_sfx_wooshs_near_props_a_8 (Utilities|Casting|CastToBP_SFX_WooshsNearPropsA (Variables|/Script/Engine.ChildActorComponent|GetChildActor (Variables|Default|GetChildActor7))))
  (Variables|/Game/Sound/Blueprints/BP_SFX_WooshsNearPropsA.BP_SFX_WooshsNearPropsA_C|SetPropsType _asbp_sfx_wooshs_near_props_a_8 "NewEnumerator5")
  (bind _asbp_sfx_wooshs_near_props_a_9 (Utilities|Casting|CastToBP_SFX_WooshsNearPropsA (Variables|/Script/Engine.ChildActorComponent|GetChildActor (Variables|Default|GetChildActor8))))
  (Variables|/Game/Sound/Blueprints/BP_SFX_WooshsNearPropsA.BP_SFX_WooshsNearPropsA_C|SetPropsType _asbp_sfx_wooshs_near_props_a_9 "NewEnumerator5")
  (bind _asbp_sfx_wooshs_near_props_a_10 (Utilities|Casting|CastToBP_SFX_WooshsNearPropsA (Variables|/Script/Engine.ChildActorComponent|GetChildActor (Variables|Default|GetChildActor9))))
  (Variables|/Game/Sound/Blueprints/BP_SFX_WooshsNearPropsA.BP_SFX_WooshsNearPropsA_C|SetPropsType _asbp_sfx_wooshs_near_props_a_10 "NewEnumerator5")
  (bind _asbp_sfx_wooshs_near_props_a_11 (Utilities|Casting|CastToBP_SFX_WooshsNearPropsA (Variables|/Script/Engine.ChildActorComponent|GetChildActor (Variables|Default|GetChildActor10))))
  (Variables|/Game/Sound/Blueprints/BP_SFX_WooshsNearPropsA.BP_SFX_WooshsNearPropsA_C|SetPropsType _asbp_sfx_wooshs_near_props_a_11 "NewEnumerator5")
  (bind _asbp_sfx_wooshs_near_props_a_12 (Utilities|Casting|CastToBP_SFX_WooshsNearPropsA (Variables|/Script/Engine.ChildActorComponent|GetChildActor (Variables|Default|GetChildActor11))))
  (Variables|/Game/Sound/Blueprints/BP_SFX_WooshsNearPropsA.BP_SFX_WooshsNearPropsA_C|SetPropsType _asbp_sfx_wooshs_near_props_a_12 "NewEnumerator5"))