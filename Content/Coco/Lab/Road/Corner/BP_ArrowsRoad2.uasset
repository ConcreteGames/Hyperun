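; BP_ArrowsRoad2 is a road-corner arrow sign whose three arrow meshes light up one after another in a chasing sequence.
; On BeginPlay a fast looping timer switches all three meshes' "On" material parameter off, then a looping MultiGate turns the next one on.
; An unconnected node that maps player bike speed to a shorter interval is left unused, so the chase runs at a fixed rate.
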(event Custom|CustomEvent_0
  (Rendering|Material|SetScalarParameterValueonMaterials (Variables|Default|GetSM_SmallArrow) "On" 0.0)
  (Utilities|FlowControl|MultiGate false true -1
    (:Out%200
      (Rendering|Material|SetScalarParameterValueonMaterials (Variables|Default|GetSM_SmallArrow) "On" 1.0))
    (:Out%201
      (Rendering|Material|SetScalarParameterValueonMaterials (Variables|Default|GetStaticMesh1) "On" 1.0))
    (:Out%202
      (Rendering|Material|SetScalarParameterValueonMaterials (Variables|Default|GetStaticMesh2) "On" 1.0))))

(event EventBeginPlay
  (Utilities|Time|SetTimerbyEvent (delegate Custom|CustomEvent_0) 0.1 true))

(fn ConstructionScript)