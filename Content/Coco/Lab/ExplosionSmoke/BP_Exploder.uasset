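; Explosion effect actor that randomizes its particles and flings a sphere along a spline path, so instances differ.
; The construction script activates one of two explosion particle systems and randomly sets the active state of the first sparks system.
; BeginPlay randomizes the circular spline's scale and yaw and both sparks rotations, then a timeline drives the sphere's location and rotation along the spline.
; Spline-point rebuilding and smoke material swapping are left unconnected.
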(event EventBeginPlay
  (bind _sphere (Variables|Default|GetSphere))
  (bind _splinecircular (Variables|Default|GetSplineCircular))
  (Transformation|SetRelativeScale3D (Variables|Default|GetSplineCircular) (Math|Vector|MakeVector (Math|Random|RandomFloatinRange 1e+01 3e+01) (Math|Random|RandomFloatinRange 1e+01 3e+01) (Math|Random|RandomFloatinRange 1.0 15.0)))
  (Transformation|SetRelativeRotation (Variables|Default|GetPS_ExplosionSparks) (Math|Rotator|MakeRotator (Math|Random|RandomFloatinRange 0.0 8e+01) 0.0 (Math|Random|RandomFloatinRange 0.0 3.6e+02)) false false)
  (Transformation|SetRelativeRotation (Variables|Default|GetPS_ExplosionSparks2) (Math|Rotator|MakeRotator (Math|Random|RandomFloatinRange 0.0 8e+01) 0.0 (Math|Random|RandomFloatinRange 0.0 3.6e+02)) false false)
  (Transformation|SetRelativeRotation (Variables|Default|GetSplineCircular) (Math|Rotator|MakeRotator 0.0 0.0 (Math|Random|RandomFloatinRange 0.0 3.6e+02)) false false)
  (bind _newtrack_0 (Timeline|Timeline_0 PlayFromStart)
    (:Update
      (Transformation|SetWorldLocation _sphere (Spline|GetLocationatTime _splinecircular _newtrack_0 "World" false) false false)
      (Transformation|SetWorldRotation _sphere (Class|SplineComponent|GetRotationatTime _splinecircular _newtrack_0 "World" false) false false))))

(event Collision|EventActorBeginOverlap
  (params (OtherActor :type Actor%20Object%20Reference)))

(event EventTick
  (params (DeltaSeconds :type Float%20%28single-precision%29)))

(fn ConstructionScript
  (bind _returnvalue (Math|Random|RandomBoolwithWeight 0.3))
  (Components|Activation|SetActive (select (Math|Random|RandomBool) (Variables|Default|GetPS_Explosion2) (Variables|Default|GetPS_ExplosionSmoke)) true true)
  (Components|Activation|SetActive (Variables|Default|GetPS_ExplosionSparks) _returnvalue _returnvalue))