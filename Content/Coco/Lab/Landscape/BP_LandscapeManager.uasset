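; Landscape manager that scatters distant props and sky around the bike run, re-centering itself far below the player on MoveLandscape.
; Outside the tutorial, BeginPlay spawns props at random spots in a Box, with count set by saved scalability level and spawns staggered by short delays.
; SpawnActorEvent re-randomizes them one per frame to spread the cost, and each placement hides props overlapping non-landscape components such as roads.
; ComboBounce drives the child skydome's bounce.
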(event Custom|SpawnActorEvent
  (bind _actorsinworld (Variables|Default|GetActorsInWorld))
  (bind _box (Variables|Default|GetBox))
  (bind _returnvalue (Transformation|GetWorldLocation _box))
  (bind _returnvalue_2 (Components|Box|GetScaledBoxExtent _box))
  (bind _returnvalue_3 (* _returnvalue_2 1.0))
  ;[1 1 1] INIT
  (Variables|Default|SetMovePropsParser (Utilities|Array|LastIndex _actorsinworld))
  (Transformation|SetActorLocationAndRotation (Utilities|Array|Get(acopy) _actorsinworld (Variables|Default|GetMovePropsParser)) (Math|Vector|MakeVector (+ (.x _returnvalue) (Math|Random|RandomFloatinRange (* (.x _returnvalue_3) -1.0) (.x _returnvalue_3))) (+ (.y _returnvalue) (Math|Random|RandomFloatinRange (* (.y _returnvalue_3) -1.0) (.y _returnvalue_3))) (+ (.z _returnvalue) (Math|Random|RandomFloatinRange (* (.z _returnvalue_3) -1.0) (.z _returnvalue_3)))) (Math|Rotator|MakeRotator 0.0 0.0 (Math|Random|RandomFloatinRange 0.0 3.6e+02)) :!label _label)
  (CallFunction|HideifTouchAnyRoad (Utilities|Array|Get(acopy) _actorsinworld (Variables|Default|GetMovePropsParser)))
  (Variables|Default|SetMovePropsParser (- (Variables|Default|GetMovePropsParser) 1))
  (if (not (<= (Variables|Default|GetMovePropsParser) -1)) ; If all props are moved
    (Class|LowEntryExtendedStandardLibrary|DelayFrames 1)
    (goto _label)))

(event Custom|MoveLandscape
  (Transformation|SetActorLocation (+ (Transformation|GetActorLocation (Game|Player|GetPlayerPawn 0)) "0, 0,-60000.000000") false false))

(event Custom|SpawnFarProps
  ;[1 1 1] INIT
  (Variables|Default|SetSpawnPropsParser (Utilities|Select :Index (Variables|/Game/Base/Blueprints/BP_Save.BP_Save_C|GetSAVE_ScalabilityLevel (Variables|/Game/Base/Blueprints/BP_GameInstance.BP_GameInstance_C|GetSaveREF (.AsBP%20Game%20Instance (Utilities|Casting|CastToBP_GameInstance (Game|GetGameInstance))))) :Option%200 45 :Option%201 30 :Option%202 18 :Option%203 9 :Option%204 3 :Option%205 0))
  (CallFunction|PlaceActor :!label _label)
  (Variables|Default|SetSpawnPropsParser (- (Variables|Default|GetSpawnPropsParser) 1))
  (if (not (<= (Variables|Default|GetSpawnPropsParser) 0)) ; If all props are spawned
    (Utilities|FlowControl|Delay 0.02)
    (goto _label)))

(event EventBeginPlay
  (if (not (Variables|/Game/Base/Blueprints/BP_GameInstance.BP_GameInstance_C|GetTutoEnable (.AsBP%20Game%20Instance (Utilities|Casting|CastToBP_GameInstance (Game|GetGameInstance)))))
    (CallFunction|SpawnFarProps)))

(fn ConstructionScript)

(fn PlaceActor
  (bind _box (Variables|Default|GetBox))
  (bind _returnvalue (Transformation|GetWorldLocation _box))
  (bind _returnvalue_2 (Components|Box|GetScaledBoxExtent _box))
  (bind _returnvalue_3 (* _returnvalue_2 1.0))
  (bind _returnvalue_4 (Game|SpawnActorfromClass "/Game/Coco/Lab/Props/FarProps/BP_FarPropMaster_Opti.BP_FarPropMaster_Opti_C" (Math|Transform|MakeTransform (Math|Vector|MakeVector (+ (.x _returnvalue) (Math|Random|RandomFloatinRange (* (.x _returnvalue_3) -1.0) (.x _returnvalue_3))) (+ (.y _returnvalue) (Math|Random|RandomFloatinRange (* (.y _returnvalue_3) -1.0) (.y _returnvalue_3))) (+ (.z _returnvalue) (Math|Random|RandomFloatinRange (* (.z _returnvalue_3) -1.0) (.z _returnvalue_3)))) (Math|Rotator|MakeRotator 0.0 0.0 (Math|Random|RandomFloatinRange 0.0 3.6e+02)) "1,1,1") "Undefined" 0 0))
  (Variables|/Script/Engine.Actor|SetTags _returnvalue_4 (Utilities|Array|MakeArray "FarProps"))
  (CallFunction|HideifTouchAnyRoad _returnvalue_4)
  (Utilities|Array|Add (Variables|Default|GetActorsInWorld) _returnvalue_4))

(fn CleanActors
  (for _array_element (Variables|Default|GetActorsInWorld)
    (Actor|DestroyActor _array_element)))

(fn HideifTouchAnyRoad
  (params (FarPropsElement :type Actor%20Object%20Reference))
  ;[1 1 1] no type test because:
  ; Collide only with "RoadOnlyVisual" coll type
  (bind _array_element (Utilities|Array|ForEachLoopwithBreak (Class|Actor|GetOverlappingComponents FarPropsElement))
    (:LoopBody
      (Rendering|SetActorHiddenInGame FarPropsElement false)
      (if (not (Components|ComponentHasTag _array_element "landscape"))
        (Rendering|SetActorHiddenInGame FarPropsElement true)))))

(fn ComboBounce
  (params (On :type Boolean))
  (Default|SkyBounce (.AsBP%20Skydome%20Parent (Utilities|Casting|CastToBP_Skydome_Parent (Variables|/Script/Engine.ChildActorComponent|GetChildActor (Variables|Default|GetSky)))) (select On 2.0 0.0)))