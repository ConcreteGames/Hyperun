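; BP_AirPlane is an airplane prop that flies continuously forward along its relative X axis.
; Each tick it offsets four static mesh components, not the actor, by a large base speed plus a scaled SpeedWithFactor read from the player's BP_Bike_Parent pawn.
; A delayed BeginPlay sets GoUp, but the only node using it is unconnected, so it does not affect movement.
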(event EventBeginPlay
  (Utilities|FlowControl|Delay 0.5)
  (Variables|Default|SetGoUp 5e+04))

(event Collision|EventActorBeginOverlap
  (params (OtherActor :type Actor%20Object%20Reference)))

(event EventTick
  (params (DeltaSeconds :type Float%20%28single-precision%29))
  (Transformation|AddRelativeLocation (Variables|Default|GetStaticMesh1) (Math|Vector|MakeVector (* DeltaSeconds (+ 2e+04 (* (Variables|/Game/Bikes/BP_Bike_Parent.BP_Bike_Parent_C|GetSpeedWithFactor (.AsBP%20Bike%20Parent (Utilities|Casting|CastToBP_Bike_Parent (Game|Player|GetPlayerPawn 0)))) 2e+01))) 0.0 0.0) false false))

(fn ConstructionScript)