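; BP_StartLight is a start light actor that runs a timed red-to-green countdown.
; Its Countdown event plays one 2D red-light sound, then swaps materials on three light meshes to pink at short delays, finishing with a fourth turning green.
; A RedlightSFX function sets a "Light" parameter on a sound component and plays it, but its calls in the graph are disconnected.
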(event Custom|Countdown
  (Class|FMODBlueprintStatics|PlayEvent2D "/Game/FMOD/Events/SFX/MISC/SFX_RedLight.SFX_RedLight")
  (Rendering|Material|SetMaterial (Variables|Default|GetSM_StartLight_polySurface3) 0 "/Game/Gameplay/CornersCones/Materials/M_Corner_pink.M_Corner_Pink")
  (Utilities|FlowControl|Delay 0.33)
  (Rendering|Material|SetMaterial (Variables|Default|GetSM_StartLight_polySurface5) 0 "/Game/Gameplay/CornersCones/Materials/M_Corner_pink.M_Corner_Pink")
  (Utilities|FlowControl|Delay 0.33)
  (Rendering|Material|SetMaterial (Variables|Default|GetSM_StartLight_polySurface6) 0 "/Game/Gameplay/CornersCones/Materials/M_Corner_pink.M_Corner_Pink")
  (Utilities|FlowControl|Delay 0.33)
  (Rendering|Material|SetMaterial (Variables|Default|GetSM_StartLight_polySurface1) 0 "/Game/Gameplay/CornersCones/Materials/M_Corner_Green.M_Corner_Green"))

(event EventBeginPlay)

(event Collision|EventActorBeginOverlap
  (params (OtherActor :type Actor%20Object%20Reference)))

(event EventTick
  (params (DeltaSeconds :type Float%20%28single-precision%29)))

(fn ConstructionScript)

(fn RedlightSFX
  (params (Sound%20To%20Play :type Float%20%28single-precision%29))
  (bind _redlightsound (Variables|Default|GetRedLightSound))
  (Class|FMODAudioComponent|SetParameter _redlightsound "Light" Sound%20To%20Play)
  (Class|FMODAudioComponent|Play _redlightsound))