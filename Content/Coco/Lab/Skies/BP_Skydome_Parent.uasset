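; Parent skydome Blueprint that drives global lighting colors and direction through MPC_All, expecting BP_LandscapeManager as its parent actor.
; Construction writes light, ambient and flipped light vector parameters, recaptures the BP_PostProcess cube, and pushes fog colors to the manager's smooth terrain meshes.
; Tunnel uses a timeline to darken both colors toward quartered shade color on entry, reversing slower on exit.
; SkyBounce sets the sphere material's Bounce scalar.
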(event Custom|Tunnel
  (params (GoingIn :type Boolean))
  (bind _shadecolor (Variables|Default|GetShadeColor))
  (bind _light (Variables|Default|GetLight))
  (bind _returnvalue (* _shadecolor "(R=0.250000,G=0.250000,B=0.250000,A=1.000000)"))
  (if GoingIn
    (Components|Timeline|SetPlayRate _light 3.0)
    (bind _newtrack_0 (Timeline|Light Play)
      (:Update
        (Rendering|Material|SetVectorParameterValue "/Game/Coco/Cel/MPC_All.MPC_All" "LightColor" (Math|Color|Lerp(LinearColor) (Variables|Default|GetLightColor) _returnvalue _newtrack_0) :!class /Script/Engine.KismetMaterialLibrary)
        (Rendering|Material|SetVectorParameterValue "/Game/Coco/Cel/MPC_All.MPC_All" "AmbientColor" (Math|Color|Lerp(LinearColor) (Variables|Default|GetShadeColor) _returnvalue _newtrack_0) :!class /Script/Engine.KismetMaterialLibrary)))
    (else
      (Components|Timeline|SetPlayRate _light 1.0)
      (Timeline|Light Reverse))))

(event EventBeginPlay)

(fn ConstructionScript
  (bind _returnvalue (Actor|GetParentActor))
  (bind _asbp_landscape_manager (Utilities|Casting|CastToBP_LandscapeManager _returnvalue))
  (bind _sm_terrainsmooth_near (Variables|/Game/Coco/Lab/Landscape/BP_LandscapeManager.BP_LandscapeManager_C|GetSM_TerrainSmooth_Near _asbp_landscape_manager))
  (Rendering|Material|SetVectorParameterValue "/Game/Coco/Cel/MPC_All.MPC_All" "LightColor" (Variables|Default|GetLightColor) :!class /Script/Engine.KismetMaterialLibrary)
  (Rendering|Material|SetVectorParameterValue "/Game/Coco/Cel/MPC_All.MPC_All" "LightVector" (* (Variables|Default|GetLightVector) (Utilities|Struct|MakeLinearColor -1.0 -1.0 1.0 1.0)) :!class /Script/Engine.KismetMaterialLibrary)
  (Rendering|Material|SetVectorParameterValue "/Game/Coco/Cel/MPC_All.MPC_All" "AmbientColor" (Variables|Default|GetShadeColor) :!class /Script/Engine.KismetMaterialLibrary)
  ;[1 0.03247 0] Update capture cube
  (bind _outactors (Actor|GetAllActorsOfClass "/Game/Coco/Outline/BP_PostProcess.BP_PostProcess_C"))
  (Rendering|SceneCapture|CaptureScene (Variables|/Game/Coco/Outline/BP_PostProcess.BP_PostProcess_C|GetSceneCaptureComponentCube (Utilities|Array|Get(acopy) _outactors)) :!class /Script/Engine.SceneCaptureComponentCube)
  ;[1 0.03247 0] Set Fog Color on terrain OR use light & shade colors?
  (Rendering|Material|SetVectorParameterValueonMaterials _sm_terrainsmooth_near "Color1" (Math|Conversions|ToVector(LinearColor) (Variables|Default|GetTerrainFogColor1)))
  (Rendering|Material|SetVectorParameterValueonMaterials _sm_terrainsmooth_near "Color2" (Math|Conversions|ToVector(LinearColor) (Variables|Default|GetTerrainFogColor2))))

(fn SkyBounce
  (params (SkyBounce :type Float%20%28single-precision%29))
  (Rendering|Material|SetScalarParameterValueonMaterials (Variables|Default|GetSphere) "Bounce" SkyBounce))