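; Parent Blueprint for bike customization colors, showing its MainColor on a sphere.
; The construction script sets the sphere material's Color parameter, then writes the same color to the MPC_All parameter collection as BikeColor1, or BikeColor2 when IsSecondaryColor is set.
; All active logic runs at construction; the event graph is empty, and a disconnected node chain that stores RGB values as Tags never runs.
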(event EventBeginPlay)

(event Collision|EventActorBeginOverlap
  (params (OtherActor :type Actor%20Object%20Reference)))

(event EventTick
  (params (DeltaSeconds :type Float%20%28single-precision%29)))

(fn ConstructionScript
  (bind _maincolor (Variables|Default|GetMainColor))
  (bind _maincolor_2 (Variables|Default|GetMainColor))
  (bind _maincolor_3 (Variables|Default|GetMainColor))
  (Rendering|Material|SetVectorParameterValueonMaterials (Variables|Default|GetSphere) "Color" (Math|Vector|MakeVector (.r _maincolor) (.g _maincolor) (.b _maincolor)))
  (if (Variables|Default|GetIsSecondaryColor)
    (Rendering|Material|SetVectorParameterValue "/Game/Coco/Cel/MPC_All.MPC_All" "BikeColor2" (Utilities|Struct|MakeLinearColor (.r _maincolor_3) (.g _maincolor_3) (.b _maincolor_3) 1.0) :!class /Script/Engine.KismetMaterialLibrary)
    (else
      (Rendering|Material|SetVectorParameterValue "/Game/Coco/Cel/MPC_All.MPC_All" "BikeColor1" (Utilities|Struct|MakeLinearColor (.r _maincolor_2) (.g _maincolor_2) (.b _maincolor_2) 1.0) :!class /Script/Engine.KismetMaterialLibrary))))