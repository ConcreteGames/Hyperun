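; Bike customization actor for the dark steel rim option, which applies its material to the bike's wheel rims when it begins play.
; It finds the first BP_Bike_Parent actor in the world, casts the CapBack and CapFront child actors to BP_WheelCap_Parent, and calls SetRimMaterial on each with its Material variable.
; The construction script only calls the parent version.
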(event EventBeginPlay
  (bind _material (Variables|Default|GetMaterial))
  (bind _outactors (Actor|GetAllActorsOfClass "/Game/Bikes/BP_Bike_Parent.BP_Bike_Parent_C"))
  (Utilities|FlowControl|Sequence
    (:then_0
      (bind _asbp_wheel_cap_parent (Utilities|Casting|CastToBP_WheelCap_Parent (Variables|/Script/Engine.ChildActorComponent|GetChildActor (Variables|/Game/Bikes/BP_Bike_Parent.BP_Bike_Parent_C|GetCapBack (Utilities|Array|Get(acopy) _outactors)))))
      (Default|SetRimMaterial _asbp_wheel_cap_parent _material))
    (:then_1
      (bind _asbp_wheel_cap_parent_2 (Utilities|Casting|CastToBP_WheelCap_Parent (Variables|/Script/Engine.ChildActorComponent|GetChildActor (Variables|/Game/Bikes/BP_Bike_Parent.BP_Bike_Parent_C|GetCapFront (Utilities|Array|Get(acopy) _outactors)))))
      (Default|SetRimMaterial _asbp_wheel_cap_parent_2 _material))))

(event Collision|EventActorBeginOverlap
  (params (OtherActor :type Actor%20Object%20Reference)))

(event EventTick
  (params (DeltaSeconds :type Float%20%28single-precision%29)))

(fn ConstructionScript
  (|CallParentFunction))