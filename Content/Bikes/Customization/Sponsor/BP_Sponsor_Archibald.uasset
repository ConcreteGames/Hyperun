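; Sponsor Blueprint for the Archibald brand that paints its artwork into the sponsor render target used for bike customization.
; On BeginPlay it clears T_Sponsor to transparent, then draws the Archibald texture over the whole canvas with masked blending.
; A disconnected chain that would call SetSponsor on the first bike's body never runs.
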(event EventBeginPlay
  (Rendering|ClearRenderTarget2D "/Game/Bikes/Customization/Sponsor/T_Sponsor.T_Sponsor" "(R=0.000000,G=0.000000,B=0.000000,A=0.000000)")
  (bind (_canvas _size _context) (Rendering|BeginDrawCanvastoRenderTarget "/Game/Bikes/Customization/Sponsor/T_Sponsor.T_Sponsor"))
  (Canvas|DrawTexture :self _canvas :RenderTexture "/Game/Bikes/Customization/Sponsor/T_SponsorOneFile_Archibald_v2.T_SponsorOneFile_Archibald_v2" :ScreenSize _size :BlendMode "BLEND_Masked")
  (Rendering|EndDrawCanvastoRenderTarget _context))

(fn ConstructionScript
  (|CallParentFunction))