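; Bike body variant 04 for bike customization, a child Blueprint that exposes material setters for its meshes.
; SetBodyMaterial recolors slot 1 on the body and rear-lights meshes, while SetExhaustsMaterial sets slot 0 on the exhaust mesh.
; Breakage is inactive: BreakBody is empty, and BeginPlay calls an empty CustomHideBorkenBody, with leftover break and hide nodes left disconnected.
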(event EventBeginPlay
  (CallFunction|CustomHideBorkenBody true))

(event Collision|EventActorBeginOverlap
  (params (OtherActor :type Actor%20Object%20Reference)))

(event EventBreakBody
  (params (LifeLeft :type Integer)))

(event EventTick
  (params (DeltaSeconds :type Float%20%28single-precision%29)))

(event EventSetBodyMaterial
  (params (MainMat :type Material%20Object%20Reference) (SecondMat :type Material%20Object%20Reference))
  (Rendering|Material|SetMaterial (Variables|Default|GetSM_Body_04) 1 MainMat))

(event EventSetExhaustsMaterial
  (params (Material :type Material%20Object%20Reference))
  (Rendering|Material|SetMaterial (Variables|Default|GetSM_Body04_Exhaust) 0 Material))

(fn ConstructionScript
  (|CallParentFunction))

(fn CustomHideBorkenBody
  (params (Hidden :type Boolean)))