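; Bike body customization part for the Quasar body, with setters for its body and exhaust materials.
; After a short delay on BeginPlay it hides the tyres and caps of the first BP_Bike_Parent found, restoring them on EndPlay.
; The saved item state in the game instance selects either the Quasar mesh with post-processing enabled or the SMQuasar mesh with it disabled.
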(event EventBeginPlay
  (bind _postprocess (Variables|Default|GetPostProcess))
  (Utilities|FlowControl|Sequence
    (:then_0
      (Utilities|FlowControl|Delay 0.2)
      (bind _outactors (Actor|GetAllActorsOfClass "/Game/Bikes/BP_Bike_Parent.BP_Bike_Parent_C"))
      (Rendering|SetVisibility (Variables|/Game/Bikes/BP_Bike_Parent.BP_Bike_Parent_C|GetTyreBack (Utilities|Array|Get(acopy) _outactors)) false false))
    (:then_1
      (if (Utilities|Enum|Equal(Enum) (.ItemState (Utilities|Struct|BreakSTRU_Item (Utilities|Array|Get(acopy) (Variables|/Game/Base/Blueprints/BP_Save.BP_Save_C|GetSAVE_Items_Body (Variables|/Game/Base/Blueprints/BP_GameInstance.BP_GameInstance_C|GetSaveREF (.AsBP%20Game%20Instance (Utilities|Casting|CastToBP_GameInstance (Game|GetGameInstance))))) 3))) "NewEnumerator0")
        (Rendering|SetVisibility (Variables|Default|Getquasar) true true)
        (Rendering|SetVisibility (Variables|Default|GetSM_Quasar) false false)
        (Variables|/Script/Engine.PostProcessComponent|SetbEnabled _postprocess true)
        (else
          (Rendering|SetVisibility (Variables|Default|GetSM_Quasar) true false)
          (Rendering|SetVisibility (Variables|Default|Getquasar) false true)
          (Variables|/Script/Engine.PostProcessComponent|SetbEnabled _postprocess false))))))

(event EventSetBodyMaterial
  (params (MainMat :type Material%20Object%20Reference) (SecondMat :type Material%20Object%20Reference))
  (bind _quasar (Variables|Default|Getquasar))
  (Rendering|Material|SetMaterial _quasar 2 MainMat)
  (Rendering|Material|SetMaterial _quasar 3 SecondMat))

(event EventSetExhaustsMaterial
  (params (Material :type Material%20Object%20Reference))
  (Rendering|Material|SetMaterial (Variables|Default|Getquasar) 1 Material))

(event EventEndPlay
  (params (EndPlayReason :type EEndPlayReason%20Enum :default "Destroyed"))
  (bind _outactors (Actor|GetAllActorsOfClass "/Game/Bikes/BP_Bike_Parent.BP_Bike_Parent_C"))
  (Rendering|SetVisibility (Variables|/Game/Bikes/BP_Bike_Parent.BP_Bike_Parent_C|GetTyreBack (Utilities|Array|Get(acopy) _outactors)) true false))

(fn ConstructionScript
  (|CallParentFunction))