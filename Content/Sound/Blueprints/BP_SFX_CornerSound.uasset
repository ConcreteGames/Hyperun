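; Corner sound Blueprint built to give left/right audio feedback as the player nears a road edge, but all its event logic is disconnected and never runs.
; The unwired chains start a 2D distance event with an "LR" side parameter and map player distance from EvoLimit to its "Evo" parameter.
; Others play a one-shot corner bip or stop both sounds, while the overlap, Tick, Dead and Stunned events are empty.
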(event OnComponentBeginOverlap(BoxRight)
  (params (OverlappedComponent :type Primitive%20Component%20Object%20Reference) (OtherActor :type Actor%20Object%20Reference) (OtherComp :type Primitive%20Component%20Object%20Reference) (OtherBodyIndex :type Integer) (bFromSweep :type Boolean) (SweepResult :type Hit%20Result%20Structure%20%28by%20ref%29))
  ;[0.1212 1 0.2773] Right Play and Stop
)

(event OnComponentBeginOverlap(BoxLeft)
  (params (OverlappedComponent :type Primitive%20Component%20Object%20Reference) (OtherActor :type Actor%20Object%20Reference) (OtherComp :type Primitive%20Component%20Object%20Reference) (OtherBodyIndex :type Integer) (bFromSweep :type Boolean) (SweepResult :type Hit%20Result%20Structure%20%28by%20ref%29))
  ;[0.1537 1 0.18] Left play and stop
)

(event OnComponentEndOverlap(BoxLeft)
  (params (OverlappedComponent :type Primitive%20Component%20Object%20Reference) (OtherActor :type Actor%20Object%20Reference) (OtherComp :type Primitive%20Component%20Object%20Reference) (OtherBodyIndex :type Integer))
  ;[0.1537 1 0.18] Left play and stop
)

(event OnComponentEndOverlap(BounceZone)
  (params (OverlappedComponent :type Primitive%20Component%20Object%20Reference) (OtherActor :type Actor%20Object%20Reference) (OtherComp :type Primitive%20Component%20Object%20Reference) (OtherBodyIndex :type Integer))
  ;[0.07387 1 0.1304] Limit box and bip sound
)

(event OnComponentEndOverlap(BoxRight)
  (params (OverlappedComponent :type Primitive%20Component%20Object%20Reference) (OtherActor :type Actor%20Object%20Reference) (OtherComp :type Primitive%20Component%20Object%20Reference) (OtherBodyIndex :type Integer))
  ;[0.1212 1 0.2773] Right Play and Stop
)

(event Custom|Stunned
  ;[0.1857 1 0.1683] Init Dead and Stun
)

(event Custom|Dead
  ;[0.1857 1 0.1683] Init Dead and Stun
)

(event EventTick
  (params (DeltaSeconds :type Float%20%28single-precision%29))
  ;[0.1857 1 0.1683] Tick for distance
)

(fn ConstructionScript)