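; Sound actor that plays a one-shot whoosh when its trigger box is overlapped near a prop.
; The construction script picks the whoosh event by PropsType and sizes the trigger from the first bike's speed.
; Collision is enabled shortly after BeginPlay; overlap maps bike speed to the sound's Speed parameter and plays it once.
; InitBoxExtent's overlap does nothing, and the event graph's duplicate setup logic is disconnected.
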(event OnComponentBeginOverlap(Trigger)
  (params (OverlappedComponent :type Primitive%20Component%20Object%20Reference) (OtherActor :type Actor%20Object%20Reference) (OtherComp :type Primitive%20Component%20Object%20Reference) (OtherBodyIndex :type Integer) (bFromSweep :type Boolean) (SweepResult :type Hit%20Result%20Structure%20%28by%20ref%29))
  (bind _outactors (Actor|GetAllActorsOfClass "/Game/Bikes/BP_Bike_Parent.BP_Bike_Parent_C"))
  (Class|FMODAudioComponent|SetParameter (Variables|Default|GetWooshs) "Speed" (Math|Float|MapRangeClamped (Variables|/Game/Bikes/BP_Bike_Parent.BP_Bike_Parent_C|GetSpeedWithFactor (Utilities|Array|Get(acopy) _outactors)) 1e+02 1e+03 0.0 1.0))
  (Utilities|FlowControl|DoOnce false
    (:Completed
      (Class|FMODAudioComponent|Play (Variables|Default|GetWooshs)))))

(event OnComponentBeginOverlap(InitBoxExtent)
  (params (OverlappedComponent :type Primitive%20Component%20Object%20Reference) (OtherActor :type Actor%20Object%20Reference) (OtherComp :type Primitive%20Component%20Object%20Reference) (OtherBodyIndex :type Integer) (bFromSweep :type Boolean) (SweepResult :type Hit%20Result%20Structure%20%28by%20ref%29)))

(event EventBeginPlay
  (bind _trigger (Variables|Default|GetTrigger))
  (Utilities|FlowControl|Delay 0.5)
  (Collision|SetCollisionEnabled _trigger "QueryOnly")
  (Collision|SetCollisionResponsetoChannel _trigger "ECC_Pawn" "ECR_Overlap"))

(fn ConstructionScript
  (bind _wooshs (Variables|Default|GetWooshs))
  (switch Utilities|FlowControl|Switch|SwitchonE_PropsSounds (Variables|Default|GetPropsType)
    (:NewEnumerator0
      (Class|FMODAudioComponent|SetEvent _wooshs "/Game/FMOD/Events/SFX/PROPS/SFX_WHOOSH_BigStereo.SFX_WHOOSH_BigStereo")
      (Variables|Default|SetXA 2.5e+02)
      (Variables|Default|SetXB 1.4e+03)
      (Variables|Default|SetYA 2e+03)
      (Variables|Default|SetYB 1.2e+03))
    (:NewEnumerator1
      (Class|FMODAudioComponent|SetEvent _wooshs "/Game/FMOD/Events/SFX/PROPS/SFX_WHOOSH_SideProps.SFX_WHOOSH_SideProps" :!label _label)
      (Variables|Default|SetXA 2.5e+02)
      (Variables|Default|SetXB 1.4e+03)
      (Variables|Default|SetYA 2e+03)
      (Variables|Default|SetYB 1.2e+03))
    (:NewEnumerator2
      (goto _label))
    (:NewEnumerator3
      (Class|FMODAudioComponent|SetEvent _wooshs "/Game/FMOD/Events/SFX/PROPS/SFX_WHOOSH_Lights.SFX_WHOOSH_Lights")
      (Variables|Default|SetXA 2e+02)
      (Variables|Default|SetXB 1.4e+03)
      (Variables|Default|SetYA 2e+03)
      (Variables|Default|SetYB 1.2e+03))
    (:NewEnumerator4
      (Class|FMODAudioComponent|SetEvent _wooshs "/Game/FMOD/Events/SFX/PROPS/SFX_WHOOSH_Jumpdoor.SFX_WHOOSH_Jumpdoor")
      (Variables|Default|SetXA 2e+02)
      (Variables|Default|SetXB 1.4e+03)
      (Variables|Default|SetYA 2e+03)
      (Variables|Default|SetYB 1.2e+03))
    (:NewEnumerator5
      (Class|FMODAudioComponent|SetEvent _wooshs "/Game/FMOD/Events/SFX/PROPS/SFX_WHOOSH_Tunnel.SFX_WHOOSH_Tunnel")
      (Variables|Default|SetXA 2e+02)
      (Variables|Default|SetXB 1.4e+03)
      (Variables|Default|SetYA 2e+03)
      (Variables|Default|SetYB 1.2e+03))
    (:NewEnumerator6
      (Class|FMODAudioComponent|SetEvent _wooshs "/Game/FMOD/Events/SFX/PROPS/SFX_WHOOSH_Flags.SFX_WHOOSH_Flags")
      (Variables|Default|SetXA 2e+02)
      (Variables|Default|SetXB 1.4e+03)
      (Variables|Default|SetYA 2e+03)
      (Variables|Default|SetYB 1.2e+03)))
  (CallFunction|WooshBoxExtent (Variables|Default|GetXA) (Variables|Default|GetXB) (Variables|Default|GetYA) (Variables|Default|GetYB)))

(fn WooshBoxExtent
  (params (XA :type Float%20%28single-precision%29) (XB :type Float%20%28single-precision%29) (YA :type Float%20%28single-precision%29) (YB :type Float%20%28single-precision%29))
  (bind _outactors (Actor|GetAllActorsOfClass "/Game/Bikes/BP_Bike_Parent.BP_Bike_Parent_C"))
  (Variables|Default|SetBoxExtent (Math|Vector|MakeVector (Math|Float|MapRangeClamped (Variables|/Game/Bikes/BP_Bike_Parent.BP_Bike_Parent_C|GetSpeedWithFactor (Utilities|Array|Get(acopy) _outactors)) 1e+02 1.1e+03 XA XB) (Math|Float|MapRangeClamped (Variables|/Game/Bikes/BP_Bike_Parent.BP_Bike_Parent_C|GetSpeedWithFactor (Utilities|Array|Get(acopy) _outactors)) 1e+02 1.1e+03 YA YB) 5e+02))
  (Components|Box|SetBoxExtent (Variables|Default|GetTrigger) (Variables|Default|GetBoxExtent) true))