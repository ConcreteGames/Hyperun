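; Sound actor that plays a one-time whoosh when its trigger box is overlapped, scaled to the bike's speed.
; On overlap it maps the first BP_Bike_Parent's speed to the Wooshs "Speed" parameter, then plays through a DoOnce that is never reset.
; The construction script sizes the box's X and Y extents from that speed.
; WooshBoxExtent offers the same resize with adjustable ranges and less height, but is not called here.
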(event OnComponentBeginOverlap(Trigger)
  (params (OverlappedComponent :type Primitive%20Component%20Object%20Reference) (OtherActor :type Actor%20Object%20Reference) (OtherComp :type Primitive%20Component%20Object%20Reference) (OtherBodyIndex :type Integer) (bFromSweep :type Boolean) (SweepResult :type Hit%20Result%20Structure%20%28by%20ref%29))
  (bind _outactors (Actor|GetAllActorsOfClass "/Game/Bikes/BP_Bike_Parent.BP_Bike_Parent_C"))
  (Class|FMODAudioComponent|SetParameter (Variables|Default|GetWooshs) "Speed" (Math|Float|MapRangeClamped (Variables|/Game/Bikes/BP_Bike_Parent.BP_Bike_Parent_C|GetSpeedWithFactor (Utilities|Array|Get(acopy) _outactors)) 1e+02 1e+03 0.0 1.0))
  (Utilities|FlowControl|DoOnce false
    (:Completed
      (Class|FMODAudioComponent|Play (Variables|Default|GetWooshs)))))

(fn ConstructionScript
  (bind _outactors (Actor|GetAllActorsOfClass "/Game/Bikes/BP_Bike_Parent.BP_Bike_Parent_C"))
  (Variables|Default|SetBoxExtent (Math|Vector|MakeVector (Math|Float|MapRangeClamped (Variables|/Game/Bikes/BP_Bike_Parent.BP_Bike_Parent_C|GetSpeedWithFactor (Utilities|Array|Get(acopy) _outactors)) 1e+02 1.1e+03 1e+02 4e+02) (Math|Float|MapRangeClamped (Variables|/Game/Bikes/BP_Bike_Parent.BP_Bike_Parent_C|GetSpeedWithFactor (Utilities|Array|Get(acopy) _outactors)) 1e+02 1.1e+03 2e+02 4e+02) 1e+03))
  (Components|Box|SetBoxExtent (Variables|Default|GetTrigger) (Variables|Default|GetBoxExtent) true))

(fn WooshBoxExtent
  (params (XA :type Float%20%28single-precision%29) (XB :type Float%20%28single-precision%29) (YA :type Float%20%28single-precision%29) (YB :type Float%20%28single-precision%29))
  (bind _outactors (Actor|GetAllActorsOfClass "/Game/Bikes/BP_Bike_Parent.BP_Bike_Parent_C"))
  (Variables|Default|SetBoxExtent (Math|Vector|MakeVector (Math|Float|MapRangeClamped (Variables|/Game/Bikes/BP_Bike_Parent.BP_Bike_Parent_C|GetSpeedWithFactor (Utilities|Array|Get(acopy) _outactors)) 1e+02 1.1e+03 XA XB) (Math|Float|MapRangeClamped (Variables|/Game/Bikes/BP_Bike_Parent.BP_Bike_Parent_C|GetSpeedWithFactor (Utilities|Array|Get(acopy) _outactors)) 1e+02 1.1e+03 YA YB) 5e+02))
  (Components|Box|SetBoxExtent (Variables|Default|GetTrigger) (Variables|Default|GetBoxExtent) true))