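; Small left-hand corner cone, a child Blueprint that marks a corner with sound, colored smoke and a rock.
; On BeginPlay it flags its corner-sound child actor as left and tints the smoke particle green.
; The smoke is randomly removed, or removed when too tilted; otherwise its world rotation is reset.
; The first capsule overlap calls Breakless on the child RecklessRock actor.
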(event OnComponentBeginOverlap(Capsule)
  (params (OverlappedComponent :type Primitive%20Component%20Object%20Reference) (OtherActor :type Actor%20Object%20Reference) (OtherComp :type Primitive%20Component%20Object%20Reference) (OtherBodyIndex :type Integer) (bFromSweep :type Boolean) (SweepResult :type Hit%20Result%20Structure%20%28by%20ref%29))
  (Utilities|FlowControl|DoOnce false
    (:Completed
      (bind _asbp_reckless_rock (Utilities|Casting|CastToBP_RecklessRock (Variables|/Script/Engine.ChildActorComponent|GetChildActor (Variables|Default|GetBP_RecklessRock))))
      (Default|Breakless _asbp_reckless_rock))))

(event Custom|Corner%20Sound
  (bind _asbp_sfx_corner_sound (Utilities|Casting|CastToBP_SFX_CornerSound (Variables|/Script/Engine.ChildActorComponent|GetChildActor (Variables|Default|GetCorner%20Feedback))))
  (Variables|/Game/Sound/Blueprints/BP_SFX_CornerSound.BP_SFX_CornerSound_C|SetLeftOrRight _asbp_sfx_corner_sound 0.0)
  (Variables|/Game/Sound/Blueprints/BP_SFX_CornerSound.BP_SFX_CornerSound_C|SetIsLeft _asbp_sfx_corner_sound true))

(event EventBeginPlay
  (bind _ps_fumigene (Variables|Default|GetPS_Fumigene))
  (CallFunction|CornerSound)
  (Variables|/Script/Engine.ParticleSystemComponent|SetInstanceParameters (Variables|Default|GetPS_Fumigene) (Utilities|Array|MakeArray (Utilities|Struct|MakeParticleSysParam "Color" "PSPT_Vector" 0.0 0.0 (Math|Conversions|ToVector(LinearColor) "(R=0.251264,G=0.715000,B=0.000000,A=1.000000)"))))
  ;[1 1 1] Duplicate crade
  (if (Math|Random|RandomBoolwithWeight 0.5)
    (if (< (Math|Vector|DotProduct (Math|Vector|GetUpVector (Variables|Default|GetPS_Fumigene)) (Math|Vector|MakeVector 0.0 0.0 1.0)) 0.75)
      (Components|DestroyComponent _ps_fumigene :!label _label)
      (else
        (Transformation|SetWorldRotation _ps_fumigene "0, 0, 0" false false)))
    (else
      (goto _label))))

(fn ConstructionScript
  (|CallParentFunction))