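; Left-corner road dressing that registers fences, a turn arrow and a wall limit as instances in the level's shared BP_ISMBank.
; Arrow style follows bike speed, falling back to the gamemode's corner arrow type.
; BeginPlay randomly keeps a green smoke flare if near upright; a capsule overlap calls Breakless once on the child RecklessRock.
; EndPlay removes as many bank instances as it added, always at index 0 rather than its own indices.
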(event OnComponentBeginOverlap(Capsule)
  (params (OverlappedComponent :type Primitive%20Component%20Object%20Reference) (OtherActor :type Actor%20Object%20Reference) (OtherComp :type Primitive%20Component%20Object%20Reference) (OtherBodyIndex :type Integer) (bFromSweep :type Boolean) (SweepResult :type Hit%20Result%20Structure%20%28by%20ref%29))
  (Utilities|FlowControl|DoOnce false
    (:Completed
      (bind _asbp_reckless_rock (Utilities|Casting|CastToBP_RecklessRock (Variables|/Script/Engine.ChildActorComponent|GetChildActor (Variables|Default|GetBP_RecklessRock))))
      (Default|Breakless _asbp_reckless_rock))))

(event EventBeginPlay
  (bind _spawner_cornerarrow_l (Variables|Default|GetSpawner_CornerArrow_L))
  (bind _spawner_walllimit (Variables|Default|GetSpawner_WallLimit))
  (bind _ps_fumigene (Variables|Default|GetPS_Fumigene))
  (bind _returnvalue (Transformation|GetWorldTransform _spawner_walllimit))
  (bind _returnvalue_2 (Transformation|GetWorldTransform _spawner_cornerarrow_l))
  ;[0 1 0.1435] BEGIN
  (Variables|/Script/Engine.ParticleSystemComponent|SetInstanceParameters (Variables|Default|GetPS_Fumigene) (Utilities|Array|MakeArray (Utilities|Struct|MakeParticleSysParam "Color" "PSPT_Vector" 0.0 0.0 (Math|Conversions|ToVector(LinearColor) "(R=0.251264,G=0.715000,B=0.000000,A=1.000000)"))))
  ;[1 1 1] Duplicate crade
  (if (Math|Random|RandomBoolwithWeight 0.5)
    (if (< (Math|Vector|DotProduct (Math|Vector|GetUpVector (Variables|Default|GetPS_Fumigene)) (Math|Vector|MakeVector 0.0 0.0 1.0)) 0.75)
      (Components|DestroyComponent _ps_fumigene :!label _label)
      (else
        (Transformation|SetWorldRotation _ps_fumigene "0, 0, 0" false false)))
    (else
      (goto _label)))
  ;[1 1 1] ISMBank REF
  (bind _outactors (Actor|GetAllActorsOfClass "/Game/Gameplay/Roads/Blueprints/BP_ISMBank.BP_ISMBank_C"))
  (Utilities|IsValid (Utilities|Array|Get(acopy) _outactors)
    (:Is%20Valid
      (Variables|Default|SetBP_ISMBank_REF (Utilities|Array|Get(acopy) _outactors))
      (Utilities|FlowControl|Sequence
        (:then_0
          (for _array_element (Utilities|Array|MakeArray (Variables|Default|GetFence2) (Variables|Default|GetFence1) (Variables|Default|GetFence3))
            (bind _asarrow_component (Utilities|Casting|CastToArrowComponent _array_element))
            (Variables|Default|SetArrowComp _asarrow_component)
            ;[1 1 1] Fence
            (if (Components|ComponentHasTag (Variables|Default|GetArrowComp) "Spawner_Fence")
              (Components|InstancedStaticMesh|AddInstance (Variables|/Game/Gameplay/Roads/Blueprints/BP_ISMBank.BP_ISMBank_C|GetISM_Fence (Variables|Default|GetBP_ISMBank_REF)) (Math|Transform|MakeTransform (.location (Transformation|GetWorldTransform (Variables|Default|GetArrowComp))) (.rotation (Transformation|GetWorldTransform (Variables|Default|GetArrowComp))) "1,1,1"))
              (Variables|Default|SetISM_Fence (+ (Variables|Default|GetISM_Fence) 1)))))
        (:then_1
          ;[1 1 1] CornerArrow
          (Variables|Default|SetChosenArrow (select (> (Variables|/Game/Bikes/BP_Bike_Parent.BP_Bike_Parent_C|GetSpeedWithFactor (.AsBP%20Bike%20Parent (Utilities|Casting|CastToBP_Bike_Parent (Game|Player|GetPlayerPawn 0)))) 5e+02) 2 (Utilities|Select :Index (Variables|/Game/Base/Blueprints/BP_GamemodeRun.BP_GamemodeRun_C|GetCornerArrowType (.AsBP%20Gamemode%20Run (Utilities|Casting|CastToBP_GamemodeRun (Game|GetGameMode)))) :Option%200 0 :Option%201 1)))
          (Components|InstancedStaticMesh|AddInstance (Utilities|Select :Index (Variables|Default|GetChosenArrow) :Option%200 (Variables|/Game/Gameplay/Roads/Blueprints/BP_ISMBank.BP_ISMBank_C|GetISM_CornerArrow_L_Normal (Variables|Default|GetBP_ISMBank_REF)) :Option%201 (Variables|/Game/Gameplay/Roads/Blueprints/BP_ISMBank.BP_ISMBank_C|GetISM_CornerArrow_L_Circle (Variables|Default|GetBP_ISMBank_REF)) :Option%202 (Variables|/Game/Gameplay/Roads/Blueprints/BP_ISMBank.BP_ISMBank_C|GetISM_CornerArrow_L_Big (Variables|Default|GetBP_ISMBank_REF))) (Math|Transform|MakeTransform (+ (+ (.location _returnvalue_2) (* (Math|Vector|GetUpVector (Variables|Default|GetISM)) (Utilities|Select :Index (Variables|Default|GetChosenArrow) :Option%200 3.5e+02 :Option%201 3.5e+02 :Option%202 0.0))) (* (Math|Vector|GetForwardVector _spawner_cornerarrow_l) (Utilities|Select :Index (Variables|Default|GetChosenArrow) :Option%200 6.5e+02 :Option%201 7e+02 :Option%202 4.9e+02))) (.rotation _returnvalue_2) (Utilities|Select :Index (Variables|Default|GetChosenArrow) :Option%200 "1.500000,1.500000,1.500000" :Option%201 "1.750000,1.750000,1.750000" :Option%202 "3.050000,3.050000,3.050000")))
          (Variables|Default|SetISM_CornerArrow_L (+ (Variables|Default|GetISM_CornerArrow_L) 1)))
        (:then_2
          ;[1 1 1] WallLimit
          (Components|InstancedStaticMesh|AddInstance (Variables|/Game/Gameplay/Roads/Blueprints/BP_ISMBank.BP_ISMBank_C|GetISM_WallLimit (Variables|Default|GetBP_ISMBank_REF)) (Math|Transform|MakeTransform (.location _returnvalue) (.rotation _returnvalue) "0.500000,1,0.500000"))
          (Variables|Default|SetISM_WallLimit (+ (Variables|Default|GetISM_WallLimit) 1)))))
    (:Is%20Not%20Valid
      (Development|PrintString "Road_Parent: Il n'y a pas de BP_ISMBank dans la scene ! NEED" true true "(R=1.000000,G=0.004775,B=0.000000,A=1.000000)" 999.0))))

(event EventEndPlay
  (params (EndPlayReason :type EEndPlayReason%20Enum :default "Destroyed"))
  (bind _bp_ismbank_ref (Variables|Default|GetBP_ISMBank_REF))
  ;[0.176 1 0] END
  ;[1 1 1] ISM remove
  (for _index (range 1 (Variables|Default|GetISM_Fence))
    (Class|InstancedStaticMeshComponent|RemoveInstance (Variables|/Game/Gameplay/Roads/Blueprints/BP_ISMBank.BP_ISMBank_C|GetISM_Fence (Variables|Default|GetBP_ISMBank_REF))))
  (for _index_2 (range 1 (Variables|Default|GetISM_CornerArrow_L))
    (Class|InstancedStaticMeshComponent|RemoveInstance (Utilities|Select :Index (Variables|Default|GetChosenArrow) :Option%200 (Variables|/Game/Gameplay/Roads/Blueprints/BP_ISMBank.BP_ISMBank_C|GetISM_CornerArrow_L_Normal _bp_ismbank_ref) :Option%201 (Variables|/Game/Gameplay/Roads/Blueprints/BP_ISMBank.BP_ISMBank_C|GetISM_CornerArrow_L_Circle _bp_ismbank_ref) :Option%202 (Variables|/Game/Gameplay/Roads/Blueprints/BP_ISMBank.BP_ISMBank_C|GetISM_CornerArrow_L_Big _bp_ismbank_ref))))
  (for _index_3 (range 1 (Variables|Default|GetISM_WallLimit))
    (Class|InstancedStaticMeshComponent|RemoveInstance (Variables|/Game/Gameplay/Roads/Blueprints/BP_ISMBank.BP_ISMBank_C|GetISM_WallLimit (Variables|Default|GetBP_ISMBank_REF)))))

(fn ConstructionScript
  (|CallParentFunction))