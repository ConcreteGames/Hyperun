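; Small right-hand corner cone that sets up corner audio feedback and a breakable rock child actor.
; On BeginPlay it flags the CornerFeedback sound actor as right-side and tints its particle system magenta.
; The particles survive only on a 50% roll when near upright, then get zeroed world rotation; otherwise they are destroyed.
; The first capsule overlap calls Breakless on the BP_RecklessRock child.
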(event OnComponentBeginOverlap(Capsule)
  (params (OverlappedComponent :type Primitive%20Component%20Object%20Reference) (OtherActor :type Actor%20Object%20Reference) (OtherComp :type Primitive%20Component%20Object%20Reference) (OtherBodyIndex :type Integer) (bFromSweep :type Boolean) (SweepResult :type Hit%20Result%20Structure%20%28by%20ref%29))
  (Utilities|FlowControl|DoOnce false
    (:Completed
      (bind _asbp_reckless_rock (Utilities|Casting|CastToBP_RecklessRock (Variables|/Script/Engine.ChildActorComponent|GetChildActor (Variables|Default|GetBP_RecklessRock))))
      (Default|Breakless _asbp_reckless_rock))))

(event Custom|Corner%20Sound
  (bind _asbp_sfx_corner_sound (Utilities|Casting|CastToBP_SFX_CornerSound (Variables|/Script/Engine.ChildActorComponent|GetChildActor (Variables|Default|GetCorner%20Feedback))))
  (Variables|/Game/Sound/Blueprints/BP_SFX_CornerSound.BP_SFX_CornerSound_C|SetLeftOrRight _asbp_sfx_corner_sound 1.0)
  (Variables|/Game/Sound/Blueprints/BP_SFX_CornerSound.BP_SFX_CornerSound_C|SetIsLeft _asbp_sfx_corner_sound false))

(event EventBeginPlay
  (bind _particlesystem (Variables|Default|GetParticleSystem))
  (CallFunction|CornerSound)
  (Variables|/Script/Engine.ParticleSystemComponent|SetInstanceParameters (Variables|Default|GetParticleSystem) (Utilities|Array|MakeArray (Utilities|Struct|MakeParticleSysParam "Color" "PSPT_Vector" 0.0 0.0 (Math|Conversions|ToVector(LinearColor) "(R=0.765000,G=0.059670,B=0.623934,A=1.000000)"))))
  ;[1 1 1] Duplicate crade
  (if (Math|Random|RandomBoolwithWeight 0.5)
    (if (< (Math|Vector|DotProduct (Math|Vector|GetUpVector (Variables|Default|GetParticleSystem)) (Math|Vector|MakeVector 0.0 0.0 1.0)) 0.75)
      (Components|DestroyComponent _particlesystem :!label _label)
      (else
        (Transformation|SetWorldRotation _particlesystem "0, 0, 0" false false)))
    (else
      (goto _label))))

(event Collision|EventActorBeginOverlap
  (params (OtherActor :type Actor%20Object%20Reference)))

(event EventTick
  (params (DeltaSeconds :type Float%20%28single-precision%29)))

(fn ConstructionScript
  (|CallParentFunction))