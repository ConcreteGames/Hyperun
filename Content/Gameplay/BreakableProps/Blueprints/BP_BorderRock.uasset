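; BP_BorderRock is a breakable border prop, either a rock or a red sign, drawn through the shared BP_ISMBank instanced meshes.
; On BeginPlay it adds its instance to the bank, randomizing rotation and scale for rocks.
; KillMe runs once, plays impact sound and particles if a bike broke it, then uses a tiny line trace to find the instance index.
; On a hit it removes that instance and expires the actor.
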(event Custom|KillMe
  (params (BrokeByBike :type Boolean))
  (bind _returnvalue (Transformation|GetActorLocation))
  ;[1 1 1] DoOnce
  (if (Variables|Default|GetEnable)
    (Variables|Default|SetEnable false)
    ;[1 0.5082 0] Sfx
    (if BrokeByBike
      (Class|FMODBlueprintStatics|PlayEvent2D "/Game/FMOD/Events/SFX/PROPS/SFX_PROPS_SideRocks.SFX_PROPS_SideRocks")
      (Effects|SpawnEmitterAttached "/Game/Coco/Lab/RecklessRock/PS_Impact.PS_Impact" (Variables|Default|GetDefaultSceneRoot) "None"))
    (bind (_outhit _returnvalue_2) (Collision|LineTraceByChannel (+ _returnvalue "0, 0,0.100000") _returnvalue "TraceTypeQuery5" false 0 "None"))
    (if _returnvalue_2
      (bind _outactors (Actor|GetAllActorsOfClass "/Game/Gameplay/Roads/Blueprints/BP_ISMBank.BP_ISMBank_C"))
      (Class|InstancedStaticMeshComponent|RemoveInstance (select (Variables|Default|GetNeedRedSign) (Variables|/Game/Gameplay/Roads/Blueprints/BP_ISMBank.BP_ISMBank_C|GetISM_RedSign (Utilities|Array|Get(acopy) _outactors)) (Variables|/Game/Gameplay/Roads/Blueprints/BP_ISMBank.BP_ISMBank_C|GetISM_Rock (Utilities|Array|Get(acopy) _outactors))) (.HitItem (Collision|BreakHitResult _outhit)))
      (Actor|SetLifeSpan 0.01))))

(event EventBeginPlay
  (bind _returnvalue (Transformation|GetActorTransform))
  (bind _outactors (Actor|GetAllActorsOfClass "/Game/Gameplay/Roads/Blueprints/BP_ISMBank.BP_ISMBank_C"))
  (if (Variables|Default|GetNeedRedSign)
    (Components|InstancedStaticMesh|AddInstance (Variables|/Game/Gameplay/Roads/Blueprints/BP_ISMBank.BP_ISMBank_C|GetISM_RedSign (Utilities|Array|Get(acopy) _outactors)) (Math|Transform|MakeTransform (.location _returnvalue) (.rotation _returnvalue) "0.500000,0.500000,0.500000"))
    (else
      (Components|InstancedStaticMesh|AddInstance (Variables|/Game/Gameplay/Roads/Blueprints/BP_ISMBank.BP_ISMBank_C|GetISM_Rock (Utilities|Array|Get(acopy) _outactors)) (Math|Transform|MakeTransform (Transformation|GetActorLocation) (Math|Random|RandomRotator false) (Math|Vector|MakeVector (Math|Random|RandomFloatinRange 0.25 1.0) (Math|Random|RandomFloatinRange 0.25 1.0) (Math|Random|RandomFloatinRange 0.25 1.0)))))))

(fn ConstructionScript)