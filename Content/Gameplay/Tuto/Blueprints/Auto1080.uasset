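; Tutorial trigger actor that automatically feeds strafe inputs to the bike, apparently to perform a 1080 trick.
; Any overlap with the AutoRight component drives the first BP_Bike_Parent found in the level, without checking the overlapping actor.
; It calls the bike's debug strafe press and release functions in a rapid alternating left-right sequence, spaced by short fixed delays.
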(event OnComponentBeginOverlap(AutoRight)
  (params (OverlappedComponent :type Primitive%20Component%20Object%20Reference) (OtherActor :type Actor%20Object%20Reference) (OtherComp :type Primitive%20Component%20Object%20Reference) (OtherBodyIndex :type Integer) (bFromSweep :type Boolean) (SweepResult :type Hit%20Result%20Structure%20%28by%20ref%29))
  (bind _outactors (Actor|GetAllActorsOfClass "/Game/Bikes/BP_Bike_Parent.BP_Bike_Parent_C"))
  (Default|DebugActionStrafeLeftPress (Utilities|Array|Get(acopy) _outactors))
  (Utilities|FlowControl|Delay 0.02)
  (Default|DebugActionStrafeLeftRelease (Utilities|Array|Get(acopy) _outactors))
  (Utilities|FlowControl|Delay 0.02)
  (Default|DebugActionStrafeRightPress (Utilities|Array|Get(acopy) _outactors))
  (Utilities|FlowControl|Delay 0.02)
  (Default|DebugActionStrafeRightRelease (Utilities|Array|Get(acopy) _outactors))
  (Utilities|FlowControl|Delay 0.02)
  (Default|DebugActionStrafeLeftPress (Utilities|Array|Get(acopy) _outactors))
  (Utilities|FlowControl|Delay 0.02)
  (Default|DebugActionStrafeLeftRelease (Utilities|Array|Get(acopy) _outactors))
  (Utilities|FlowControl|Delay 0.02)
  (Default|DebugActionStrafeRightPress (Utilities|Array|Get(acopy) _outactors))
  (Utilities|FlowControl|Delay 0.02)
  (Default|DebugActionStrafeRightRelease (Utilities|Array|Get(acopy) _outactors))
  (Utilities|FlowControl|Delay 0.02)
  (Default|DebugActionStrafeLeftPress (Utilities|Array|Get(acopy) _outactors))
  (Utilities|FlowControl|Delay 0.02)
  (Default|DebugActionStrafeLeftRelease (Utilities|Array|Get(acopy) _outactors))
  (Utilities|FlowControl|Delay 0.02)
  (Default|DebugActionStrafeRightPress (Utilities|Array|Get(acopy) _outactors))
  (Utilities|FlowControl|Delay 0.02)
  (Default|DebugActionStrafeRightRelease (Utilities|Array|Get(acopy) _outactors)))

(fn ConstructionScript)