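; BP_TutoDoor is a tutorial checkpoint door that validates once, on the first overlap with its collision.
; Validation turns its meshes green, plays a 2D sound, and decrements the remaining door count on the first BP_Road_TutoFloor2 found in the level.
; The construction script shows one random child of Visual and sets flags on its child-actor collectible.
; A leftover F-key debug input triggers only the validation feedback.
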(event OnComponentBeginOverlap(Coll)
  (params (OverlappedComponent :type Primitive%20Component%20Object%20Reference) (OtherActor :type Actor%20Object%20Reference) (OtherComp :type Primitive%20Component%20Object%20Reference) (OtherBodyIndex :type Integer) (bFromSweep :type Boolean) (SweepResult :type Hit%20Result%20Structure%20%28by%20ref%29))
  (if (not (Variables|Default|GetIsValidated))
    (Variables|Default|SetIsValidated true)
    (CallFunction|ValidateDoor)
    (bind _outactors (Actor|GetAllActorsOfClass "/Game/Gameplay/Tuto/Blueprints/BP_Road_TutoFloor2.BP_Road_TutoFloor2_C"))
    (Default|RemoveOneDoortoValidate (Utilities|Array|Get(acopy) _outactors))))

(event EventBeginPlay)

(event Collision|EventActorBeginOverlap
  (params (OtherActor :type Actor%20Object%20Reference)))

(event EventTick
  (params (DeltaSeconds :type Float%20%28single-precision%29)))

(event Input|KeyboardEvents|F
  (params (Key :type Key%20Structure :default "AnyKey"))
  (:Pressed
    (Development|PrintString "Hello")
    (CallFunction|ValidateDoor)))

(fn ConstructionScript
  (bind _visual (Variables|Default|GetVisual))
  (bind _children (Components|GetChildrenComponents _visual false))
  ;[1 1 1] random half tire visual
  (Rendering|SetVisibility _children false false)
  (Rendering|SetVisibility (Utilities|Array|Get(acopy) _children (Math|Random|RandomIntegerinRange 0 (Utilities|Array|LastIndex _children))) true false)
  ;[1 1 1] Set collectible visible and pickable
  (bind _asbp_collectible_parent (Utilities|Casting|CastToBP_Collectible_Parent (Variables|/Script/Engine.ChildActorComponent|GetChildActor (Variables|Default|GetBP_Collectible))))
  (Variables|/Game/Gameplay/Collectibles/BP_Collectible_Parent.BP_Collectible_Parent_C|SetIsIvisibleAtStart _asbp_collectible_parent true)
  (Variables|/Game/Gameplay/Collectibles/BP_Collectible_Parent.BP_Collectible_Parent_C|SetIsEnable _asbp_collectible_parent true))

(fn ValidateDoor
  (Rendering|Material|SetMaterial (Variables|Default|GetStaticMesh) 0 "/Game/Base/Materials/M_green.M_Green")
  (Class|FMODBlueprintStatics|PlayEvent2D "/Game/FMOD/Events/VOICES/Tuto/SFX_TutoDoor.SFX_TutoDoor"))