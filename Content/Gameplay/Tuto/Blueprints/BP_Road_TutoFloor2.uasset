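; Tutorial road floor piece whose set of doors gates progress to the next tutorial step.
; BringDoors runs a one-second timeline that raises the Doors component from below the floor into place.
; The construction script derives the door count from Doors' children, minus one to offset an unexplained extra.
; RemoveOneDoorToValidate decrements that count and, at zero, tells BP_GamemodeRun to play the next step, only once.
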(event Custom|BringDoors
  (bind _doors (Variables|Default|GetDoors))
  (Components|Timeline|SetTimelineLength (Variables|Default|GetDoorsInDuration) 1.0)
  (Timeline|DoorsInDuration Play
    (:Update
      (bind _percentage (CallFunction|GetTimelinePercentage (Variables|Default|GetDoorsInDuration)))
      (Transformation|SetRelativeLocation _doors (Math|Vector|MakeVector 0.0 0.0 (* (- 1.0 _percentage) -1.5e+03)) false false))
    (:Finished
      (Transformation|SetRelativeLocation _doors (Math|Vector|MakeVector 0.0 0.0 0.0) false false))))

(event EventDynamicCreation)

(fn ConstructionScript
  (|CallParentFunction)
  (CallFunction|SetNumberOfDoors))

(fn RemoveOneDoortoValidate
  (bind _output_get (Variables|Default|SetNumberOfDoors (- (Variables|Default|GetNumberOfDoors) 1)))
  (if (< _output_get 1)
    (if (not (Variables|Default|GetNextPhase))
      (Variables|Default|SetNextPhase true)
      ;[1 1 1] Next tuto step
      (bind _asbp_gamemode_run (Utilities|Casting|CastToBP_GamemodeRun (Game|GetGameMode)))
      (Default|PlayNextTutoStep _asbp_gamemode_run))))

(fn SetNumberOfDoors
  (Variables|Default|SetNumberOfDoors (- (Class|SceneComponent|GetNumChildrenComponents (Variables|Default|GetDoors)) 1)))