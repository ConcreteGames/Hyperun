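; BP_Road_3x3_Tube_In is a road tile that randomizes its look in the construction script.
; It hides every child of Visual in game, then unhides one at random as the road variant.
; Each child of Rocks gets a random position along X, a random side on Y, random rotation and non-uniform random scale.
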(fn ConstructionScript
  (bind _returnvalue (Math|Random|RandomFloatinRange 0.4 1.0))
  (bind _visual (Variables|Default|GetVisual))
  (bind _children (Components|GetChildrenComponents _visual false))
  ;[1 1 1] Show random road
  (Development|SetHiddeninGame _children true false)
  (Development|SetHiddeninGame (Utilities|Array|Get(acopy) _children (Math|Random|RandomIntegerinRange 0 (Utilities|Array|LastIndex _children))) false false)
  ;[1 1 1] Place rocks
  (for _array_element (Components|GetChildrenComponents (Variables|Default|GetRocks) false)
    (Transformation|SetRelativeLocationAndRotation _array_element (Math|Vector|MakeVector (Math|Random|RandomFloatinRange 0.0 1.5e+03) (select (Math|Random|RandomBool) 7.5e+02 -7.5e+02) 0.0) (Math|Random|RandomRotator false) false false)
    (Transformation|SetRelativeScale3D _array_element (Math|Vector|MakeVector _returnvalue _returnvalue _returnvalue))))