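; Road tile Blueprint (in an old tiles folder) that builds a tube from child-actor segments, called "frites", at construction time.
; The construction script shifts the Tube to re-center its corner pivot, then walks all its descendant components.
; Segments up to the needed count get the same relative offset and a roll step of 360° divided by that count, with alternating two-shade materials.
; Surplus segments are hidden.
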(fn ConstructionScript
  (Transformation|AddRelativeLocation (Variables|Default|GetTube) "0.000000,-50.000000, 0" false false) ; On le décale de sa propre largeur\npour que le tube soit bien centré\ncar son point de pivot est dans le coin\net pas au milieu comme avant
  (for _array_element (Components|GetChildrenComponents (Variables|Default|GetTube) true)
    (bind _aschild_actor_component (Utilities|Casting|CastToChildActorComponent _array_element))
    (Variables|Default|SetFriteID (+ (Variables|Default|GetFriteID) 1))
    (if (<= (Variables|Default|GetFriteID) (Variables|Default|GetNumberOfFritesNeeded))
      ;[1 1 1] Set location, rotation and color
      (Rendering|SetVisibility _aschild_actor_component true true)
      (Transformation|SetRelativeLocationAndRotation _aschild_actor_component (Math|Vector|MakeVector 0.0 1e+02 0.0) (Math|Rotator|MakeRotator (* (/ 3.6e+02 (Math|Conversions|ToFloat(Integer) (Variables|Default|GetNumberOfFritesNeeded))) -1.0) 0.0 0.0) false false)
      (bind _asmesh_component (Utilities|Casting|CastToMeshComponent (Components|GetChildComponent (Components|GetChildComponent _aschild_actor_component 0) 0)))
      (Rendering|Material|SetMaterial _asmesh_component 0 (select (Variables|Default|GetIsColor1) "/Game/Coco/M_Road_Shade4.M_Road_Shade4" "/Game/Coco/M_Road_Shade1.M_Road_Shade1"))
      (Variables|Default|SetIsColor1 (select (Variables|Default|GetIsColor1) false true)) ; Switch
      (else
        ;[1 1 1] Hide the nonused frite
        (Rendering|SetVisibility _aschild_actor_component false true)))))