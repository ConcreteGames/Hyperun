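; Legacy 3x1 road tile Blueprint that randomizes which road visual it shows.
; Its construction script hides all direct children of the Visual component, then unhides one at a random index, so the pick can change whenever the script reruns.
; A disconnected graph section, which never runs, would scatter the Rocks children to either side with random rotation and non-uniform scale.
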(fn ConstructionScript
  (bind _visual (Variables|Default|GetVisual))
  (bind _children (Components|GetChildrenComponents _visual false))
  ;[1 1 1] Show random road
  (Development|SetHiddeninGame _children true false)
  (Development|SetHiddeninGame (Utilities|Array|Get(acopy) _children (Math|Random|RandomIntegerinRange 0 (Utilities|Array|LastIndex _children))) false false))