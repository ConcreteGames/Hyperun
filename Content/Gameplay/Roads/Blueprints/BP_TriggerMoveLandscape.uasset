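; Trigger placed in the road run that shifts the landscape and marks the end of a big jump or tunnel road section.
; On first box overlap it disables its collision, finds the BP_LandscapeManager, then calls MoveLandscape and SpawnActorEvent on it.
; It then clears the jump/tunnel lock on BP_GamemodeRun and spawns the following road pool, or logs an error if no landscape manager exists.
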(event OnComponentBeginOverlap(BoxTrigger)
  (params (OverlappedComponent :type Primitive%20Component%20Object%20Reference) (OtherActor :type Actor%20Object%20Reference) (OtherComp :type Primitive%20Component%20Object%20Reference) (OtherBodyIndex :type Integer) (bFromSweep :type Boolean) (SweepResult :type Hit%20Result%20Structure%20%28by%20ref%29))
  (bind _returnvalue (Game|GetGameMode))
  (bind _asbp_gamemode_run (Utilities|Casting|CastToBP_GamemodeRun _returnvalue))
  ;[1 1 1] DoOnce
  (Collision|SetCollisionEnabled (Variables|Default|GetBoxTrigger) "NoCollision")
  (bind _outactors (Actor|GetAllActorsOfClass "/Game/Coco/Lab/Landscape/BP_LandscapeManager.BP_LandscapeManager_C"))
  (Utilities|IsValid (Utilities|Array|Get(acopy) _outactors)
    (:Is%20Valid
      (Default|MoveLandscape (Utilities|Array|Get(acopy) _outactors))
      (Default|SpawnActorEvent (Utilities|Array|Get(acopy) _outactors))
      ;[1 1 1] End of roads buffer
      (Variables|/Game/Base/Blueprints/BP_GamemodeRun.BP_GamemodeRun_C|SetBigJumpOrTunnelLockLD _asbp_gamemode_run false)
      (Default|SpawnRoadsPoolAfterJumporTunnel _asbp_gamemode_run))
    (:Is%20Not%20Valid
      (CallFunction|LogErerror "THERE'S NO LANDSCAPE IN SCENE... NEEEEEEEEEED!"))))

(fn ConstructionScript)