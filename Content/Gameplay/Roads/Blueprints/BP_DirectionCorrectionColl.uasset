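; BP_DirectionCorrectionColl is a road trigger volume that corrects a bike's direction when it is overlapped.
; Its collision turns on 0.2 seconds after BeginPlay, then turns off on the first overlap, making it one-shot.
; It then calls DirectionCorrection on the overlapping BP_Bike_Parent, passing its own component and marking the bike as not on a curve.
; Overlaps are ignored and logged when the actor sits at world origin.
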(event OnComponentBeginOverlap(DirectionCorrectionColl)
  (params (OverlappedComponent :type Primitive%20Component%20Object%20Reference) (OtherActor :type Actor%20Object%20Reference) (OtherComp :type Primitive%20Component%20Object%20Reference) (OtherBodyIndex :type Integer) (bFromSweep :type Boolean) (SweepResult :type Hit%20Result%20Structure%20%28by%20ref%29))
  ;[1 1 1] Secu 2
  (if (Math|Vector|NotEqual(Vector) (Transformation|GetActorLocation) "0, 0, 0" 0.0001)
    ;[1 1 1] DoOnce
    (Collision|SetCollisionEnabled (Variables|Default|GetDirectionCorrectionColl) "NoCollision")
    (bind _asbp_bike_parent (Utilities|Casting|CastToBP_Bike_Parent OtherActor))
    (Default|DirectionCorrection _asbp_bike_parent (Variables|Default|GetDirectionCorrectionColl) false)
    (else
      (CallFunction|LogErerror "OutColl is on 0,0,0 so I don't kill it."))))

(event EventBeginPlay
  ;[1 1 1] Secu 1
  (Utilities|FlowControl|Delay 0.2)
  (Collision|SetCollisionEnabled (Variables|Default|GetDirectionCorrectionColl) "QueryOnly"))

(fn ConstructionScript)