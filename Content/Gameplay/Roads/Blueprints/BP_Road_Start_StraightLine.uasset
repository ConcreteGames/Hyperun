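; BP_Road_Start_StraightLine is a straight starting road piece that randomizes its scenery in the Construction Script.
; Unless TRP is replaying, it rolls a ±1 side, stored in TRPProceduralCurve, to mirror EtherPatterns on Y.
; It scatters grass children along X with random yaw and scale, and fills ISMSpawnersArray with arrow components.
; A rare weighted roll assigns BP_Dragon to the Dragon child actor.
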(fn ConstructionScript
  (bind _returnvalue (Math|Random|RandomFloatinRange 0.5 1.5))
  (|CallParentFunction)
  (Utilities|FlowControl|Sequence
    (:then_0
      ;[1 1 1] TRP, if not 0, keep the given value
      (bind _trp_replaying (CallFunction|TRPTestifTRPandGetRoadValues))
      (if _trp_replaying
        _
        (else
          (Variables|Default|SetTRP_ProceduralCurve (Math|Rotator|MakeRotator (select (Math|Random|RandomBool) 1.0 -1.0) 0.0 0.0))))
      ;[1 1 1] Random side of patterns
      (Transformation|SetRelativeScale3D (Variables|Default|GetEtherPatterns) (Math|Vector|MakeVector 1.0 (.roll (Variables|Default|GetTRP_ProceduralCurve)) 1.0)))
    (:then_1
      ;[1 1 1] Grass
      (for _array_element (Components|GetChildrenComponents (Variables|Default|GetGrass) false)
        (Transformation|SetRelativeTransform _array_element (Math|Transform|MakeTransform (Math|Vector|MakeVector (Math|Random|RandomFloatinRange 0.0 7e+03) (.y (.location (Transformation|GetRelativeTransform _array_element))) (.z (.location (Transformation|GetRelativeTransform _array_element)))) (Math|Rotator|MakeRotator (.roll (.rotation (Transformation|GetRelativeTransform _array_element))) (.pitch (.rotation (Transformation|GetRelativeTransform _array_element))) (Math|Random|RandomFloatinRange 0.0 3.6e+02)) (Math|Vector|MakeVector _returnvalue _returnvalue _returnvalue)) false false)))
    (:then_2
      (Variables|Default|SetISMSpawnersArray (Utilities|Array|MakeArray (Variables|Default|GetArrow1) (Variables|Default|GetArrow2) (Variables|Default|GetArrow3) (Variables|Default|GetArrow4) (Variables|Default|GetArrow) (Variables|Default|GetArrow5) (Variables|Default|GetArrow21) (Variables|Default|GetArrow22) (Variables|Default|GetArrow23) (Variables|Default|GetArrow24) (Variables|Default|GetArrow25) (Variables|Default|GetArrow33) (Variables|Default|GetArrow34) (Variables|Default|GetArrow35) (Variables|Default|GetArrow36) (Variables|Default|GetArrow37) (Variables|Default|GetArrow38) (Variables|Default|GetArrow39) (Variables|Default|GetArrow40) (Variables|Default|GetArrow41) (Variables|Default|GetArrow42) (Variables|Default|GetArrow43) (Variables|Default|GetArrow44) (Variables|Default|GetArrow45) (Variables|Default|GetArrow46) (Variables|Default|GetArrow47) (Variables|Default|GetArrow48) (Variables|Default|GetArrow49) (Variables|Default|GetArrow50) (Variables|Default|GetArrow51) (Variables|Default|GetArrow52) (Variables|Default|GetArrow56) (Variables|Default|GetArrow57) (Variables|Default|GetArrow58) (Variables|Default|GetArrow59) (Variables|Default|GetArrow55) (Variables|Default|GetArrow60) (Variables|Default|GetArrow61) (Variables|Default|GetArrow63) (Variables|Default|GetArrow64) (Variables|Default|GetArrow65) (Variables|Default|GetArrow66) (Variables|Default|GetArrow67) (Variables|Default|GetArrow68) (Variables|Default|GetArrow62) (Variables|Default|GetArrow69))))
    (:then_3
      (if (Math|Random|RandomBoolwithWeight 0.02)
        (ChildActorComponent|SetChildActorClass (Variables|Default|GetDragon) "/Game/Coco/Lab/Props/NearProps/Dragon/BP_Dragon.BP_Dragon_C")))))