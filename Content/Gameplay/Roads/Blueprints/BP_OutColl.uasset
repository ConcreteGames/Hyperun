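; BP_OutColl is a one-shot exit trigger for a road piece, enabled as query-only shortly after spawn.
; On first overlap it disables its collision, notifies its BP_Road_Parent and destroys itself almost immediately.
; An overlapping BP_Bike_Parent also receives a straight-road direction correction using this collider.
; As a safeguard, overlaps while it sits at the world origin are only logged and leave it alive.
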(event OnComponentBeginOverlap(OutColl)
  (params (OverlappedComponent :type Primitive%20Component%20Object%20Reference) (OtherActor :type Actor%20Object%20Reference) (OtherComp :type Primitive%20Component%20Object%20Reference) (OtherBodyIndex :type Integer) (bFromSweep :type Boolean) (SweepResult :type Hit%20Result%20Structure%20%28by%20ref%29))
  ;[1 1 1] Secu 2
  (if (Math|Vector|NotEqual(Vector) (Transformation|GetActorLocation) "0, 0, 0" 0.0001)
    ;[1 1 1] DoOnce
    (Collision|SetCollisionEnabled (Variables|Default|GetOutColl) "NoCollision")
    (Utilities|FlowControl|Sequence
      (:then_0
        (bind _asbp_road_parent (Utilities|Casting|CastToBP_Road_Parent (Variables|Default|GetRoadParent))
          (:then
            (Default|OutCollBeginOverlap _asbp_road_parent)
            (Actor|SetLifeSpan 0.001))
          (:CastFailed
            (CallFunction|LogErerror "BP_OUTRoadColl: My parent is not a \"BP_Road_Parent\""))))
      (:then_1
        (bind _asbp_bike_parent (Utilities|Casting|CastToBP_Bike_Parent OtherActor))
        (Default|DirectionCorrection _asbp_bike_parent (Variables|Default|GetOutColl) false)))
    (else
      (CallFunction|LogErerror "OutColl is on 0,0,0 so I don't kill it."))))

(event EventBeginPlay
  ;[1 1 1] Secu 1
  (Utilities|FlowControl|Delay 0.2)
  (Collision|SetCollisionEnabled (Variables|Default|GetOutColl) "QueryOnly"))

(fn ConstructionScript)