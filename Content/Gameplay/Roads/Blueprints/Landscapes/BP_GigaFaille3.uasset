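; BP_GigaFaille3 is a road landscape piece forming a rift between left and right rock walls, with a gap that depends on bike speed.
; On BeginPlay, it samples a curve with the player bike's SpeedWithFactor and offsets both sides symmetrically in Y, without later updates.
; The construction script shows one random child visual per side and sets the prop type on its child woosh SFX actor.
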(event EventBeginPlay
  (bind _returnvalue (Game|Player|GetPlayerPawn 0))
  (bind _crv_riftgapbyspeed (Variables|Default|GetCRV_RiftGapBySpeed))
  (bind _asbp_bike_parent (Utilities|Casting|CastToBP_Bike_Parent _returnvalue))
  (bind _speedwithfactor (Variables|/Game/Bikes/BP_Bike_Parent.BP_Bike_Parent_C|GetSpeedWithFactor _asbp_bike_parent))
  (bind _returnvalue_2 (Math|Curves|GetFloatValue _crv_riftgapbyspeed _speedwithfactor))
  ;[1 1 1] Dynamic rift gap by speed
  (Transformation|SetRelativeLocation (Variables|Default|GetOffset_L) (Math|Vector|MakeVector 0.0 (* _returnvalue_2 -1.0) 0.0) false false)
  (Transformation|SetRelativeLocation (Variables|Default|GetOffset_R) (Math|Vector|MakeVector 0.0 _returnvalue_2 0.0) false false))

(fn ConstructionScript
  (bind _visual_l (Variables|Default|GetVisual_L))
  (bind _visual_r (Variables|Default|GetVisual_R))
  (bind _children (Components|GetChildrenComponents _visual_r false))
  (bind _children_2 (Components|GetChildrenComponents _visual_l false))
  ;[1 1 1] Random rock visual
  (Development|SetHiddeninGame _children_2 true false)
  (Development|SetHiddeninGame (Utilities|Array|Get(acopy) _children_2 (Math|Random|RandomIntegerinRange 0 (Utilities|Array|LastIndex _children_2))) false false)
  (Development|SetHiddeninGame _children true false)
  (Development|SetHiddeninGame (Utilities|Array|Get(acopy) _children (Math|Random|RandomIntegerinRange 0 (Utilities|Array|LastIndex _children))) false false)
  (bind _asbp_sfx_wooshs_near_props_a (Utilities|Casting|CastToBP_SFX_WooshsNearPropsA (Variables|/Script/Engine.ChildActorComponent|GetChildActor (Variables|Default|GetSfx_Woosh))))
  (Variables|/Game/Sound/Blueprints/BP_SFX_WooshsNearPropsA.BP_SFX_WooshsNearPropsA_C|SetPropsType _asbp_sfx_wooshs_near_props_a "NewEnumerator0"))