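; Level 1 road piece for a straight, sloped tunnel, built from "frite" child-actor tiles and arrow-based ISM spawners.
; The construction script registers both lists and moves the AttachPoint to the end of the last section.
; Vertex snapping of the frites waits until DynamicCreation, because a road nested in another road may have moved.
; A SetFrite helper, uncalled here, spaces child curve tiles with random roll and pitch.
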(event EventDynamicCreation
  ;[1 1 1] Je mets le Vertex Snap ici (et pas à la fin du contruction script)
  ; car j'ai besoin que la variable "MyPreviousFriteRotation" de chaque frite
  ; soit mise à jour après que la route dans la quelle elle est ait bougé.
  ;
  ; En effet, cette route peut être potentiellement "une road dans une road"
  ; avec le passage des MacroPatterns en roads, donc elle peut avoir été bougée !
  (CallFunction|RoadVertexSnap3 (Variables|Default|GetFrites)))

(fn ConstructionScript
  (bind _attachpoint (Variables|Default|GetAttachPoint))
  (|CallParentFunction)
  (Variables|Default|SetFrites (Utilities|Array|MakeArray (Variables|Default|Get1_Frite1) (Variables|Default|GetChildActor2) (Variables|Default|GetChildActor3) (Variables|Default|GetChildActor4) (Variables|Default|GetChildActor5) (Variables|Default|GetChildActor6) (Variables|Default|GetChildActor7) (Variables|Default|GetChildActor) (Variables|Default|GetChildActor1) (Variables|Default|GetChildActor8) (Variables|Default|GetChildActor9) (Variables|Default|GetChildActor10) (Variables|Default|GetChildActor11) (Variables|Default|GetChildActor12) (Variables|Default|GetChildActor13) (Variables|Default|GetChildActor14) (Variables|Default|GetChildActor15) (Variables|Default|GetChildActor16) (Variables|Default|GetChildActor17) (Variables|Default|GetChildActor18) (Variables|Default|GetChildActor19) (Variables|Default|GetChildActor20) (Variables|Default|GetChildActor21) (Variables|Default|GetChildActor22) (Variables|Default|GetChildActor23) (Variables|Default|GetLastFrite_1)))
  (Variables|Default|SetISMSpawnersArray (Utilities|Array|MakeArray (Variables|Default|GetArrow3) (Variables|Default|GetArrow4) (Variables|Default|GetArrow1) (Variables|Default|GetArrow6) (Variables|Default|GetArrow5) (Variables|Default|GetArrow2) (Variables|Default|GetArrow7) (Variables|Default|GetSpawner_TunnelInOut)))
  ;[1 1 1] On positionne l'Attach point à la fin de la dernière partie
  (Transformation|AttachComponentToComponent _attachpoint (Variables|Default|GetArrow6) "None" "KeepRelative" "KeepRelative" "KeepRelative" true)
  (Transformation|SetRelativeTransform _attachpoint (Math|Transform|MakeTransform "1500.000000, 0, 0" "0, 0, 0" "1,1,1") false false)
  (Transformation|SetWorldScale3D _attachpoint "1.000000,1.000000,1.000000"))

(fn SetFrite
  (params (FirstFrite :type Scene%20Component%20Object%20Reference) (RollMin :type Float%20%28single-precision%29) (RollMax :type Float%20%28single-precision%29) (PitchMin :type Float%20%28single-precision%29) (PitchMax :type Float%20%28single-precision%29))
  (for _array_element (Components|GetChildrenComponents FirstFrite true)
    (bind _aschild_actor_component (Utilities|Casting|CastToChildActorComponent _array_element))
    (Utilities|Casting|CastToBP_Tile_3x1_CurveFrite (Variables|/Script/Engine.ChildActorComponent|GetChildActor _aschild_actor_component))
    (LocalVariables|SetCurrentFrite _array_element)
    (Transformation|SetRelativeLocationAndRotation (LocalVariables|GetCurrentFrite) "300.000000, 0, 0" (Math|Rotator|MakeRotator (Math|Random|RandomFloatinRange RollMin RollMax) (Math|Random|RandomFloatinRange PitchMin PitchMax) 0.0) false false :!pinned true) ; 1st group of frites
  ))