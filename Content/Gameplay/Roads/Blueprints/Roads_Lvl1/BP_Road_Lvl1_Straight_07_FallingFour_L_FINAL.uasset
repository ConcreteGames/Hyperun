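; Level 1 road segment Blueprint, a straight "FallingFour" left variant built from arrow and spawner markers.
; Its construction script runs the parent's, fills the ISM spawner array and pins the AttachPoint past the end of the last part.
; It then has every curved "frite" tile child actor under Roads update its rotation.
; A SetFrite helper offsets a frite's child tiles with random roll and pitch, though the construction script never calls it.
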(fn ConstructionScript
  (bind _attachpoint (Variables|Default|GetAttachPoint))
  (|CallParentFunction)
  (Variables|Default|SetISMSpawnersArray (Utilities|Array|MakeArray (Variables|Default|GetSpawner_Corner_R3) (Variables|Default|GetSpawner_Corner_R4) (Variables|Default|GetArrow) (Variables|Default|GetArrow1) (Variables|Default|GetArrow2) (Variables|Default|GetArrow3) (Variables|Default|GetSpawner_Corner_R2) (Variables|Default|GetArrow7) (Variables|Default|GetArrow6) (Variables|Default|GetSpawner_Corner_R) (Variables|Default|GetArrow4) (Variables|Default|GetArrow5) (Variables|Default|GetSpawner_FallingFour_L) (Variables|Default|GetArrow8) (Variables|Default|GetArrow9) (Variables|Default|GetArrow10) (Variables|Default|GetArrow11) (Variables|Default|GetArrow12) (Variables|Default|GetArrow13) (Variables|Default|GetArrow14) (Variables|Default|GetArrow15) (Variables|Default|GetArrow16) (Variables|Default|GetArrow17) (Variables|Default|GetArrow18) (Variables|Default|GetArrow19) (Variables|Default|GetArrow20) (Variables|Default|GetArrow21) (Variables|Default|GetArrow22) (Variables|Default|GetArrow23) (Variables|Default|GetArrow56) (Variables|Default|GetArrow57) (Variables|Default|GetArrow58) (Variables|Default|GetArrow59) (Variables|Default|GetArrow60) (Variables|Default|GetArrow61) (Variables|Default|GetArrow62) (Variables|Default|GetArrow63) (Variables|Default|GetArrow64) (Variables|Default|GetArrow65) (Variables|Default|GetArrow66) (Variables|Default|GetArrow67) (Variables|Default|GetArrow68) (Variables|Default|GetArrow69) (Variables|Default|GetArrow70) (Variables|Default|GetArrow71) (Variables|Default|GetArrow24) (Variables|Default|GetArrow25) (Variables|Default|GetArrow26) (Variables|Default|GetArrow27) (Variables|Default|GetArrow28) (Variables|Default|GetArrow29) (Variables|Default|GetArrow30) (Variables|Default|GetArrow31) (Variables|Default|GetArrow32) (Variables|Default|GetArrow33) (Variables|Default|GetArrow34) (Variables|Default|GetArrow35) (Variables|Default|GetArrow36) (Variables|Default|GetArrow37) (Variables|Default|GetArrow38) (Variables|Default|GetArrow39) (Variables|Default|GetArrow40) (Variables|Default|GetArrow41) (Variables|Default|GetArrow42) (Variables|Default|GetArrow43) (Variables|Default|GetArrow44) (Variables|Default|GetArrow45) (Variables|Default|GetArrow46) (Variables|Default|GetArrow47) (Variables|Default|GetArrow48) (Variables|Default|GetArrow49) (Variables|Default|GetArrow50) (Variables|Default|GetArrow51) (Variables|Default|GetArrow52) (Variables|Default|GetArrow53) (Variables|Default|GetArrow54) (Variables|Default|GetArrow55)))
  ;[1 1 1] On positionne l'Attach point à la fin de la dernière partie
  (Transformation|AttachComponentToComponent _attachpoint (Variables|Default|GetArrow5) "None" "KeepRelative" "KeepRelative" "KeepRelative" true)
  (Transformation|SetRelativeTransform _attachpoint (Math|Transform|MakeTransform "1500.000000, 0, 0" "0, 0, 0" "1,1,1") false false)
  (Transformation|SetWorldScale3D _attachpoint "1.000000,1.000000,1.000000")
  ;[1 1 1] On met à jour toutes les frites de toutes les roads enfants
  (for _array_element (Components|GetChildrenComponents (Variables|Default|GetRoads) true)
    (bind _aschild_actor_component (Utilities|Casting|CastToChildActorComponent _array_element))
    (bind _asbp_tile_3x_1_curve_frite (Utilities|Casting|CastToBP_Tile_3x1_CurveFrite (Variables|/Script/Engine.ChildActorComponent|GetChildActor _aschild_actor_component)))
    (Default|UpdateMyRotation _asbp_tile_3x_1_curve_frite)))

(fn SetFrite
  (params (FirstFrite :type Scene%20Component%20Object%20Reference) (RollMin :type Float%20%28single-precision%29) (RollMax :type Float%20%28single-precision%29) (PitchMin :type Float%20%28single-precision%29) (PitchMax :type Float%20%28single-precision%29))
  (for _array_element (Components|GetChildrenComponents FirstFrite true)
    (bind _aschild_actor_component (Utilities|Casting|CastToChildActorComponent _array_element))
    (Utilities|Casting|CastToBP_Tile_3x1_CurveFrite (Variables|/Script/Engine.ChildActorComponent|GetChildActor _aschild_actor_component))
    (LocalVariables|SetCurrentFrite _array_element)
    (Transformation|SetRelativeLocationAndRotation (LocalVariables|GetCurrentFrite) "300.000000, 0, 0" (Math|Rotator|MakeRotator (Math|Random|RandomFloatinRange RollMin RollMax) (Math|Random|RandomFloatinRange PitchMin PitchMax) 0.0) false false :!pinned true) ; 1st group of frites
  ))