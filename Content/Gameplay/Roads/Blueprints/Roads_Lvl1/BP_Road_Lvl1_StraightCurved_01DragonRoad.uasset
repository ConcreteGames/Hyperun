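; Level 1 "Dragon Road" road piece that builds a randomly curved stretch from a series of child-actor segments.
; The construction script gives each segment the same offset and small random two-axis rotation, with AttachPoint placed beyond the last one.
; A TRP replay check skips re-randomizing the curve during replay.
; On DynamicCreation, the segment array (Frites) goes to RoadVertexSnap3.
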(event EventDynamicCreation
  (CallFunction|RoadVertexSnap3 (Variables|Default|GetFrites)))

(fn ConstructionScript
  (|CallParentFunction)
  (Variables|Default|SetFrites (Utilities|Array|MakeArray (Variables|Default|GetFirstRoad) (Variables|Default|GetChildActor) (Variables|Default|GetChildActor1) (Variables|Default|GetChildActor2) (Variables|Default|GetChildActor3) (Variables|Default|GetChildActor4) (Variables|Default|GetChildActor5) (Variables|Default|GetChildActor6) (Variables|Default|GetChildActor7) (Variables|Default|GetChildActor8) (Variables|Default|GetLAST)))
  (Transformation|AttachComponentToComponent (Variables|Default|GetAttachPoint) (Variables|Default|GetLAST) "None" "SnapToTarget" "SnapToTarget" "SnapToTarget" true)
  ;[1 1 1] random curve
  (bind _trp_replaying (CallFunction|TRPTestifTRPandGetRoadValues))
  (if _trp_replaying
    _
    (else
      (Variables|Default|SetTRP_ProceduralCurve (Math|Rotator|MakeRotator (Math|Random|RandomFloatinRange -4.0 4.0) (Math|Random|RandomFloatinRange -1.0 3.0) 0.0))))
  (Transformation|SetRelativeLocationAndRotation (Variables|Default|GetChildActor) "300.000000, 0, 0" (Variables|Default|GetTRP_ProceduralCurve) false false)
  (Transformation|SetRelativeLocationAndRotation (Variables|Default|GetAttachPoint) "300.000000, 0, 0" (Math|Rotator|MakeRotator 0.0 0.0 0.0) false false))