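; Level 1 straight road piece shaped as a sharp half-pipe, with per-instance procedural variation.
; Its Construction Script registers the ISM spawner components, then randomizes the side tilt and a two-way ether pattern unless a TRP replay is active.
; The left and right anchors roll in mirror image by that angle.
; The pattern swaps C1 and C2 between two positions along X.
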(fn ConstructionScript
  (bind _c1 (Variables|Default|GetC1))
  (bind _c2 (Variables|Default|GetC2))
  (bind _relativelocation (Variables|/Script/Engine.SceneComponent|GetRelativeLocation _c2))
  (bind _relativelocation_2 (Variables|/Script/Engine.SceneComponent|GetRelativeLocation _c1))
  (|CallParentFunction)
  (Variables|Default|SetISMSpawnersArray (Utilities|Array|MakeArray (Variables|Default|GetFL) (Variables|Default|GetFR) (Variables|Default|GetArrow21) (Variables|Default|GetArrow) (Variables|Default|GetArrow37) (Variables|Default|GetArrow28) (Variables|Default|GetArrow29) (Variables|Default|GetArrow30) (Variables|Default|GetArrow31) (Variables|Default|GetArrow32) (Variables|Default|GetArrow33) (Variables|Default|GetArrow34) (Variables|Default|GetArrow35) (Variables|Default|GetArrow36) (Variables|Default|GetArrow27) (Variables|Default|GetArrow41) (Variables|Default|GetArrow42) (Variables|Default|GetArrow43) (Variables|Default|GetArrow44) (Variables|Default|GetArrow45) (Variables|Default|GetArrow46) (Variables|Default|GetArrow47) (Variables|Default|GetArrow48) (Variables|Default|GetArrow49) (Variables|Default|GetSpawner_SharpPipe_R) (Variables|Default|GetSpawner_SharpPipe_L) (Variables|Default|GetSpawner_SharpPipe_Middle)))
  ;[1 1 1] random 1 float + 1 bool
  (bind _trp_replaying (CallFunction|TRPTestifTRPandGetRoadValues))
  (if _trp_replaying
    _
    (else
      (Variables|Default|SetTRP_ProceduralCurve (Math|Rotator|MakeRotator (Math|Random|RandomFloatinRange 2e+01 55.0) 0.0 0.0))
      (Variables|Default|SetTRP_EtherPattern (Math|Conversions|ToInteger(Boolean) (Math|Random|RandomBool)))))
  ;[1 1 1] roads tilt
  (Transformation|SetRelativeRotation (Variables|Default|GetAnchorRight) (Math|Rotator|MakeRotator (* (.roll (Variables|Default|GetTRP_ProceduralCurve)) -1.0) 0.0 0.0) false false)
  (Transformation|SetRelativeRotation (Variables|Default|GetAnchorLeft) (Math|Rotator|MakeRotator (.roll (Variables|Default|GetTRP_ProceduralCurve)) 0.0 0.0) false false)
  ;[1 1 1] ethers
  (Transformation|SetRelativeLocation _c1 (Math|Vector|MakeVector (select (Math|Conversions|ToBoolean(Integer) (Variables|Default|GetTRP_EtherPattern)) 1.05e+04 5.5e+03) (.y _relativelocation_2) (.z _relativelocation_2)) false false)
  (Transformation|SetRelativeLocation _c2 (Math|Vector|MakeVector (select (Math|Conversions|ToBoolean(Integer) (Variables|Default|GetTRP_EtherPattern)) 5.5e+03 1.05e+04) (.y _relativelocation) (.z _relativelocation)) false false))