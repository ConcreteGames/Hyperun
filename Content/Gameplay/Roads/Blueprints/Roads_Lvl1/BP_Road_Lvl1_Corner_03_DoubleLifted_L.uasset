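; Level 1 procedural road piece: a double-lifted corner (L variant) built from two chains of curved "frite" tile child actors.
; Construction randomizes one roll/pitch step unless a TRP replay is running, applying it along both chains to form the curve.
; It then positions the rough corner anchor, moves the AttachPoint to the second chain's end, refreshes tile rotations and registers ISM spawners.
; On DynamicCreation, both chains get their road vertices snapped.
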(event EventDynamicCreation
  (CallFunction|RoadVertexSnap3 (Variables|Default|GetFrites1))
  (CallFunction|RoadVertexSnap3 (Variables|Default|GetFrites2)))

(fn ConstructionScript
  (bind _attachpoint (Variables|Default|GetAttachPoint))
  (|CallParentFunction)
  (Variables|Default|SetFrites1 (Utilities|Array|MakeArray (Variables|Default|Get1_Frite1) (Variables|Default|GetChildActor2) (Variables|Default|GetChildActor3) (Variables|Default|GetChildActor4) (Variables|Default|GetChildActor5) (Variables|Default|GetChildActor6) (Variables|Default|GetChildActor7) (Variables|Default|Get1_LastFrite)))
  (Variables|Default|SetFrites2 (Utilities|Array|MakeArray (Variables|Default|Get2_Frite1) (Variables|Default|GetChildActor8) (Variables|Default|GetChildActor9) (Variables|Default|GetChildActor10) (Variables|Default|GetChildActor11) (Variables|Default|GetChildActor12) (Variables|Default|GetChildActor13) (Variables|Default|Get2_LastFrite)))
  (Utilities|FlowControl|Sequence
    (:then_0
      ;[1 1 1] random pitch
      (bind _trp_replaying (CallFunction|TRPTestifTRPandGetRoadValues))
      (if _trp_replaying
        _
        (else
          (Variables|Default|SetTRP_ProceduralCurve (Math|Rotator|MakeRotator (Math|Random|RandomFloatinRange (Variables|Default|GetFriteRollMin) (Variables|Default|GetFriteRollMax)) (Math|Random|RandomFloatinRange (Variables|Default|GetFritePitchMin) (Variables|Default|GetFritePitchMax)) 0.0))))
      (Transformation|SetRelativeLocationAndRotation (Variables|Default|GetChildActor2) "300.000000, 0, 0" (Variables|Default|GetTRP_ProceduralCurve) false false :!pinned true) ; 1st group of frites
      (Transformation|SetRelativeLocationAndRotation (Variables|Default|GetRoughCornerAnchor) "300.000000,0.000000, 0" (Math|Rotator|MakeRotator 0.0 0.0 0.0) false false :!pinned true) ; Snap Rough Corner
      (Transformation|SetRelativeLocationAndRotation (Variables|Default|GetChildActor8) "300.000000,0.000000, 0" (Variables|Default|GetTRP_ProceduralCurve) false false :!pinned true) ; 2nd group of frites
      ;[1 1 1] On positionne l'Attach point à la fin de la dernière partie
      (Transformation|AttachComponentToComponent _attachpoint (Variables|Default|Get2_LastFrite) "None" "KeepRelative" "KeepRelative" "KeepRelative" true)
      (Transformation|SetRelativeTransform _attachpoint (Math|Transform|MakeTransform "300.000000, 0, 0" "0, 0, 0" "1,1,1") false false)
      ;[1 1 1] On met à jour toutes les frites de toutes les roads enfants
      (for _array_element (Components|GetChildrenComponents (Variables|Default|GetRoads) true)
        (bind _aschild_actor_component (Utilities|Casting|CastToChildActorComponent _array_element))
        (bind _asbp_tile_3x_1_curve_frite (Utilities|Casting|CastToBP_Tile_3x1_CurveFrite (Variables|/Script/Engine.ChildActorComponent|GetChildActor _aschild_actor_component)))
        (Default|UpdateMyRotation _asbp_tile_3x_1_curve_frite)))
    (:then_1
      (Variables|Default|SetISMSpawnersArray (Utilities|Array|MakeArray (Variables|Default|GetArrow) (Variables|Default|GetL))))))