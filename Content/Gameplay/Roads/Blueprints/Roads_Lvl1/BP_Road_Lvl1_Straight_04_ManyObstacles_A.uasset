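; Level 1 straight road piece Blueprint, a "many obstacles" variant built on a parent road class.
; The construction script registers its straight, obstacle and arrow components in the ISM spawners array.
; It picks one of four ether patterns, each a combination of mirroring the C1 and C2 components on Y through negative scale.
; During TRP replay it skips the random roll and uses the existing pattern value.
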(fn ConstructionScript
  (|CallParentFunction)
  (Variables|Default|SetISMSpawnersArray (Utilities|Array|MakeArray (Variables|Default|GetStraight) (Variables|Default|GetSpawner_ManyObstacles_A) (Variables|Default|GetArrow1) (Variables|Default|GetArrow2) (Variables|Default|GetArrow3) (Variables|Default|GetArrow4) (Variables|Default|GetArrow5) (Variables|Default|GetArrow6) (Variables|Default|GetArrow7) (Variables|Default|GetArrow)))
  ;[1 1 1] random eth
  (bind _trp_replaying (CallFunction|TRPTestifTRPandGetRoadValues))
  (if _trp_replaying
    _
    (else
      (Variables|Default|SetTRP_EtherPattern (Math|Random|RandomIntegerinRange 0 3))))
  (switch int (Variables|Default|GetTRP_EtherPattern)
    (:0
      (Variables|Default|SetFirstBool false)
      (Variables|Default|SetSecondBool false))
    (:1
      (Variables|Default|SetFirstBool true)
      (Variables|Default|SetSecondBool true))
    (:2
      (Variables|Default|SetFirstBool true)
      (Variables|Default|SetSecondBool false))
    (:3
      (Variables|Default|SetFirstBool false)
      (Variables|Default|SetSecondBool true)))
  (Transformation|SetRelativeScale3D (Variables|Default|GetC1) (Math|Vector|MakeVector 1.0 (select (Variables|Default|GetFirstBool) -1.0 1.0) 1.0))
  (Transformation|SetRelativeScale3D (Variables|Default|GetC2) (Math|Vector|MakeVector 1.0 (select (Variables|Default|GetSecondBool) -1.0 1.0) 1.0)))