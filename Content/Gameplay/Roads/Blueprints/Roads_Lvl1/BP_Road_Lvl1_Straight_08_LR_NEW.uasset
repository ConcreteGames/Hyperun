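; Level 1 straight road piece Blueprint, a child that extends its parent's construction script.
; It fills the ISM spawner array with six arrow components and rotates AnchorRot by the TRPProceduralCurve value.
; It then attaches AttachPoint to LastArrow at a forward offset with unit world scale.
; A random-curve branch that keeps the existing value during TRP replay is left unconnected and never runs.
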(fn ConstructionScript
  (bind _attachpoint (Variables|Default|GetAttachPoint))
  (|CallParentFunction)
  (Variables|Default|SetISMSpawnersArray (Utilities|Array|MakeArray (Variables|Default|GetArrow8) (Variables|Default|GetArrow) (Variables|Default|GetLastArrow) (Variables|Default|GetArrow4) (Variables|Default|GetArrow6) (Variables|Default|GetArrow7)))
  (Transformation|SetRelativeRotation (Variables|Default|GetAnchorRot) (Variables|Default|GetTRP_ProceduralCurve) false false)
  (Transformation|AttachComponentToComponent _attachpoint (Variables|Default|GetLastArrow) "None" "KeepRelative" "KeepRelative" "KeepRelative" true)
  (Transformation|SetRelativeLocationAndRotation _attachpoint "1500.000000, 0, 0" "0, 0, 0" false false)
  (Transformation|SetWorldScale3D _attachpoint "1.000000,1.000000,1.000000"))