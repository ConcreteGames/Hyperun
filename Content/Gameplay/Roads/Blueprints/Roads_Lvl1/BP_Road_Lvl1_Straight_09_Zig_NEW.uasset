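; BP_Road_Lvl1_Straight_09_Zig_NEW is a Level 1 straight road segment, a zig variant built on a parent road Blueprint.
; Its Construction Script runs the parent's, then fills ISMSpawnersArray with arrow, Zig and RockArc components, likely spawn points for instanced meshes.
; It also casts two Woosh child actors to BP_SFX_WooshsNearPropsA and gives both the same prop type for near-prop whoosh sounds.
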(fn ConstructionScript
  (|CallParentFunction)
  (Variables|Default|SetISMSpawnersArray (Utilities|Array|MakeArray (Variables|Default|GetArrow6) (Variables|Default|GetArrow2) (Variables|Default|GetArrow1) (Variables|Default|GetArrow5) (Variables|Default|GetZig) (Variables|Default|GetArrow7) (Variables|Default|GetArrow8) (Variables|Default|GetArrow9) (Variables|Default|GetArrow4) (Variables|Default|GetRockArc)))
  (bind _asbp_sfx_wooshs_near_props_a (Utilities|Casting|CastToBP_SFX_WooshsNearPropsA (Variables|/Script/Engine.ChildActorComponent|GetChildActor (Variables|Default|GetWoosh1))))
  (Variables|/Game/Sound/Blueprints/BP_SFX_WooshsNearPropsA.BP_SFX_WooshsNearPropsA_C|SetPropsType _asbp_sfx_wooshs_near_props_a "NewEnumerator0")
  (bind _asbp_sfx_wooshs_near_props_a_2 (Utilities|Casting|CastToBP_SFX_WooshsNearPropsA (Variables|/Script/Engine.ChildActorComponent|GetChildActor (Variables|Default|GetWoosh2))))
  (Variables|/Game/Sound/Blueprints/BP_SFX_WooshsNearPropsA.BP_SFX_WooshsNearPropsA_C|SetPropsType _asbp_sfx_wooshs_near_props_a_2 "NewEnumerator0"))