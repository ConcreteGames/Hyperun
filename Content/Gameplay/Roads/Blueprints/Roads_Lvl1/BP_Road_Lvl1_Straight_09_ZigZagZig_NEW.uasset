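; Level 1 straight road segment Blueprint, a zig-zag-zig layout variant built on a parent road class.
; Its construction script runs the parent's script, then fills ISMSpawnersArray with this segment's spawner components: arrows, zig and zag pieces, and arcs.
; The file holds no other logic, so any use of that array lies outside it.
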(fn ConstructionScript
  (|CallParentFunction)
  (Variables|Default|SetISMSpawnersArray (Utilities|Array|MakeArray (Variables|Default|GetArrow1) (Variables|Default|GetZa1) (Variables|Default|GetZi2) (Variables|Default|GetArrow4) (Variables|Default|GetArrow3) (Variables|Default|GetZi1) (Variables|Default|GetArrow2) (Variables|Default|GetArrow5) (Variables|Default|GetArrow6) (Variables|Default|GetArrow7) (Variables|Default|GetArrow) (Variables|Default|GetSpawner_Arc3) (Variables|Default|GetSpawner_Arc1) (Variables|Default|GetSpawner_Arc2))))