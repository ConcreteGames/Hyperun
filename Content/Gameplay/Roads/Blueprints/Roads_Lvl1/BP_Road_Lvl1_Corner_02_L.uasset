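; Left-hand corner road piece for level 1 that randomizes its roadside props at construction.
; The construction script runs the parent setup, then calls RandomNearProps on the NearProps scene, with a chance of spawning and combinations of props allowed.
; It then fills the ISM spawner array with the piece's arrow components, which serve as spawn markers.
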(fn ConstructionScript
  (|CallParentFunction)
  (Utilities|FlowControl|Sequence
    (:then_0
      (CallFunction|RandomNearProps (Variables|Default|GetNearProps) 0.5 true 0.5))
    (:then_1
      (Variables|Default|SetISMSpawnersArray (Utilities|Array|MakeArray (Variables|Default|GetArrow5) (Variables|Default|GetArrow1) (Variables|Default|GetArrow2) (Variables|Default|GetArrow3) (Variables|Default|GetArrow9) (Variables|Default|GetArrow10) (Variables|Default|GetArrow) (Variables|Default|GetArrow4))))))