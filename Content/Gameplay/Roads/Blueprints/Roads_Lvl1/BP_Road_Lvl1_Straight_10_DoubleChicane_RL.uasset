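; Level 1 road piece Blueprint, named as a straight section with a right-left double chicane.
; Its construction script runs the parent construction script, then fills ISMSpawnersArray with a hand-picked set of Arrow components.
; The arrows appear to mark instanced static mesh spawn points; the code that uses the array is outside this graph.
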(fn ConstructionScript
  (|CallParentFunction)
  (Variables|Default|SetISMSpawnersArray (Utilities|Array|MakeArray (Variables|Default|GetArrow38) (Variables|Default|GetArrow13) (Variables|Default|GetArrow14) (Variables|Default|GetArrow15) (Variables|Default|GetArrow16) (Variables|Default|GetArrow11) (Variables|Default|GetArrow19) (Variables|Default|GetArrow20) (Variables|Default|GetArrow21) (Variables|Default|GetArrow22) (Variables|Default|GetArrow27) (Variables|Default|GetArrow28) (Variables|Default|GetArrow12) (Variables|Default|GetArrow33) (Variables|Default|GetArrow34) (Variables|Default|GetArrow35) (Variables|Default|GetArrow36) (Variables|Default|GetArrow37) (Variables|Default|GetArrow32) (Variables|Default|GetArrow44) (Variables|Default|GetArrow45) (Variables|Default|GetArrow46) (Variables|Default|GetArrow47) (Variables|Default|GetArrow48) (Variables|Default|GetArrow49) (Variables|Default|GetArrow50) (Variables|Default|GetArrow51) (Variables|Default|GetArrow52) (Variables|Default|GetArrow4) (Variables|Default|GetArrow7) (Variables|Default|GetArrow) (Variables|Default|GetArrow6) (Variables|Default|GetArrow3))))