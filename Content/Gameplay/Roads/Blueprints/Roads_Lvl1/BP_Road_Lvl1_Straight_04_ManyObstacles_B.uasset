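; Level 1 straight road segment with many obstacles (variant B), randomly built in one of two mirrored layouts by its construction script.
; After the parent construction script, it rolls the TRPEtherPattern flag, skipping the roll when TRP is replaying.
; The flag selects the BL or BR obstacle spawner for the ISM spawner array, swaps the sides of GK1 and GK2, and mirrors C1 and C2 via Y scale.
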(fn ConstructionScript
  (|CallParentFunction)
  ;[1 1 1] random eth
  (bind _trp_replaying (CallFunction|TRPTestifTRPandGetRoadValues))
  (if _trp_replaying
    _
    (else
      (Variables|Default|SetTRP_EtherPattern (Math|Conversions|ToInteger(Boolean) (Math|Random|RandomBool)))))
  (Variables|Default|SetISMSpawnersArray (Utilities|Array|MakeArray (Variables|Default|GetArrow7) (Variables|Default|GetArrow3) (Variables|Default|GetArrow4) (Variables|Default|GetArrow5) (Variables|Default|GetArrow2) (Variables|Default|GetArrow6) (Variables|Default|GetArrow) (Variables|Default|GetArrow1) (Variables|Default|GetStraight) (Utilities|Select :Index (Variables|Default|GetTRP_EtherPattern) :Option%200 (Variables|Default|GetSpawner_ManyObstacles_B_L) :Option%201 (Variables|Default|GetSpawner_ManyObstacles_B_R)))) ; Après le test de TRP car besoin du bool
  (Transformation|SetRelativeLocation (Variables|Default|GetGK1) (Math|Vector|MakeVector 3.5e+03 (select (Math|Conversions|ToBoolean(Integer) (Variables|Default|GetTRP_EtherPattern)) -6.5e+02 6.5e+02) 0.0) false false)
  (Transformation|SetRelativeLocation (Variables|Default|GetGK2) (Math|Vector|MakeVector 7.5e+03 (select (Math|Conversions|ToBoolean(Integer) (Variables|Default|GetTRP_EtherPattern)) 6.5e+02 -6.5e+02) 0.0) false false)
  (Transformation|SetRelativeScale3D (Variables|Default|GetC1) (Math|Vector|MakeVector 1.0 (select (Math|Conversions|ToBoolean(Integer) (Variables|Default|GetTRP_EtherPattern)) 1.0 -1.0) 1.0))
  (Transformation|SetRelativeScale3D (Variables|Default|GetC2) (Math|Vector|MakeVector 1.0 (select (Math|Conversions|ToBoolean(Integer) (Variables|Default|GetTRP_EtherPattern)) 1.0 -1.0) 1.0)))