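; Level 1 road piece for a lifted left U-turn corner, built from two chains of child-actor segments ("Frites").
; Construction applies one random pitch to both chains, reusing the stored value during TRP replay, and attaches the second chain to an anchor.
; It also registers ISM spawner components and adds a crowd actor with 50% probability.
; On DynamicCreation, each chain gets a road vertex snap pass.
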(event EventDynamicCreation
  (CallFunction|RoadVertexSnap3 (Variables|Default|GetFrites1))
  (CallFunction|RoadVertexSnap3 (Variables|Default|GetFrites2)))

(fn ConstructionScript
  (bind _2_frite1 (Variables|Default|Get2_Frite1))
  (|CallParentFunction)
  (Variables|Default|SetFrites1 (Utilities|Array|MakeArray (Variables|Default|Get1_Frite1) (Variables|Default|GetChildActor1) (Variables|Default|GetChildActor2) (Variables|Default|GetChildActor3) (Variables|Default|GetChildActor4) (Variables|Default|GetChildActor5) (Variables|Default|GetChildActor12) (Variables|Default|GetChildActor13) (Variables|Default|GetChildActor14) (Variables|Default|GetChildActor15) (Variables|Default|Get1_LastFrite)))
  (Variables|Default|SetFrites2 (Utilities|Array|MakeArray (Variables|Default|Get2_Frite1) (Variables|Default|GetChildActor22) (Variables|Default|GetChildActor23) (Variables|Default|GetChildActor24) (Variables|Default|GetChildActor25) (Variables|Default|GetChildActor26) (Variables|Default|GetChildActor27) (Variables|Default|GetChildActor28) (Variables|Default|GetChildActor29) (Variables|Default|GetChildActor30) (Variables|Default|Get2_LastFrite)))
  (Utilities|FlowControl|Sequence
    (:then_0
      ;[1 1 1] random pitch
      (bind _trp_replaying (CallFunction|TRPTestifTRPandGetRoadValues))
      (if _trp_replaying
        _
        (else
          (Variables|Default|SetTRP_ProceduralCurve (Math|Rotator|MakeRotator 0.0 (Math|Random|RandomFloatinRange 2.0 5.0) 0.0))))
      (CallFunction|SetRollandPitchOfCurveOfFrites2 (Variables|Default|GetFrites1) 0.0 0.0 (.pitch (Variables|Default|GetTRP_ProceduralCurve)) (.pitch (Variables|Default|GetTRP_ProceduralCurve)))
      (CallFunction|SetRollandPitchOfCurveOfFrites2 (Variables|Default|GetFrites2) 0.0 0.0 (.pitch (Variables|Default|GetTRP_ProceduralCurve)) (.pitch (Variables|Default|GetTRP_ProceduralCurve)))
      (Transformation|AttachComponentToComponent _2_frite1 (Variables|Default|GetAnchorFrite2) "None" "KeepRelative" "KeepRelative" "KeepRelative" true)
      (Transformation|SetRelativeLocationAndRotation _2_frite1 "0, 0, 0" "0, 0, 0" false false))
    (:then_1
      (Variables|Default|SetISMSpawnersArray (Utilities|Array|MakeArray (Variables|Default|GetArrow2) (Variables|Default|GetArrow3) (Variables|Default|GetL) (Variables|Default|GetL2) (Variables|Default|GetArrow4) (Variables|Default|GetArrow1) (Variables|Default|GetArrow5) (Variables|Default|GetArrow) (Variables|Default|GetR))))
    (:then_2
      ;[1 1 1] Random Crowd 1/5
      (if (Math|Random|RandomBoolwithWeight 0.5)
        (ChildActorComponent|SetChildActorClass (Variables|Default|GetCrowd) "/Game/Coco/Lab/Props/NearProps/RoadCrowd/BP_RoadCowd.BP_RoadCowd_C")))))