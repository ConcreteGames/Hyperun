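; Level 1 straight road piece with a left wall ride, a child Blueprint that extends its parent's construction script.
; Construction registers arrow and empty components as ISM spawners, then gives six numbered components a shared offset and random curve rotation.
; During a TRP replay it skips the random roll, keeping the curve value reproducible.
; SetFrite, not called here, randomizes roll and pitch on curve-frite child actor tiles.
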(fn ConstructionScript
  (|CallParentFunction)
  (Variables|Default|SetISMSpawnersArray (Utilities|Array|MakeArray (Variables|Default|GetArrow) (Variables|Default|GetArrow16) (Variables|Default|GetArrow8) (Variables|Default|GetArrow9) (Variables|Default|GetArrow10) (Variables|Default|GetArrow11) (Variables|Default|GetArrow7) (Variables|Default|GetArrow3) (Variables|Default|GetArrow4) (Variables|Default|GetArrow5) (Variables|Default|GetArrow12) (Variables|Default|GetArrow13) (Variables|Default|GetArrow14) (Variables|Default|GetArrow15) (Variables|Default|GetArrow21) (Variables|Default|GetArrow22) (Variables|Default|GetArrow26) (Variables|Default|GetArrow27) (Variables|Default|GetArrow28) (Variables|Default|GetArrow29) (Variables|Default|GetArrow30) (Variables|Default|GetArrow31) (Variables|Default|GetArrow32) (Variables|Default|GetArrow33) (Variables|Default|GetArrow34) (Variables|Default|GetArrow35) (Variables|Default|GetArrow36) (Variables|Default|GetArrow37) (Variables|Default|GetEmpty2) (Variables|Default|GetEmpty1)))
  ;[1 1 1] random curve
  (bind _trp_replaying (CallFunction|TRPTestifTRPandGetRoadValues))
  (if _trp_replaying
    _
    (else
      (Variables|Default|SetTRP_ProceduralCurve (Math|Rotator|MakeRotator (Math|Random|RandomFloatinRange 1e+01 2e+01) 0.0 0.0))))
  (Transformation|SetRelativeLocationAndRotation (Variables|Default|Get2) "0.000000,300.000000, 0" (Variables|Default|GetTRP_ProceduralCurve) false false))

(fn SetFrite
  (params (FirstFrite :type Scene%20Component%20Object%20Reference) (RollMin :type Float%20%28single-precision%29) (RollMax :type Float%20%28single-precision%29) (PitchMin :type Float%20%28single-precision%29) (PitchMax :type Float%20%28single-precision%29))
  (for _array_element (Components|GetChildrenComponents FirstFrite true)
    (bind _aschild_actor_component (Utilities|Casting|CastToChildActorComponent _array_element))
    (Utilities|Casting|CastToBP_Tile_3x1_CurveFrite (Variables|/Script/Engine.ChildActorComponent|GetChildActor _aschild_actor_component))
    (LocalVariables|SetCurrentFrite _array_element)
    (Transformation|SetRelativeLocationAndRotation (LocalVariables|GetCurrentFrite) "300.000000, 0, 0" (Math|Rotator|MakeRotator (Math|Random|RandomFloatinRange RollMin RollMax) (Math|Random|RandomFloatinRange PitchMin PitchMax) 0.0) false false :!pinned true) ; 1st group of frites
  ))