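; Level 1 straight tunnel road piece, LR variant, built on a parent road Blueprint.
; Its construction script runs the parent's script, then fills ISMSpawnersArray with the piece's Arrow components.
; The array name indicates these arrows mark spawn points for instanced static meshes, with the spawning logic outside this graph.
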(fn ConstructionScript
  (|CallParentFunction)
  (Variables|Default|SetISMSpawnersArray (Utilities|Array|MakeArray (Variables|Default|GetArrow12) (Variables|Default|GetArrow2) (Variables|Default|GetArrow3) (Variables|Default|GetArrow4) (Variables|Default|GetArrow5) (Variables|Default|GetArrow1) (Variables|Default|GetArrow6) (Variables|Default|GetArrow7) (Variables|Default|GetArrow8) (Variables|Default|GetArrow) (Variables|Default|GetArrow9) (Variables|Default|GetArrow11) (Variables|Default|GetArrow10) (Variables|Default|GetArrow13) (Variables|Default|GetArrow14) (Variables|Default|GetArrow15) (Variables|Default|GetArrow18) (Variables|Default|GetArrow20) (Variables|Default|GetArrow22) (Variables|Default|GetArrow23) (Variables|Default|GetArrow16) (Variables|Default|GetArrow19) (Variables|Default|GetArrow21) (Variables|Default|GetArrow17))))