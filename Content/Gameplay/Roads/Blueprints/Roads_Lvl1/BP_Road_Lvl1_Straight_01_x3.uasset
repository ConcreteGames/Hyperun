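; Level 1 straight road segment Blueprint (x3 variant) that dresses itself with randomized nearby props.
; The construction script runs the parent's, then sets ISMSpawnersArray to its three arrow components.
; It rolls one random prop type per construction and applies that class to the child actor components under NearProps, so they all match: street lamp, flag, BP_Arv, forest or bird pool.
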(fn ConstructionScript
  (|CallParentFunction)
  (Variables|Default|SetISMSpawnersArray (Utilities|Array|MakeArray (Variables|Default|GetArrow1) (Variables|Default|GetArrow2) (Variables|Default|GetArrow)))
  ;[1 1 1] near props
  (Variables|Default|SetNearPropType (Math|Random|RandomIntegerinRange 0 4))
  (for _array_element (Components|GetChildrenComponents (Variables|Default|GetNearProps) false)
    (bind _aschild_actor_component (Utilities|Casting|CastToChildActorComponent _array_element))
    (ChildActorComponent|SetChildActorClass _aschild_actor_component (Utilities|Select :Index (Variables|Default|GetNearPropType) :Option%200 "/Game/Coco/Lab/Props/NearProps/Lampadaire/BP_Lampadaire.BP_Lampadaire_C" :Option%201 "/Game/Coco/Lab/Props/NearProps/Lampadaire/BP_Flag.BP_Flag_C" :Option%202 "/Game/Coco/Lab/Props/NearProps/Lampadaire/BP_Arv.BP_Arv_C" :Option%203 "/Game/Coco/Lab/Props/NearProps/Lampadaire/BP_Forest.BP_Forest_C" :Option%204 "/Game/Coco/Lab/Props/NearProps/Lampadaire/BP_birdsPool.BP_birdsPool_C"))))