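; Level 1 straight road segment variant with a single obstacle randomly placed on the left or right side.
; The construction script rolls a random pattern unless TRP is replaying, in which case it skips the roll.
; That pattern selects the obstacle spawner added alongside Arrow to the ISM spawner array.
; It also positions component K and a simple collectible on opposite lateral sides of the road.
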(fn ConstructionScript
  (|CallParentFunction)
  ;[1 1 1] random eth
  (bind _trp_replaying (CallFunction|TRPTestifTRPandGetRoadValues))
  (if _trp_replaying
    _
    (else
      (Variables|Default|SetTRP_EtherPattern (Math|Conversions|ToInteger(Boolean) (Math|Random|RandomBool)))))
  (Variables|Default|SetISMSpawnersArray (Utilities|Array|MakeArray (Variables|Default|GetArrow) (Utilities|Select :Index (Variables|Default|GetTRP_EtherPattern) :Option%200 (Variables|Default|GetSpawner_ObstacleStraight_R) :Option%201 (Variables|Default|GetSpawner_ObstacleStraight_L))))
  (Transformation|SetRelativeLocation (Variables|Default|Getk) (Math|Vector|MakeVector 3e+03 (select (Math|Conversions|ToBoolean(Integer) (Variables|Default|GetTRP_EtherPattern)) 4e+02 -4e+02) 0.0) false false)
  (Transformation|SetRelativeLocation (Variables|Default|GetBP_Collectible_Simple) (Math|Vector|MakeVector 3e+03 (select (Math|Conversions|ToBoolean(Integer) (Variables|Default|GetTRP_EtherPattern)) -3.5e+02 3.5e+02) 0.0) false false))