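; BP_Road_Lvl1_Straight_09_ZagZigZag_NEW is a level 1 straight road segment variant with a zag-zig-zag layout of spawn points.
; Its construction script runs the parent construction logic, then fills ISMSpawnersArray with its arrow, zig, zag and arc spawner components.
; The array is presumably consumed by inherited logic, as this child only registers the spawners.
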(fn ConstructionScript
  (|CallParentFunction)
  (Variables|Default|SetISMSpawnersArray (Utilities|Array|MakeArray (Variables|Default|GetArrow2) (Variables|Default|GetZag2) (Variables|Default|GetZig1) (Variables|Default|GetArrow3) (Variables|Default|GetArrow4) (Variables|Default|GetZag1) (Variables|Default|GetArrow5) (Variables|Default|GetArrow6) (Variables|Default|GetArrow7) (Variables|Default|GetArrow8) (Variables|Default|GetArrow1) (Variables|Default|GetSpawner_Arc2) (Variables|Default|GetSpawner_Arc3) (Variables|Default|GetSpawner_Arc1))))