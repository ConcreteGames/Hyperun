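; Level 1 road piece, a straight with a right-hand lifted U-turn, built from two chains of "frite" child-actor tiles.
; Construction applies one random pitch, skipped during TRP replay, to the chained tiles as a shared relative transform, then updates the CurveFrite tiles under Roads.
; It also registers ISM spawners and randomly adds a crowd actor.
; On DynamicCreation, RoadVertexSnap3 runs on each chain.
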(event EventDynamicCreation
  (CallFunction|RoadVertexSnap3 (Variables|Default|GetFrites1))
  (CallFunction|RoadVertexSnap3 (Variables|Default|GetFrites2)))

(fn ConstructionScript
  (|CallParentFunction)
  (Utilities|FlowControl|Sequence
    (:then_0
      (Variables|Default|SetFrites1 (Utilities|Array|MakeArray (Variables|Default|Get1_Frite1) (Variables|Default|GetChildActor1) (Variables|Default|GetChildActor2) (Variables|Default|GetChildActor3) (Variables|Default|GetChildActor4) (Variables|Default|GetChildActor5) (Variables|Default|GetChildActor12) (Variables|Default|GetChildActor13) (Variables|Default|GetChildActor14) (Variables|Default|GetChildActor15) (Variables|Default|Get1_LastFrite)))
      (Variables|Default|SetFrites2 (Utilities|Array|MakeArray (Variables|Default|Get2_Frite1) (Variables|Default|GetChildActor22) (Variables|Default|GetChildActor23) (Variables|Default|GetChildActor24) (Variables|Default|GetChildActor25) (Variables|Default|GetChildActor26) (Variables|Default|GetChildActor27) (Variables|Default|GetChildActor28) (Variables|Default|GetChildActor29) (Variables|Default|GetChildActor30) (Variables|Default|Get2_LastFrite)))
      (Variables|Default|SetISMSpawnersArray (Utilities|Array|MakeArray (Variables|Default|GetArrow8) (Variables|Default|GetArrow1) (Variables|Default|GetArrow13) (Variables|Default|GetArrow11) (Variables|Default|GetArrow2) (Variables|Default|GetArrow3) (Variables|Default|GetArrow4) (Variables|Default|GetArrow5) (Variables|Default|GetArrow9) (Variables|Default|GetArrow10) (Variables|Default|GetArrow6) (Variables|Default|GetArrow7) (Variables|Default|GetArrow) (Variables|Default|GetCR1) (Variables|Default|GetCR2)))
      ;[1 1 1] random curve
      (bind _trp_replaying (CallFunction|TRPTestifTRPandGetRoadValues))
      (if _trp_replaying
        _
        (else
          (Variables|Default|SetTRP_ProceduralCurve (Math|Rotator|MakeRotator 0.0 (Math|Random|RandomFloatinRange (Variables|Default|GetFritePitchMin) (Variables|Default|GetFritePitchMax)) 0.0))))
      (Transformation|SetRelativeLocationAndRotation (Variables|Default|GetChildActor1) "300.000000, 0, 0" (Variables|Default|GetTRP_ProceduralCurve) false false :!pinned true) ; groups of frites
      ;[1 1 1] On met à jour toutes les frites de toutes les roads enfants
      (for _array_element (Components|GetChildrenComponents (Variables|Default|GetRoads) true)
        (bind _aschild_actor_component (Utilities|Casting|CastToChildActorComponent _array_element))
        (bind _asbp_tile_3x_1_curve_frite (Utilities|Casting|CastToBP_Tile_3x1_CurveFrite (Variables|/Script/Engine.ChildActorComponent|GetChildActor _aschild_actor_component)))
        (Default|UpdateMyRotation _asbp_tile_3x_1_curve_frite)))
    (:then_1
      ;[1 1 1] Random Crowd 1/5
      (if (Math|Random|RandomBoolwithWeight 0.5)
        (ChildActorComponent|SetChildActorClass (Variables|Default|GetCrowd) "/Game/Coco/Lab/Props/NearProps/RoadCrowd/BP_RoadCowd.BP_RoadCowd_C")))))