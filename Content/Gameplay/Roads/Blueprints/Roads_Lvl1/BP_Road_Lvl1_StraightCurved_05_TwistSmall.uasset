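; Level 1 procedural road piece forming a straight stretch with a small random twist, built from a series of child-actor segments.
; Construction applies one shared offset and rotation to each segment after the first, with the attach point following the last.
; The random rotation is rolled unless a TRP replay is running, which takes stored values from the GameMode.
; On DynamicCreation, the segment list goes to RoadVertexSnap3.
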(event EventDynamicCreation
  (CallFunction|RoadVertexSnap3 (Variables|Default|GetFrites)))

(fn ConstructionScript
  (|CallParentFunction)
  (Variables|Default|SetFrites (Utilities|Array|MakeArray (Variables|Default|GetFirstRoad) (Variables|Default|GetChildActor) (Variables|Default|GetChildActor1) (Variables|Default|GetChildActor2) (Variables|Default|GetChildActor3) (Variables|Default|GetChildActor4) (Variables|Default|GetChildActor5) (Variables|Default|GetChildActor6) (Variables|Default|GetChildActor7) (Variables|Default|GetChildActor8) (Variables|Default|GetChildActor9) (Variables|Default|GetChildActor10) (Variables|Default|GetChildActor11) (Variables|Default|GetChildActor12) (Variables|Default|GetChildActor13) (Variables|Default|GetChildActor14) (Variables|Default|GetLAST)))
  (Transformation|AttachComponentToComponent (Variables|Default|GetAttachPoint) (Variables|Default|GetLAST) "None" "SnapToTarget" "SnapToTarget" "SnapToTarget" true)
  ;[1 1 1] If TRP, get the values from Gamemode
  ; If not, set the values (then it's GET by the gamemode)
  (bind _trp_replaying (CallFunction|TRPTestifTRPandGetRoadValues))
  (if _trp_replaying
    _
    (else
      (Variables|Default|SetTRP_ProceduralCurve (Math|Rotator|MakeRotator (select (Math|Random|RandomBool) (Math|Random|RandomFloatinRange 4.0 7.0) (Math|Random|RandomFloatinRange -7.0 -4.0)) (Math|Random|RandomFloatinRange 0.0 3.0) 0.0))))
  (Transformation|SetRelativeLocationAndRotation (Variables|Default|GetChildActor) "300.000000, 0, 0" (Variables|Default|GetTRP_ProceduralCurve) false false)
  (Transformation|SetRelativeLocationAndRotation (Variables|Default|GetAttachPoint) "300.000000, 0, 0" "0, 0, 0" false false))