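; Level 1 procedural road piece forming a smooth downward step from two chains of child-actor segments.
; The construction script pitches the first chain down by a random angle per segment, then counter-pitches the second, with a 50% chance of extra rise.
; Random values are stored in TRP variables and not re-rolled during TRP replay.
; AttachPoint follows the last segment, and DynamicCreation runs RoadVertexSnap3 on both chains.
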(event EventDynamicCreation
  (CallFunction|RoadVertexSnap3 (Variables|Default|GetFrites1))
  (CallFunction|RoadVertexSnap3 (Variables|Default|GetFrites2)))

(fn ConstructionScript
  (bind _first2 (Variables|Default|GetFirst2))
  (|CallParentFunction)
  (Variables|Default|SetFrites1 (Utilities|Array|MakeArray (Variables|Default|GetFirst2) (Variables|Default|GetChildActor8) (Variables|Default|GetChildActor9) (Variables|Default|GetChildActor10) (Variables|Default|GetChildActor11) (Variables|Default|GetLast2)))
  (Variables|Default|SetFrites2 (Utilities|Array|MakeArray (Variables|Default|GetFIRSTROAD) (Variables|Default|GetChildActor) (Variables|Default|GetChildActor1) (Variables|Default|GetChildActor2) (Variables|Default|GetChildActor3) (Variables|Default|GetLastPart1)))
  ;[1 1 1] random 2 float + 1 bool
  (bind _trp_replaying (CallFunction|TRPTestifTRPandGetRoadValues))
  (if _trp_replaying
    _
    (else
      (Variables|Default|SetTRP_ProceduralCurve (Math|Rotator|MakeRotator 0.0 (Math|Random|RandomFloatinRange -6.0 -2.0) (Math|Random|RandomFloatinRange 2.0 4.0)))
      (Variables|Default|SetTRP_EtherPattern (Math|Conversions|ToInteger(Boolean) (Math|Random|RandomBool)))))
  (Transformation|AttachComponentToComponent (Variables|Default|GetAttachPoint) (Variables|Default|GetLast2) "None" "SnapToTarget" "SnapToTarget" "SnapToTarget" true)
  (Transformation|SetRelativeLocationAndRotation (Variables|Default|GetChildActor) "300.000000, 0, 0" (Math|Rotator|MakeRotator 0.0 (.pitch (Variables|Default|GetTRP_ProceduralCurve)) 0.0) false false)
  (Transformation|AttachComponentToComponent _first2 (Variables|Default|GetLastPart1) "None" "SnapToTarget" "SnapToTarget" "SnapToTarget" true)
  (Transformation|SetRelativeLocationAndRotation _first2 "300.000000, 0, 0" (Math|Rotator|MakeRotator 0.0 0.0 0.0) false false)
  (Transformation|SetRelativeLocationAndRotation (Variables|Default|GetLast2) "300.000000, 0, 0" (Math|Rotator|MakeRotator 0.0 (select (Math|Conversions|ToBoolean(Integer) (Variables|Default|GetTRP_EtherPattern)) (+ (* (.pitch (Variables|Default|GetTRP_ProceduralCurve)) -1.0) (.yaw (Variables|Default|GetTRP_ProceduralCurve))) (* (.pitch (Variables|Default|GetTRP_ProceduralCurve)) -1.0)) 0.0) false false)
  (Transformation|SetRelativeLocationAndRotation (Variables|Default|GetAttachPoint) "300.000000, 0, 0" "0, 0, 0" false false) ; End
)