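; Level 1 straight cut-tube road piece that gets a randomly rolled end section, tilted to either side.
; Construction registers its line, arrow and tube ISM spawners, then rolls the out and tube anchors by one of two opposite-signed random angles.
; The angles and side choice are stored in TRP curve and pattern values, so TRP replays skip randomization.
; The attach point is then snapped to the end anchor.
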(fn ConstructionScript
  (bind _attachpoint (Variables|Default|GetAttachPoint))
  (|CallParentFunction)
  (Variables|Default|SetISMSpawnersArray (Utilities|Array|MakeArray (Variables|Default|GetLine1) (Variables|Default|GetArrow) (Variables|Default|GetArrow1) (Variables|Default|GetSpawner_Tube)))
  ;[1 1 1] random 2 float + 1 bool
  (bind _trp_replaying (CallFunction|TRPTestifTRPandGetRoadValues))
  (if _trp_replaying
    _
    (else
      (Variables|Default|SetTRP_ProceduralCurve (Math|Rotator|MakeRotator (Math|Random|RandomFloatinRange -75.0 -5e+01) (Math|Random|RandomFloatinRange 5e+01 75.0) 0.0))
      (Variables|Default|SetTRP_EtherPattern (Math|Conversions|ToInteger(Boolean) (Math|Random|RandomBool)))))
  ;[1 1 1] Fin à rotation random
  (Transformation|SetRelativeRotation (Variables|Default|GetOutRotaAnchor) (Math|Rotator|MakeRotator (select (Math|Conversions|ToBoolean(Integer) (Variables|Default|GetTRP_EtherPattern)) (.pitch (Variables|Default|GetTRP_ProceduralCurve)) (.roll (Variables|Default|GetTRP_ProceduralCurve))) 0.0 0.0) false false)
  (Transformation|AttachComponentToComponent _attachpoint (Variables|Default|GetEndAnchor) "None" "SnapToTarget" "SnapToTarget" "SnapToTarget" true)
  (Transformation|SetRelativeLocationAndRotation _attachpoint "0, 0, 0" "0, 0, 0" false false))