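; Level 1 straight double-way road segment, a child Blueprint whose construction script configures its layout after running the parent's.
; It fills the ISM spawner array from its arrow, line and one-way spawner components.
; A random bool, skipped during TRP replay, mirrors the collectibles anchor on Y and is stored as the TRP pattern value.
; The attach point is parented to the end line with a forward offset and unit world scale.
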(fn ConstructionScript
  (bind _attachpoint (Variables|Default|GetAttachPoint))
  (|CallParentFunction)
  (Variables|Default|SetISMSpawnersArray (Utilities|Array|MakeArray (Variables|Default|GetArrow40) (Variables|Default|Getline2) (Variables|Default|Getline3) (Variables|Default|GetArrow5) (Variables|Default|GetArrow6) (Variables|Default|GetArrow7) (Variables|Default|GetArrow8) (Variables|Default|GetArrow9) (Variables|Default|GetArrow22) (Variables|Default|GetArrow23) (Variables|Default|GetArrow24) (Variables|Default|GetArrow25) (Variables|Default|GetArrow26) (Variables|Default|GetArrow27) (Variables|Default|GetArrow28) (Variables|Default|GetArrow29) (Variables|Default|GetArrow30) (Variables|Default|GetArrow31) (Variables|Default|GetArrow32) (Variables|Default|GetArrow33) (Variables|Default|GetArrow34) (Variables|Default|GetArrow35) (Variables|Default|GetArrow36) (Variables|Default|GetArrow37) (Variables|Default|GetArrow38) (Variables|Default|GetArrow39) (Variables|Default|Getline1) (Variables|Default|GetArrow42) (Variables|Default|GetArrow43) (Variables|Default|GetArrow44) (Variables|Default|GetArrow45) (Variables|Default|GetArrow46) (Variables|Default|GetArrow52) (Variables|Default|GetArrow49) (Variables|Default|GetArrow50) (Variables|Default|GetArrow51) (Variables|Default|GetArrow47) (Variables|Default|GetArrow48) (Variables|Default|GetArrow53) (Variables|Default|GetArrow41) (Variables|Default|GetArrow55) (Variables|Default|GetArrow56) (Variables|Default|GetArrow57) (Variables|Default|GetArrow) (Variables|Default|GetArrow1) (Variables|Default|GetArrow2) (Variables|Default|GetArrow54) (Variables|Default|GetArrow21) (Variables|Default|GetlineEnd) (Variables|Default|GetArrow3) (Variables|Default|GetArrow4) (Variables|Default|GetSpawner_OneWay_R) (Variables|Default|GetSpawner_OneWay_L2) (Variables|Default|GetSpawner_OneWay_R2) (Variables|Default|GetSpawner_OneWay_L)))
  ;[1 1 1] random curve
  (bind _trp_replaying (CallFunction|TRPTestifTRPandGetRoadValues))
  (if _trp_replaying
    _
    (else
      (Variables|Default|SetTRP_EtherPattern (Math|Conversions|ToInteger(Boolean) (Math|Random|RandomBool)))))
  (Transformation|SetRelativeScale3D (Variables|Default|GetAnchor4Collectibles) (Math|Vector|MakeVector 1.0 (select (Math|Conversions|ToBoolean(Integer) (Variables|Default|GetTRP_EtherPattern)) 1.0 -1.0) 1.0))
  (Transformation|AttachComponentToComponent _attachpoint (Variables|Default|GetlineEnd) "None" "KeepRelative" "KeepRelative" "KeepRelative" true)
  (Transformation|SetRelativeLocationAndRotation _attachpoint "1500.000000, 0, 0" "0, 0, 0" false false)
  (Transformation|SetWorldScale3D _attachpoint "1.000000,1.000000,1.000000"))