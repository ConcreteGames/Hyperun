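; Level 1 left looping corner road piece, built from curve "frite" tiles, that drives the bike's FOV effect through the loop.
; Between entry and exit or jump-gap triggers, Tick maps bike height through two curves, switching past halfway, into an FOV offset.
; Construction positions end anchors, hides tile meshes, randomly offsets Ether (skipping the roll during TRP replay) and randomly adds a crowd.
; DynamicCreation vertex-snaps the tiles.
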(event OnComponentBeginOverlap(EnterLooping)
  (params (OverlappedComponent :type Primitive%20Component%20Object%20Reference) (OtherActor :type Actor%20Object%20Reference) (OtherComp :type Primitive%20Component%20Object%20Reference) (OtherBodyIndex :type Integer) (bFromSweep :type Boolean) (SweepResult :type Hit%20Result%20Structure%20%28by%20ref%29))
  (Variables|Default|SetFOVLooping true)
  (bind _asbp_bike_parent (Utilities|Casting|CastToBP_Bike_Parent (Game|Player|GetPlayerPawn 0)))
  (Variables|/Game/Bikes/BP_Bike_Parent.BP_Bike_Parent_C|SetFOVLooping_Need _asbp_bike_parent true))

(event OnComponentBeginOverlap(JumpGapDetector)
  (params (OverlappedComponent :type Primitive%20Component%20Object%20Reference) (OtherActor :type Actor%20Object%20Reference) (OtherComp :type Primitive%20Component%20Object%20Reference) (OtherBodyIndex :type Integer) (bFromSweep :type Boolean) (SweepResult :type Hit%20Result%20Structure%20%28by%20ref%29))
  (if (Variables|Default|GetFOVLooping)
    (Variables|/Game/Bikes/BP_Bike_Parent.BP_Bike_Parent_C|SetFOVLooping_ValueToAdd (stale EventTick _asbp_bike_parent_2) 0.0)
    (Variables|Default|SetFOVLooping false)
    (bind _asbp_bike_parent (Utilities|Casting|CastToBP_Bike_Parent (Game|Player|GetPlayerPawn 0)))
    (Variables|/Game/Bikes/BP_Bike_Parent.BP_Bike_Parent_C|SetFOVLooping_Need _asbp_bike_parent false)))

(event OnComponentBeginOverlap(QuitLooping)
  (params (OverlappedComponent :type Primitive%20Component%20Object%20Reference) (OtherActor :type Actor%20Object%20Reference) (OtherComp :type Primitive%20Component%20Object%20Reference) (OtherBodyIndex :type Integer) (bFromSweep :type Boolean) (SweepResult :type Hit%20Result%20Structure%20%28by%20ref%29))
  (if (Variables|Default|GetFOVLooping)
    (Variables|/Game/Bikes/BP_Bike_Parent.BP_Bike_Parent_C|SetFOVLooping_ValueToAdd (stale EventTick _asbp_bike_parent_2) 0.0)
    (Variables|Default|SetFOVLooping false)
    (bind _asbp_bike_parent (Utilities|Casting|CastToBP_Bike_Parent (Game|Player|GetPlayerPawn 0)))
    (Variables|/Game/Bikes/BP_Bike_Parent.BP_Bike_Parent_C|SetFOVLooping_Need _asbp_bike_parent false)))

(event EventDynamicCreation
  ;[0.1825 1 0] DYNAMIC CREATION
  (CallFunction|RoadVertexSnap3 (Variables|Default|GetFrites)))

(event EventTick
  (params (DeltaSeconds :type Float%20%28single-precision%29))
  (bind _bikelocation (Variables|Default|GetBikeLocation))
  (bind _relativelocation (Variables|/Script/Engine.SceneComponent|GetRelativeLocation _bikelocation))
  (bind _returnvalue (- (.z _relativelocation) 1e+02))
  (bind _returnvalue_2 (/ _returnvalue 4e+03))
  (bind _returnvalue_3 (> _returnvalue_2 1.0))
  (bind _returnvalue_4 (> _returnvalue_2 0.0))
  (bind _returnvalue_5 (select _returnvalue_3 1.0 _returnvalue_2))
  (bind _returnvalue_6 (select _returnvalue_4 _returnvalue_5 0.0))
  (if (Variables|Default|GetFOVLooping)
    (bind _asbp_bike_parent (Utilities|Casting|CastToBP_Bike_Parent (Game|Player|GetPlayerPawn 0)))
    (Transformation|SetWorldLocation (Variables|Default|GetBikeLocation) (Transformation|GetWorldLocation (Variables|/Game/Bikes/BP_Bike_Parent.BP_Bike_Parent_C|GetBikeScene _asbp_bike_parent)) false false)
    (bind _asbp_bike_parent_2 (Utilities|Casting|CastToBP_Bike_Parent (Game|Player|GetPlayerPawn 0)))
    ;[1 1 1] Test is in loop
    (if (and (> _returnvalue_6 0.5) (not (Variables|Default|GetBikeIsInLooping)))
      (Variables|Default|SetBikeIsInLooping true))
    ;[1 1 1] Test end of loop
    (if (and (Variables|Default|GetBikeIsInLooping) (== (Math|Curves|GetFloatValue (select (Variables|Default|GetBikeIsInLooping) (Variables|Default|GetCRV_FOVLoopingPart2) (Variables|Default|GetCRV_FOVLoopingPart1)) _returnvalue_6) 0.0))
      (Variables|/Game/Bikes/BP_Bike_Parent.BP_Bike_Parent_C|SetFOVLooping_ValueToAdd _asbp_bike_parent_2 0.0)
      (Variables|Default|SetFOVLooping false)
      (bind _asbp_bike_parent_3 (Utilities|Casting|CastToBP_Bike_Parent (Game|Player|GetPlayerPawn 0)))
      (Variables|/Game/Bikes/BP_Bike_Parent.BP_Bike_Parent_C|SetFOVLooping_Need _asbp_bike_parent_3 false)
      (else
        (Variables|/Game/Bikes/BP_Bike_Parent.BP_Bike_Parent_C|SetFOVLooping_ValueToAdd _asbp_bike_parent_2 (Math|Curves|GetFloatValue (select (Variables|Default|GetBikeIsInLooping) (Variables|Default|GetCRV_FOVLoopingPart2) (Variables|Default|GetCRV_FOVLoopingPart1)) _returnvalue_6))))))

(fn ConstructionScript
  (bind _arrow3 (Variables|Default|GetArrow3))
  (bind _endanchor (Variables|Default|GetEndAnchor))
  (bind _arrow4 (Variables|Default|GetArrow4))
  (bind _returnvalue (Transformation|GetWorldTransform _arrow3))
  (bind _returnvalue_2 (Transformation|GetWorldTransform _endanchor))
  (|CallParentFunction)
  (Variables|Default|SetISMSpawnersArray (Utilities|Array|MakeArray (Variables|Default|GetArrow1) (Variables|Default|GetArrow2) (Variables|Default|GetArrow4) (Variables|Default|GetArrow5) (Variables|Default|GetArrow3) (Variables|Default|GetArrow) (Variables|Default|GetSpawner_LoopingGrid_L)))
  (Utilities|FlowControl|Sequence
    (:then_0
      ;[1 1 1] get frites
      (Variables|Default|SetFrites (Utilities|Array|MakeArray (Variables|Default|GetBP_Tile_3x1_CurveFrite) (Variables|Default|GetChildActor) (Variables|Default|GetChildActor1) (Variables|Default|GetChildActor2) (Variables|Default|GetChildActor3) (Variables|Default|GetChildActor4) (Variables|Default|GetChildActor5) (Variables|Default|GetChildActor6) (Variables|Default|GetChildActor7) (Variables|Default|GetChildActor8) (Variables|Default|GetChildActor9) (Variables|Default|GetChildActor10) (Variables|Default|GetChildActor11) (Variables|Default|GetChildActor12) (Variables|Default|GetChildActor13) (Variables|Default|GetChildActor14) (Variables|Default|GetChildActor15) (Variables|Default|GetChildActor16) (Variables|Default|GetChildActor17) (Variables|Default|GetChildActor18) (Variables|Default|GetChildActor19) (Variables|Default|GetChildActor20) (Variables|Default|GetChildActor21) (Variables|Default|GetChildActor22) (Variables|Default|GetChildActor23) (Variables|Default|GetChildActor24) (Variables|Default|GetChildActor25) (Variables|Default|GetChildActor26) (Variables|Default|GetChildActor27) (Variables|Default|GetChildActor28) (Variables|Default|GetChildActor29) (Variables|Default|GetChildActor30) (Variables|Default|GetChildActor31) (Variables|Default|GetChildActor32) (Variables|Default|GetChildActor33) (Variables|Default|GetChildActor34) (Variables|Default|GetChildActor35) (Variables|Default|GetChildActor36) (Variables|Default|GetChildActor37) (Variables|Default|GetChildActor38) (Variables|Default|GetChildActor39) (Variables|Default|GetChildActor40) (Variables|Default|GetChildActor41)))
      ;[1 1 1] Random Ether location
      ; (use of procedural curve for float precision)
      (bind _trp_replaying (CallFunction|TRPTestifTRPandGetRoadValues))
      (if _trp_replaying
        _
        (else
          (Variables|Default|SetTRP_ProceduralCurve (Math|Rotator|MakeRotator (Math|Random|RandomFloatinRange -2.5e+02 2.5e+02) 0.0 0.0))))
      (Transformation|SetRelativeLocation (Variables|Default|GetE1) (Math|Vector|MakeVector 1.5e+02 (.roll (Variables|Default|GetTRP_ProceduralCurve)) 0.0) false false)
      ;[1 1 1] Set end roads position
      (Transformation|AttachComponentToComponent _arrow4 (Variables|Default|GetChildActor41) "None" "KeepRelative" "KeepRelative" "KeepRelative" true)
      (Transformation|SetRelativeLocationAndRotation _arrow4 "300.000000, 0, 0" "0, 0, 0" false false)
      ;[1 1 1] Attach point
      (Transformation|SetWorldLocationAndRotation (Variables|Default|GetAttachPoint) (.location _returnvalue_2) (.rotation _returnvalue_2) false false))
    (:then_1
      ;[1 1 1] Set QuitLooping security position
      (Transformation|SetWorldLocationAndRotation (Variables|Default|GetQuitLooping) (.location _returnvalue) (.rotation _returnvalue) false false)
      ;[1 1 1] Hide frites
      (for _array_element (Variables|Default|GetFrites)
        (bind _aschild_actor_component (Utilities|Casting|CastToChildActorComponent _array_element))
        (bind _asbp_tile_3x_1_curve_frite (Utilities|Casting|CastToBP_Tile_3x1_CurveFrite (Variables|/Script/Engine.ChildActorComponent|GetChildActor _aschild_actor_component)))
        (Rendering|SetVisibility (Variables|/Game/Gameplay/Roads/Blueprints/Tiles/BP_Tile_3x1_CurveFrite.BP_Tile_3x1_CurveFrite_C|GetSM_RoadDragon _asbp_tile_3x_1_curve_frite) false false)))
    (:then_2
      ;[1 1 1] Random Crowd 1/5
      (if (Math|Random|RandomBoolwithWeight 0.5)
        (ChildActorComponent|SetChildActorClass (Variables|Default|GetCrowd) "/Game/Coco/Lab/Props/NearProps/RoadCrowd/BP_RoadCowd.BP_RoadCowd_C")))))