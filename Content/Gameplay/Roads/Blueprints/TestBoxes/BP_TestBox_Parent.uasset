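; Parent test box for the road system that checks whether the space it covers collides with a road or lies outside the world.
; TestIfOverlapingRoad gathers overlaps from every primitive component under Anchor, treating components tagged "landscape" as ground and anything else as road.
; It returns IsOverlapingRoad, plus IsOutOfWorld when no landscape is touched.
; BeginPlay and construction are empty, and the overlap logging is disconnected debug code.
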(event EventBeginPlay)

(fn ConstructionScript)

(fn TestifOverlapingRoad
  (for _array_element (Components|GetChildrenComponents (Variables|Default|GetAnchor) true)
    (bind _asprimitive_component (Utilities|Casting|CastToPrimitiveComponent _array_element))
    (for _array_element_2 (Class|PrimitiveComponent|GetOverlappingComponents _asprimitive_component)
      (if (Components|ComponentHasTag _array_element_2 "landscape")
        (LocalVariables|SetIsOverlapingAtLeastOneLandscape true)
        (else
          (LocalVariables|SetIsOverlapingAtLeastOneRoad true)))))
  (return (LocalVariables|GetIsOverlapingAtLeastOneRoad) (not (LocalVariables|GetIsOverlapingAtLeastOneLandscape))))