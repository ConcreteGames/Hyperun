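; A 3x1 "frite" slice tile of a curved road that carries an anchor collision and optional border decoration.
; AnchorCollRotation lerps the anchor from the previous frite's rotation to its own, which is re-cached and reset to alpha 0 after BeginPlay or on UpdateMyRotation.
; After a short delay for CurveCreator, it randomly spawns border rocks, or red signs on alternate tiles via a GameInstance toggle, and kills them on EndPlay.
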(event Custom|UpdateMyRotation
  (Variables|Default|SetMyRotation (Transformation|GetWorldRotation (Variables|Default|GetAnchorColl)))
  (CallFunction|AnchorCollRotation 0.0))

(event EventBeginPlay
  (Utilities|FlowControl|Delay 0.2) ; Need it to have time to let\nCurveCreator do its job
  (CallFunction|SpawnBorderRockswithRandom)
  (Variables|Default|SetMyRotation (Transformation|GetWorldRotation (Variables|Default|GetAnchorColl)))
  (CallFunction|AnchorCollRotation 0.0))

(event EventEndPlay
  (params (EndPlayReason :type EEndPlayReason%20Enum :default "Destroyed"))
  (for _array_element (Variables|Default|GetArrayOfBorderRocks)
    (Utilities|IsValid _array_element
      (:Is%20Valid
        (Default|KillMe _array_element false)))))

(fn ConstructionScript)

(fn AnchorCollRotation
  (params (Alpha :type Float%20%28single-precision%29))
  (Utilities|IsValid (Variables|Default|GetMyPreviousFrite)
    (:Is%20Valid
      (Transformation|SetWorldRotation (Variables|Default|GetAnchorColl) (Math|Rotator|Lerp(Rotator) (Variables|Default|GetMyPreviousFriteRotation) (Variables|Default|GetMyRotation) Alpha true) false false))
    (:Is%20Not%20Valid)))

(fn SpawnBorderRockswithRandom
  (bind _returnvalue (Game|GetGameInstance))
  (bind _asbp_game_instance (Utilities|Casting|CastToBP_GameInstance _returnvalue))
  (if (Variables|Default|GetNeedRock) ; If this frite need border rocks.\nFor exemple: QuarterPipe don't need rocks
    (bind _asbp_road_parent (Utilities|Casting|CastToBP_Road_Parent (Actor|GetParentActor)))
    (if (Variables|/Game/Gameplay/Roads/Blueprints/BP_Road_Parent.BP_Road_Parent_C|GetNeedRedSignInsteadOfBorderRocks _asbp_road_parent)
      ;[1 1 1] One on two redsigns alternance
      (if (Variables|/Game/Base/Blueprints/BP_GameInstance.BP_GameInstance_C|GetNeedRedSignAlternance _asbp_game_instance)
        (Variables|/Game/Base/Blueprints/BP_GameInstance.BP_GameInstance_C|SetNeedRedSignAlternance _asbp_game_instance false)
        (CallFunction|MaybeSpawnOneRock (Variables|Default|GetBorderRockSpawner_1) false true)
        (CallFunction|MaybeSpawnOneRock (Variables|Default|GetBorderRockSpawner_2) false true)
        (else
          (Variables|/Game/Base/Blueprints/BP_GameInstance.BP_GameInstance_C|SetNeedRedSignAlternance _asbp_game_instance true)))
      (else
        (CallFunction|MaybeSpawnOneRock (Variables|Default|GetBorderRockSpawner_1) true false)
        (CallFunction|MaybeSpawnOneRock (Variables|Default|GetBorderRockSpawner_2) true false)))))

(fn MaybeSpawnOneRock
  (params (ArrowSpawner :type Scene%20Component%20Object%20Reference) (Random :type Boolean) (NeedRedSign :type Boolean))
  (bind _returnvalue (Transformation|GetWorldTransform ArrowSpawner))
  (if Random
    (if (Math|Random|RandomBool)
      (bind _returnvalue_2 (Game|SpawnActorfromClass "/Game/Gameplay/BreakableProps/Blueprints/BP_BorderRock.BP_BorderRock_C" (Math|Transform|MakeTransform (.location _returnvalue) (.rotation _returnvalue) "1,1,1") "Undefined" 0 NeedRedSign 0 :!label _label))
      (Utilities|Array|Add (Variables|Default|GetArrayOfBorderRocks) _returnvalue_2))
    (else
      (goto _label))))