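; BP_Tile_3x3_NotInstance is a road tile Blueprint that randomizes the rocks placed along it.
; Its construction script gives each child of Rocks a random position along X, one of two opposite Y offsets, and random rotation and per-axis scale.
; The HideFloorCollider event sets Coll2 hidden in game.
; Logic to show one random road mesh under Visual exists but is disconnected, so it never runs.
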(event Custom|HideFloorCollider
  (Development|SetHiddeninGame (Variables|Default|GetColl2) true false))

(fn ConstructionScript
  (bind _returnvalue (Math|Random|RandomFloatinRange 0.4 1.0))
  ;[1 1 1] Place rocks
  (for _array_element (Components|GetChildrenComponents (Variables|Default|GetRocks) false)
    (Transformation|SetRelativeLocationAndRotation _array_element (Math|Vector|MakeVector (Math|Random|RandomFloatinRange 0.0 1.5e+03) (select (Math|Random|RandomBool) 7e+02 -7e+02) -1e+01) (Math|Random|RandomRotator false) false false)
    (Transformation|SetRelativeScale3D _array_element (Math|Vector|MakeVector _returnvalue _returnvalue _returnvalue))))