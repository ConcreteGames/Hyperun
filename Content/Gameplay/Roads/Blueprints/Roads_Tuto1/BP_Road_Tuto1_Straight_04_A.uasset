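; Straight road segment variant for the Tuto1 road set, built on a parent road Blueprint.
; Its construction script runs the parent's, then calls RandomNearProps on the NearProps scene with even odds of getting something and combinations allowed.
; It then fills ISMSpawnersArray with a hand-listed set of Arrow components, which by name serve as instanced static mesh spawn points.
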(fn ConstructionScript
  (|CallParentFunction)
  (CallFunction|RandomNearProps (Variables|Default|GetNearProps) 0.5 true 0.5)
  (Variables|Default|SetISMSpawnersArray (Utilities|Array|MakeArray (Variables|Default|GetArrow3) (Variables|Default|GetArrow4) (Variables|Default|GetArrow5) (Variables|Default|GetArrow13) (Variables|Default|GetArrow14) (Variables|Default|GetArrow15) (Variables|Default|GetArrow1) (Variables|Default|GetArrow2) (Variables|Default|GetArrow40) (Variables|Default|GetArrow17) (Variables|Default|GetArrow18) (Variables|Default|GetArrow19) (Variables|Default|GetArrow20) (Variables|Default|GetArrow21) (Variables|Default|GetArrow22) (Variables|Default|GetArrow23) (Variables|Default|GetArrow24) (Variables|Default|GetArrow25) (Variables|Default|GetArrow26) (Variables|Default|GetArrow27) (Variables|Default|GetArrow16) (Variables|Default|GetArrow29) (Variables|Default|GetArrow30) (Variables|Default|GetArrow31) (Variables|Default|GetArrow32) (Variables|Default|GetArrow33) (Variables|Default|GetArrow34) (Variables|Default|GetArrow35) (Variables|Default|GetArrow36) (Variables|Default|GetArrow37) (Variables|Default|GetArrow38) (Variables|Default|GetArrow39) (Variables|Default|GetArrow28) (Variables|Default|GetArrow41) (Variables|Default|GetArrow42) (Variables|Default|GetArrow43) (Variables|Default|GetArrow44) (Variables|Default|GetArrow45) (Variables|Default|GetArrow46) (Variables|Default|GetArrow47) (Variables|Default|GetArrow48) (Variables|Default|GetArrow49) (Variables|Default|GetArrow50) (Variables|Default|GetArrow51) (Variables|Default|GetArrow52) (Variables|Default|GetArrow53) (Variables|Default|GetArrow54) (Variables|Default|GetArrow55) (Variables|Default|GetArrow56) (Variables|Default|GetArrow57) (Variables|Default|GetArrow58) (Variables|Default|GetArrow59) (Variables|Default|GetArrow60) (Variables|Default|GetArrow61) (Variables|Default|GetArrow62) (Variables|Default|GetArrow63))))