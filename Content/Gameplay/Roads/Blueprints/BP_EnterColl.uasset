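; BP_EnterColl is a one-shot trigger actor that notifies its owning road piece when something begins overlapping it.
; On overlap, unless it sits at the world origin, it disables its collision as a do-once guard, calls EnterCollBeginOverlap on its RoadParent, then expires almost immediately via lifespan.
; A RoadParent that is not a BP_Road_Parent prints an error with the trigger's location; an older boolean do-once branch remains unconnected.
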(event OnComponentBeginOverlap(EnterColl)
  (params (OverlappedComponent :type Primitive%20Component%20Object%20Reference) (OtherActor :type Actor%20Object%20Reference) (OtherComp :type Primitive%20Component%20Object%20Reference) (OtherBodyIndex :type Integer) (bFromSweep :type Boolean) (SweepResult :type Hit%20Result%20Structure%20%28by%20ref%29))
  (if (Math|Vector|NotEqual(Vector) (Transformation|GetActorLocation) "0, 0, 0" 0.0001)
    ;[1 1 1] Better DoOne custom
    (Collision|SetCollisionEnabled (Variables|Default|GetEnterColl) "NoCollision")
    (bind _asbp_road_parent (Utilities|Casting|CastToBP_Road_Parent (Variables|Default|GetRoadParent))
      (:then
        (Default|EnterCollBeginOverlap _asbp_road_parent)
        (Actor|SetLifeSpan 0.001))
      (:CastFailed
        (Development|PrintString "BP_EnterRoadColl: My parent is not a \"BP_Road_Parent\"" true true "(R=1.000000,G=0.000000,B=0.000000,A=1.000000)" 1.0) ; error log
        (Development|PrintString (Utilities|String|ToString(Vector) (Transformation|GetActorLocation)))))))

(fn ConstructionScript)