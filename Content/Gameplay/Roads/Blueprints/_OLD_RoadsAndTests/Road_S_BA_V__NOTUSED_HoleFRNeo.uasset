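; Road segment Blueprint, marked unused in an old roads-and-tests folder, that lays out child pieces into a pitched road profile.
; Its construction script runs the parent's, then applies repeated relative offsets and pitches to groups of components: a downward-pitched run, then an upward one.
; Transition sections snap onto the preceding run's last component and use zero relative pitch.
; AttachPoint snaps to the final transition and is offset forward to mark the segment's end.
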(fn ConstructionScript
  (bind _firsttrans1 (Variables|Default|GetFirstTrans1))
  (bind _first2 (Variables|Default|GetFirst2))
  (bind _attachpoint (Variables|Default|GetAttachPoint))
  (bind _last2 (Variables|Default|GetLast2))
  (bind _firsttrans2 (Variables|Default|GetFirstTrans2))
  (|CallParentFunction)
  (Transformation|AttachComponentToComponent _attachpoint (Variables|Default|GetLastTrans2) "None" "SnapToTarget" "SnapToTarget" "SnapToTarget" true)
  (Utilities|FlowControl|Sequence
    (:then_0
      (Transformation|SetRelativeLocationAndRotation (Variables|Default|GetChildActor1) "300.000000, 0, 0" (Math|Rotator|MakeRotator 0.0 -8.0 0.0) false false)
      ;[1 1 1] Transition 1
      (Transformation|AttachComponentToComponent _firsttrans1 (Variables|Default|GetLast1) "None" "SnapToTarget" "SnapToTarget" "SnapToTarget" true)
      (Transformation|SetRelativeLocationAndRotation _firsttrans1 "300.000000, 0, 0" (Math|Rotator|MakeRotator 0.0 0.0 0.0) false false)
      (Transformation|AttachComponentToComponent _first2 (Variables|Default|GetLastTrans1) "None" "SnapToTarget" "SnapToTarget" "SnapToTarget" true)
      (Transformation|SetRelativeLocationAndRotation _first2 "1500.000000, 0, 0" (Math|Rotator|MakeRotator 0.0 0.0 0.0) false false)
      (Transformation|SetRelativeLocationAndRotation _last2 "300.000000, 0, 0" (Math|Rotator|MakeRotator 0.0 13.5 0.0) false false)
      ;[1 1 1] Transition 2
      (Transformation|AttachComponentToComponent _firsttrans2 _last2 "None" "SnapToTarget" "SnapToTarget" "SnapToTarget" true)
      (Transformation|SetRelativeLocationAndRotation _firsttrans2 "300.000000, 0, 0" (Math|Rotator|MakeRotator 0.0 0.0 0.0) false false)
      (Transformation|SetRelativeLocationAndRotation (Variables|Default|GetChildActor14) "1500.000000, 0, 0" (Math|Rotator|MakeRotator 0.0 0.0 0.0) false false))
    (:then_1
      (Transformation|SetRelativeLocationAndRotation _attachpoint "1500.000000, 0, 0" "0, 0, 0" false false) ; End
    )))