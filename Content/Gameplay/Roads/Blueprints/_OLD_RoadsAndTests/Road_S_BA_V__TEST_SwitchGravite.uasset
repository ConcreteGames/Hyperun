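; Test road segment for a gravity switch that carries the player bike through a twist.
; Each tick it tracks the bike's local X between start and end markers, attaching the bike to the trigger plane while inside and detaching it otherwise.
; Normalized progress samples two float curves that lift the plane and roll it up to a half turn, scaled from the curve values.
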(event EventTick
  (params (DeltaSeconds :type Float%20%28single-precision%29))
  (bind _switch_startpoint (Variables|Default|GetSwitch_StartPoint))
  (bind _switch_endpoint (Variables|Default|GetSwitch_EndPoint))
  (bind _switchtriggerplane (Variables|Default|GetSwitchTriggerPlane))
  (bind _switch_bikelocation (Variables|Default|GetSwitch_BikeLocation))
  (bind _relativelocation (Variables|/Script/Engine.SceneComponent|GetRelativeLocation _switchtriggerplane))
  (bind _relativelocation_2 (Variables|/Script/Engine.SceneComponent|GetRelativeLocation _switch_bikelocation))
  (bind _relativelocation_3 (Variables|/Script/Engine.SceneComponent|GetRelativeLocation _switch_startpoint))
  (bind _relativelocation_4 (Variables|/Script/Engine.SceneComponent|GetRelativeLocation _switch_endpoint))
  (bind _returnvalue (- (.x _relativelocation_2) (.x _relativelocation_3)))
  (bind _returnvalue_2 (- (.x _relativelocation_4) (.x _relativelocation_3)))
  (bind _returnvalue_3 (/ _returnvalue _returnvalue_2))
  (bind _asbp_bike_parent (Utilities|Casting|CastToBP_Bike_Parent (Game|Player|GetPlayerPawn 0)))
  (Transformation|SetWorldLocation (Variables|Default|GetSwitch_BikeLocation) (Transformation|GetActorLocation _asbp_bike_parent) false false)
  (if (and (> (.x _relativelocation_2) (.x _relativelocation_3)) (< (.x _relativelocation_2) (.x _relativelocation_4)))
    (Class|Actor|AttachRootComponentto _asbp_bike_parent (Variables|Default|GetSwitchTriggerPlane) "None" "KeepWorldPosition" true)
    (Transformation|SetRelativeLocationAndRotation _switchtriggerplane (Math|Vector|MakeVector (.x _relativelocation) (.y _relativelocation) (* (Math|Curves|GetFloatValue (Variables|Default|GetCRV_Switch_Loc) _returnvalue_3) 1.5e+03)) (Math|Rotator|MakeRotator (* (Math|Curves|GetFloatValue (Variables|Default|GetCRV_Switch_Rota) _returnvalue_3) 1.8e+02) 0.0 0.0) false false)
    (else
      (Transformation|DetachFromActor _asbp_bike_parent "KeepWorld" "KeepWorld" "KeepWorld"))))

(fn ConstructionScript
  (|CallParentFunction))