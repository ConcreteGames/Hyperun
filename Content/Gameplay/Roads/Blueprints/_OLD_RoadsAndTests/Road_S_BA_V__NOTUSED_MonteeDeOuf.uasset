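; Unused legacy road segment Blueprint that appears to form a steep climb from a series of child actor pieces.
; Its construction script calls the parent script, snaps AttachPoint to the LAST piece, then gives every piece the same forward offset and slight pitch, presumably compounding through nesting into a curve.
; End and AttachPoint get the same forward offset, while an alternative placement using End's world transform is never executed.
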(fn ConstructionScript
  (|CallParentFunction)
  (Transformation|AttachComponentToComponent (Variables|Default|GetAttachPoint) (Variables|Default|GetLAST) "None" "SnapToTarget" "SnapToTarget" "SnapToTarget" true)
  (Transformation|SetRelativeLocationAndRotation (Variables|Default|GetChildActor) "300.000000, 0, 0" (Math|Rotator|MakeRotator 0.0 2.0 0.0) false false)
  (Transformation|SetRelativeLocationAndRotation (Variables|Default|GetEnd) "300.000000, 0, 0" "0, 0, 0" false false))