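; Test road Blueprint that builds a road section from a set of child segment components in its construction script.
; Each segment gets a fixed forward relative offset and a small random pitch and roll, varying the road on each construction.
; AttachPoint is re-parented dynamically to the LAST segment because its parent cannot be changed by hand, then offset forward.
; RoadVertexSnap finally runs on FIRSTROAD.
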(fn ConstructionScript
  (|CallParentFunction)
  ;[1 1 1] Impossible de changer la parentée à la main, donc dynamique
  (Transformation|AttachComponentToComponent (Variables|Default|GetAttachPoint) (Variables|Default|GetLAST) "None" "SnapToTarget" "SnapToTarget" "SnapToTarget" true)
  (Transformation|SetRelativeLocationAndRotation (Variables|Default|GetFirstChild) "300.000000, 0, 0" (Math|Rotator|MakeRotator (Math|Random|RandomFloatinRange -5.0 5.0) (Math|Random|RandomFloatinRange -5.0 5.0) 0.0) false false)
  (Transformation|SetRelativeLocationAndRotation (Variables|Default|GetAttachPoint) "300.000000, 0, 0" (Math|Rotator|MakeRotator 0.0 0.0 0.0) false false)
  (CallFunction|RoadVertexSnap (Variables|Default|GetFIRSTROAD)))