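; Legacy level 1 procedural road piece that builds a sharp downward step from three arrow-based ISM spawners.
; Its construction script randomly pitches Arrow1 down, then counters that pitch on Arrow2, with a coin-flip chance of a slight final rise.
; Random values are stored in TRP variables and only rolled when not replaying, so replays can reuse the shape.
; AttachPoint snaps to Arrow2 and offsets forward to mark the piece's end.
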(fn ConstructionScript
  (bind _attachpoint (Variables|Default|GetAttachPoint))
  (|CallParentFunction)
  (Variables|Default|SetISMSpawnersArray (Utilities|Array|MakeArray (Variables|Default|GetArrow) (Variables|Default|GetArrow1) (Variables|Default|GetArrow2)))
  ;[1 1 1] random 2 float
  (bind _trp_replaying (CallFunction|TRPTestifTRPandGetRoadValues))
  (if _trp_replaying
    _
    (else
      (Variables|Default|SetTRP_ProceduralCurve (Math|Rotator|MakeRotator 0.0 (Math|Random|RandomFloatinRange -1e+01 -3e+01) (Math|Random|RandomFloatinRange 2.0 1e+01)))
      (Variables|Default|SetTRP_EtherPattern (Math|Conversions|ToInteger(Boolean) (Math|Random|RandomBool)))))
  ;[1 1 1] Random pitch
  (Transformation|SetRelativeRotation (Variables|Default|GetArrow1) (Math|Rotator|MakeRotator 0.0 (.pitch (Variables|Default|GetTRP_ProceduralCurve)) 0.0) false false)
  (Transformation|SetRelativeRotation (Variables|Default|GetArrow2) (Math|Rotator|MakeRotator 0.0 (select (Math|Conversions|ToBoolean(Integer) (Variables|Default|GetTRP_EtherPattern)) (+ (* (.pitch (Variables|Default|GetTRP_ProceduralCurve)) -1.0) (.yaw (Variables|Default|GetTRP_ProceduralCurve))) (* (.pitch (Variables|Default|GetTRP_ProceduralCurve)) -1.0)) 0.0) false false)
  ;[1 1 1] Attach point
  (Transformation|AttachComponentToComponent _attachpoint (Variables|Default|GetArrow2) "None" "SnapToTarget" "SnapToTarget" "SnapToTarget" true)
  (Transformation|SetRelativeLocationAndRotation _attachpoint "1500.000000, 0, 0" "0, 0, 0" false false) ; End
  (Transformation|SetWorldScale3D _attachpoint "1.000000,1.000000,1.000000"))