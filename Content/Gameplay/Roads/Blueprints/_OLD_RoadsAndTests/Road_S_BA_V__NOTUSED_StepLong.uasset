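; A road segment Blueprint, marked old and unused by its path, that shapes a long downward step with random slope.
; The construction script calls its parent, then bends a chain of child-actor pieces by a random negative pitch per piece, followed by a long straight middle.
; A second chain cancels that pitch, with a 50% chance of curving slightly upward.
; AttachPoint is snapped and offset past the last piece to mark the segment's end.
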(fn ConstructionScript
  (bind _attachpoint (Variables|Default|GetAttachPoint))
  (bind _trans (Variables|Default|GetTrans))
  (bind _first2 (Variables|Default|GetFirst2))
  (|CallParentFunction)
  (Variables|Default|SetRandomPitch (Math|Random|RandomFloatinRange -6.0 -2.0))
  (Transformation|AttachComponentToComponent _attachpoint (Variables|Default|GetLast2) "None" "SnapToTarget" "SnapToTarget" "SnapToTarget" true)
  (Utilities|FlowControl|Sequence
    (:then_0
      (Transformation|SetRelativeLocationAndRotation (Variables|Default|GetChildActor) "300.000000, 0, 0" (Math|Rotator|MakeRotator 0.0 (Variables|Default|GetRandomPitch) 0.0) false false)
      (Transformation|AttachComponentToComponent _trans (Variables|Default|GetLastPart1) "None" "SnapToTarget" "SnapToTarget" "SnapToTarget" true)
      (Transformation|SetRelativeLocationAndRotation _trans "300.000000, 0, 0" (Math|Rotator|MakeRotator 0.0 0.0 0.0) false false)
      ;[1 1 1] middle
      (Transformation|AttachComponentToComponent _first2 (Variables|Default|GetTrans) "None" "SnapToTarget" "SnapToTarget" "SnapToTarget" true)
      (Transformation|SetRelativeLocationAndRotation _first2 "1500.000000, 0, 0" (Math|Rotator|MakeRotator 0.0 0.0 0.0) false false)
      (Transformation|SetRelativeLocationAndRotation (Variables|Default|GetLast2) "300.000000, 0, 0" (Math|Rotator|MakeRotator 0.0 (select (Math|Random|RandomBool) (+ (* (Variables|Default|GetRandomPitch) -1.0) (Math|Random|RandomFloatinRange 2.0 4.0)) (* (Variables|Default|GetRandomPitch) -1.0)) 0.0) false false))
    (:then_1
      (Transformation|SetRelativeLocationAndRotation _attachpoint "300.000000, 0, 0" "0, 0, 0" false false) ; End
    )))