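; Legacy Level 1 straight road segment ("FallingFour_L"), built from spawner components and four chains of curve "frite" tile child actors.
; The construction script fills the ISM spawner and frite arrays, then places AttachPoint beyond Arrow4 to mark the segment's end.
; Disconnected graphs, which never run, hide the frite meshes, curve and chain the four rows via roll/pitch and anchors, or refresh tile rotations.
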(fn ConstructionScript
  (bind _attachpoint (Variables|Default|GetAttachPoint))
  (|CallParentFunction)
  (Variables|Default|SetISMSpawnersArray (Utilities|Array|MakeArray (Variables|Default|GetSpawner_Corner_L3) (Variables|Default|GetArrow) (Variables|Default|GetArrow1) (Variables|Default|GetArrow2) (Variables|Default|GetArrow3) (Variables|Default|GetArrow4) (Variables|Default|GetSpawner_Corner_L2) (Variables|Default|GetSpawner_Corner_L4) (Variables|Default|GetArrow6) (Variables|Default|GetArrow5) (Variables|Default|GetSpawner_Corner_L1) (Variables|Default|GetSpawner_FallingFour_L)))
  ;[1 1 1] Make arrays of frites
  (Variables|Default|SetFrites1 (Utilities|Array|MakeArray (Variables|Default|Get1_Frite1) (Variables|Default|GetChildActor2) (Variables|Default|GetChildActor3) (Variables|Default|GetChildActor4) (Variables|Default|GetChildActor5) (Variables|Default|GetChildActor6) (Variables|Default|GetChildActor7) (Variables|Default|GetChildActor) (Variables|Default|GetChildActor1) (Variables|Default|GetChildActor14) (Variables|Default|GetChildActor15) (Variables|Default|GetChildActor16) (Variables|Default|GetChildActor17) (Variables|Default|GetChildActor18) (Variables|Default|GetChildActor19) (Variables|Default|GetLastFrite_1)))
  (Variables|Default|SetFrites2 (Utilities|Array|MakeArray (Variables|Default|Get2_Frite1) (Variables|Default|GetChildActor8) (Variables|Default|GetChildActor9) (Variables|Default|GetChildActor10) (Variables|Default|GetChildActor11) (Variables|Default|GetChildActor12) (Variables|Default|GetChildActor13) (Variables|Default|GetChildActor20) (Variables|Default|GetChildActor21) (Variables|Default|GetChildActor26) (Variables|Default|GetChildActor27) (Variables|Default|GetChildActor28) (Variables|Default|GetChildActor29) (Variables|Default|GetChildActor30) (Variables|Default|GetChildActor22) (Variables|Default|Get2_LastFrite)))
  (Variables|Default|SetFrites3 (Utilities|Array|MakeArray (Variables|Default|Get3_Frite1) (Variables|Default|GetChildActor37) (Variables|Default|GetChildActor38) (Variables|Default|GetChildActor39) (Variables|Default|GetChildActor40) (Variables|Default|GetChildActor41) (Variables|Default|GetChildActor42) (Variables|Default|GetChildActor43) (Variables|Default|GetChildActor44) (Variables|Default|GetChildActor45) (Variables|Default|GetChildActor46) (Variables|Default|GetChildActor47) (Variables|Default|GetChildActor48) (Variables|Default|GetChildActor49) (Variables|Default|GetChildActor23) (Variables|Default|Get3_LastFrite)))
  (Variables|Default|SetFrites4 (Utilities|Array|MakeArray (Variables|Default|Get4_Frite1) (Variables|Default|GetChildActor55) (Variables|Default|GetChildActor56) (Variables|Default|GetChildActor57) (Variables|Default|GetChildActor58) (Variables|Default|GetChildActor59) (Variables|Default|GetChildActor60) (Variables|Default|GetChildActor61) (Variables|Default|GetChildActor62) (Variables|Default|GetChildActor63) (Variables|Default|GetChildActor64) (Variables|Default|GetChildActor65) (Variables|Default|GetChildActor66) (Variables|Default|GetChildActor67) (Variables|Default|GetChildActor24) (Variables|Default|Get4_LastFrite)))
  ;[1 1 1] On positionne l'Attach point à la fin de la dernière partie
  (Transformation|AttachComponentToComponent _attachpoint (Variables|Default|GetArrow4) "None" "KeepRelative" "KeepRelative" "KeepRelative" true)
  (Transformation|SetRelativeTransform _attachpoint (Math|Transform|MakeTransform "1500.000000, 0, 0" "0, 0, 0" "1,1,1") false false)
  (Transformation|SetWorldScale3D _attachpoint "1.000000,1.000000,1.000000"))