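; Old test Blueprint for a straight level 1 road piece, named as a right-side "FallingFour" variant.
; Its construction script registers arrows and corner and falling-four spawners in ISMSpawnersArray, then attaches AttachPoint beyond the last arrow to mark the piece's end.
; It then refreshes the rotation of BP_Tile_3x1_CurveFrite child actors under Roads.
; Logic for hiding or chaining frites is disconnected, and SetFrite, which randomizes roll and pitch, is never called here.
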(fn ConstructionScript
  (bind _attachpoint (Variables|Default|GetAttachPoint))
  (|CallParentFunction)
  (Variables|Default|SetFrites2 (Utilities|Array|MakeArray 0 0 0 0 0 0 0 0 0 0 0 0 0 0 0 0))
  (Variables|Default|SetFrites3 (Utilities|Array|MakeArray 0 0 0 0 0 0 0 0 0 0 0 0 0 0 0 0))
  (Variables|Default|SetFrites4 (Utilities|Array|MakeArray 0 0 0 0 0 0 0 0 0 0 0 0 0 0 0 0))
  (Variables|Default|SetISMSpawnersArray (Utilities|Array|MakeArray (Variables|Default|GetSpawner_Corner_R3) (Variables|Default|GetSpawner_Corner_R4) (Variables|Default|GetArrow) (Variables|Default|GetArrow1) (Variables|Default|GetArrow2) (Variables|Default|GetArrow3) (Variables|Default|GetSpawner_Corner_R2) (Variables|Default|GetArrow7) (Variables|Default|GetArrow6) (Variables|Default|GetSpawner_Corner_R) (Variables|Default|GetArrow4) (Variables|Default|GetArrow5) (Variables|Default|GetSpawner_FallingFour_R)))
  ;[1 1 1] On positionne l'Attach point à la fin de la dernière partie
  (Transformation|AttachComponentToComponent _attachpoint (Variables|Default|GetArrow5) "None" "KeepRelative" "KeepRelative" "KeepRelative" true)
  (Transformation|SetRelativeTransform _attachpoint (Math|Transform|MakeTransform "1500.000000, 0, 0" "0, 0, 0" "1,1,1") false false)
  (Transformation|SetWorldScale3D _attachpoint "1.000000,1.000000,1.000000")
  ;[1 1 1] On met à jour toutes les frites de toutes les roads enfants
  (for _array_element (Components|GetChildrenComponents (Variables|Default|GetRoads) true)
    (bind _aschild_actor_component (Utilities|Casting|CastToChildActorComponent _array_element))
    (bind _asbp_tile_3x_1_curve_frite (Utilities|Casting|CastToBP_Tile_3x1_CurveFrite (Variables|/Script/Engine.ChildActorComponent|GetChildActor _aschild_actor_component)))
    (Default|UpdateMyRotation _asbp_tile_3x_1_curve_frite)))

(fn SetFrite
  (params (FirstFrite :type Scene%20Component%20Object%20Reference) (RollMin :type Float%20%28single-precision%29) (RollMax :type Float%20%28single-precision%29) (PitchMin :type Float%20%28single-precision%29) (PitchMax :type Float%20%28single-precision%29))
  (for _array_element (Components|GetChildrenComponents FirstFrite true)
    (bind _aschild_actor_component (Utilities|Casting|CastToChildActorComponent _array_element))
    (Utilities|Casting|CastToBP_Tile_3x1_CurveFrite (Variables|/Script/Engine.ChildActorComponent|GetChildActor _aschild_actor_component))
    (LocalVariables|SetCurrentFrite _array_element)
    (Transformation|SetRelativeLocationAndRotation (LocalVariables|GetCurrentFrite) "300.000000, 0, 0" (Math|Rotator|MakeRotator (Math|Random|RandomFloatinRange RollMin RollMax) (Math|Random|RandomFloatinRange PitchMin PitchMax) 0.0) false false :!pinned true) ; 1st group of frites
  ))