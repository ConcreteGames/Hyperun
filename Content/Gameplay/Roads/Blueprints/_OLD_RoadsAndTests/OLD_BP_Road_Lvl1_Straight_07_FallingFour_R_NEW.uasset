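; Legacy level 1 straight road segment Blueprint (FallingFour R variant), built from four runs of BP_Tile_3x1_CurveFrite child actors.
; The construction script caches the frite runs and ISM spawner points, moves AttachPoint to the segment's end and calls UpdateMyRotation on each road tile.
; Logic to hide frites or chain the runs with roll/pitch curves is disconnected.
; SetFrite randomizes child tile roll and pitch but is not called here.
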(fn ConstructionScript
  (bind _attachpoint (Variables|Default|GetAttachPoint))
  (|CallParentFunction)
  (Variables|Default|SetFrites1 (Utilities|Array|MakeArray (Variables|Default|Get1_Frite1) (Variables|Default|GetChildActor2) (Variables|Default|GetChildActor3) (Variables|Default|GetChildActor4) (Variables|Default|GetChildActor5) (Variables|Default|GetChildActor6) (Variables|Default|GetChildActor7) (Variables|Default|GetChildActor) (Variables|Default|GetChildActor1) (Variables|Default|GetChildActor14) (Variables|Default|GetChildActor15) (Variables|Default|GetChildActor16) (Variables|Default|GetChildActor17) (Variables|Default|GetChildActor18) (Variables|Default|GetChildActor19) (Variables|Default|GetLastFrite_1)))
  (Variables|Default|SetFrites2 (Utilities|Array|MakeArray (Variables|Default|Get2_Frite1) (Variables|Default|GetChildActor8) (Variables|Default|GetChildActor9) (Variables|Default|GetChildActor10) (Variables|Default|GetChildActor11) (Variables|Default|GetChildActor12) (Variables|Default|GetChildActor13) (Variables|Default|GetChildActor20) (Variables|Default|GetChildActor21) (Variables|Default|GetChildActor26) (Variables|Default|GetChildActor27) (Variables|Default|GetChildActor28) (Variables|Default|GetChildActor29) (Variables|Default|GetChildActor30) (Variables|Default|GetChildActor31) (Variables|Default|Get2_LastFrite)))
  (Variables|Default|SetFrites3 (Utilities|Array|MakeArray (Variables|Default|Get3_Frite1) (Variables|Default|GetChildActor37) (Variables|Default|GetChildActor38) (Variables|Default|GetChildActor39) (Variables|Default|GetChildActor40) (Variables|Default|GetChildActor41) (Variables|Default|GetChildActor42) (Variables|Default|GetChildActor43) (Variables|Default|GetChildActor44) (Variables|Default|GetChildActor45) (Variables|Default|GetChildActor46) (Variables|Default|GetChildActor47) (Variables|Default|GetChildActor48) (Variables|Default|GetChildActor49) (Variables|Default|GetChildActor50) (Variables|Default|Get3_LastFrite)))
  (Variables|Default|SetFrites4 (Utilities|Array|MakeArray (Variables|Default|Get4_Frite1) (Variables|Default|GetChildActor55) (Variables|Default|GetChildActor56) (Variables|Default|GetChildActor57) (Variables|Default|GetChildActor58) (Variables|Default|GetChildActor59) (Variables|Default|GetChildActor60) (Variables|Default|GetChildActor61) (Variables|Default|GetChildActor62) (Variables|Default|GetChildActor63) (Variables|Default|GetChildActor64) (Variables|Default|GetChildActor65) (Variables|Default|GetChildActor66) (Variables|Default|GetChildActor67) (Variables|Default|GetChildActor68) (Variables|Default|Get4_LastFrite)))
  (Variables|Default|SetISMSpawnersArray (Utilities|Array|MakeArray (Variables|Default|GetSpawner_Corner_R3) (Variables|Default|GetSpawner_Corner_R4) (Variables|Default|GetArrow) (Variables|Default|GetArrow1) (Variables|Default|GetArrow2) (Variables|Default|GetArrow3) (Variables|Default|GetSpawner_Corner_R2) (Variables|Default|GetArrow7) (Variables|Default|GetArrow6) (Variables|Default|GetSpawner_Corner_R) (Variables|Default|GetArrow4) (Variables|Default|GetArrow5) (Variables|Default|GetSpawner_FallingFour_R)))
  ;[1 1 1] On positionne l'Attach point à la fin de la dernière partie
  (Transformation|AttachComponentToComponent _attachpoint (Variables|Default|GetArrow5) "None" "KeepRelative" "KeepRelative" "KeepRelative" true)
  (Transformation|SetRelativeTransform _attachpoint (Math|Transform|MakeTransform "1500.000000, 0, 0" "0, 0, 0" "1,1,1") false false)
  (Transformation|SetWorldScale3D _attachpoint "1.000000,1.000000,1.000000")
  ;[1 1 1] On met à jour toutes les frites de toutes les roads enfants
  (for _array_element (Components|GetChildrenComponents (Variables|Default|GetRoads) true)
    (bind _aschild_actor_component (Utilities|Casting|CastToChildActorComponent _array_element))
    (bind _asbp_tile_3x_1_curve_frite (Utilities|Casting|CastToBP_Tile_3x1_CurveFrite (Variables|/Script/Engine.ChildActorComponent|GetChildActor _aschild_actor_component)))
    (Default|UpdateMyRotation _asbp_tile_3x_1_curve_frite)))

(fn SetFrite
  (params (FirstFrite :type Scene%20Component%20Object%20Reference) (RollMin :type Float%20%28single-precision%29) (RollMax :type Float%20%28single-precision%29) (PitchMin :type Float%20%28single-precision%29) (PitchMax :type Float%20%28single-precision%29))
  (for _array_element (Components|GetChildrenComponents FirstFrite true)
    (bind _aschild_actor_component (Utilities|Casting|CastToChildActorComponent _array_element))
    (Utilities|Casting|CastToBP_Tile_3x1_CurveFrite (Variables|/Script/Engine.ChildActorComponent|GetChildActor _aschild_actor_component))
    (LocalVariables|SetCurrentFrite _array_element)
    (Transformation|SetRelativeLocationAndRotation (LocalVariables|GetCurrentFrite) "300.000000, 0, 0" (Math|Rotator|MakeRotator (Math|Random|RandomFloatinRange RollMin RollMax) (Math|Random|RandomFloatinRange PitchMin PitchMax) 0.0) false false :!pinned true) ; 1st group of frites
  ))