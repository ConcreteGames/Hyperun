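; Old level 1 road piece Blueprint, a sharp-rise curved variant of the straight segment, with a randomized bend.
; On construction it rotates the Arrow by a random angle within a fixed range, reusing the existing curve value when TRP is replaying.
; AttachPoint snaps to the Arrow and is offset along it, so it follows the bend.
; The Arrow is registered as the sole entry in the ISM spawners array.
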(fn ConstructionScript
  (bind _attachpoint (Variables|Default|GetAttachPoint))
  (bind _arrow (Variables|Default|GetArrow))
  (|CallParentFunction)
  (Utilities|FlowControl|Sequence
    (:then_0
      ;[1 1 1] random curve
      (bind _trp_replaying (CallFunction|TRPTestifTRPandGetRoadValues))
      (if _trp_replaying
        _
        (else
          (Variables|Default|SetTRP_ProceduralCurve (Math|Rotator|MakeRotator 0.0 (Math|Random|RandomFloatinRange 1e+01 2e+01) 0.0))))
      (Transformation|SetRelativeRotation _arrow (Variables|Default|GetTRP_ProceduralCurve) false false)
      (Transformation|AttachComponentToComponent _attachpoint _arrow "None" "SnapToTarget" "SnapToTarget" "SnapToTarget" true)
      (Transformation|SetRelativeLocationAndRotation _attachpoint "1500.000000, 0, 0" (Math|Rotator|MakeRotator 0.0 0.0 0.0) false false)
      (Transformation|SetWorldScale3D _attachpoint "1.000000,1.000000,1.000000"))
    (:then_1
      (Variables|Default|SetISMSpawnersArray (Utilities|Array|MakeArray (Variables|Default|GetArrow))))))