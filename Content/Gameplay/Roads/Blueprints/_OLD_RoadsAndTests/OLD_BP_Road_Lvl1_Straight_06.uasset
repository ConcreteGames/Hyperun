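; Retired level 1 straight road segment Blueprint, variant 06, that randomizes the lateral layout of its doors.
; After the parent construction script runs, it picks a random starting side and loops over the direct children of the Doors component.
; Each child alternates between positive and negative Y at a random distance from the center, keeping its X and Z.
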(fn ConstructionScript
  (bind _returnvalue (Math|Random|RandomFloatinRange 4.5e+02 2.5e+02))
  (|CallParentFunction)
  (LocalVariables|SetBool (Math|Random|RandomBool))
  (for _array_element (Components|GetChildrenComponents (Variables|Default|GetDoors) false)
    ;[1 1 1] Switcher de bool
    (if (LocalVariables|GetBool)
      (LocalVariables|SetBool false)
      (else
        (LocalVariables|SetBool true)))
    (Transformation|SetRelativeLocation _array_element (Math|Vector|MakeVector (.x (Variables|/Script/Engine.SceneComponent|GetRelativeLocation _array_element)) (select (LocalVariables|GetBool) _returnvalue (* _returnvalue -1.0)) (.z (Variables|/Script/Engine.SceneComponent|GetRelativeLocation _array_element))) false false)))