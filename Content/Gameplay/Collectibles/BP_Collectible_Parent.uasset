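; Base Blueprint for ether collectibles that the player's bike picks up as saved money, singly or as a bunch worth more.
; On spawn it adds its base mesh to a shared BP_ISMBank and plays a scale bounce.
; The Road calls Activation, which after a short delay enables pickup, reveals the visual and starts bobbing.
; Bike overlap credits and saves, hides it, then destroys it later; EndPlay removes bank instance index 0, not its own.
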(event OnComponentBeginOverlap(Box)
  (params (OverlappedComponent :type Primitive%20Component%20Object%20Reference) (OtherActor :type Actor%20Object%20Reference) (OtherComp :type Primitive%20Component%20Object%20Reference) (OtherBodyIndex :type Integer) (bFromSweep :type Boolean) (SweepResult :type Hit%20Result%20Structure%20%28by%20ref%29))
  ;[1 1 1] Coll
  (if (Variables|Default|GetIsEnable) ; Si activé
    ;[1 1 1] Si collisionne la moto, il est récolté
    (bind _asbp_bike_parent (Utilities|Casting|CastToBP_Bike_Parent OtherActor))
    (Default|GetOneCollectible _asbp_bike_parent (Variables|Default|GetImABunchOfCOllectible))
    (CallFunction|SaveEth)
    (for _array_element (Components|GetChildrenComponents (Variables|Default|GetAtomAnimationAnchor) true)
      (Rendering|SetVisibility _array_element false false))
    ;[1 1 1] test 1>10 pour éviter ISM dépop le mauvais
    (Utilities|FlowControl|Delay 1e+01)
    (Actor|SetLifeSpan 0.01 :!pinned true) ; Autodestruction
  ))

(event Custom|Activation
  ;[1 1 1] Fix à l'arrache du bug
  ; de choppage d'ether au start
  (Utilities|FlowControl|Delay 0.2) ; Sinon les ethers collisionnent avec la bike\nen 0,0,0... wtf
  (Variables|Default|SetIsEnable true :!pinned true) ; Devient actif,\nappelé par la Road
  ;[1 1 1] Show visual
  (Development|SetHiddeninGame (Variables|Default|GetVisual) false true)
  ;[1 1 1] Random orientation
  (Transformation|SetRelativeRotation (Variables|Default|GetBP_Atom) (Math|Random|RandomRotator false) false false)
  (Variables|Default|SetZAtStart (.z (Variables|/Script/Engine.SceneComponent|GetRelativeLocation (Variables|Default|GetAtomAnimationAnchor))))
  ;[1 1 1] Oscillation Z
  (bind _newtrack_0 (Timeline|Timeline_0 PlayFromStart)
    (:Update
      (Transformation|SetRelativeLocation (Variables|Default|GetAtomAnimationAnchor) (Math|Vector|MakeVector 0.0 0.0 (+ (* _newtrack_0 15.0) (Variables|Default|GetZAtStart))) false false))))

(event EventBeginPlay
  (bind _spawner_ethbase (Variables|Default|GetSpawner_EthBase))
  (bind _returnvalue (Transformation|GetWorldTransform _spawner_ethbase))
  ;[0.149 1 0] BEGIN  PLAY
  (Utilities|FlowControl|Sequence
    (:then_0
      ;[1 1 1] EthBase
      (Class|LowEntryExtendedStandardLibrary|DelayFrames 1)
      (bind _outactors (Actor|GetAllActorsOfClass "/Game/Gameplay/Roads/Blueprints/BP_ISMBank.BP_ISMBank_C"))
      (Utilities|IsValid (Utilities|Array|Get(acopy) _outactors)
        (:Is%20Valid
          (Variables|Default|SetBP_ISMBank_REF (Utilities|Array|Get(acopy) _outactors))
          (Components|InstancedStaticMesh|AddInstance (Variables|/Game/Gameplay/Roads/Blueprints/BP_ISMBank.BP_ISMBank_C|GetISM_EthBase (Variables|Default|GetBP_ISMBank_REF)) (Math|Transform|MakeTransform (.location _returnvalue) (.rotation _returnvalue) "1.000000,1.000000,1.000000"))
          (Variables|Default|SetISM_EthBase (+ (Variables|Default|GetISM_EthBase) 1)))))
    (:then_1
      (if (Variables|Default|GetIsIvisibleAtStart)
        _
        (else
          ;[1 1 1] De base, on cache le visuel
          (Development|SetHiddeninGame (Variables|Default|GetVisual) true true)))
      ;[1 1 1] Bounce
      (Components|Timeline|SetTimelineLength (Variables|Default|Getbbb) 0.3)
      (Timeline|bbb PlayFromStart
        (:Update
          (bind _percentage (CallFunction|GetTimelinePercentage (Variables|Default|Getbbb)))
          (Transformation|SetRelativeScale3D (Variables|Default|GetAtomAnimationAnchor) (+ "0.700000,0.700000,0.700000" (* "0.500000,0.500000,0.500000" (Math|Curves|GetFloatValue (Variables|Default|GetCRV_Bounce) _percentage)))))))))

(event EventEndPlay
  (params (EndPlayReason :type EEndPlayReason%20Enum :default "Destroyed"))
  ;[0 0 0] EndPlay
  (for _index (range 1 (Variables|Default|GetISM_EthBase))
    (Class|InstancedStaticMeshComponent|RemoveInstance (Variables|/Game/Gameplay/Roads/Blueprints/BP_ISMBank.BP_ISMBank_C|GetISM_EthBase (Variables|Default|GetBP_ISMBank_REF)))))

(fn ConstructionScript)

(fn SaveEth
  (bind _returnvalue (Game|GetGameInstance))
  (bind _asbp_game_instance (Utilities|Casting|CastToBP_GameInstance _returnvalue))
  (bind _saveref (Variables|/Game/Base/Blueprints/BP_GameInstance.BP_GameInstance_C|GetSaveREF _asbp_game_instance))
  (Variables|/Game/Base/Blueprints/BP_Save.BP_Save_C|SetSAVE_Money _saveref (+ (Variables|/Game/Base/Blueprints/BP_Save.BP_Save_C|GetSAVE_Money _saveref) (select (Variables|Default|GetImABunchOfCOllectible) 10 1)))
  (Default|JustSave _asbp_game_instance))