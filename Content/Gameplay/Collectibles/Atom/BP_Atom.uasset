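; BP_Atom is an atom collectible actor, animated with a constant spin.
; On BeginPlay it checks the tutorial flag in BP_GameInstance and, if enabled, sets a near-infinite lifespan.
; Each Tick applies a frame-rate-independent local yaw rotation to three scene components.
; The graph holds no pickup logic, as the overlap event is an unused stub.
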(event EventBeginPlay
  ;[1 1 1] Si tuto, alors lifespan quasi infini
  (bind _asbp_game_instance (Utilities|Casting|CastToBP_GameInstance (Game|GetGameInstance)))
  (if (Variables|/Game/Base/Blueprints/BP_GameInstance.BP_GameInstance_C|GetTutoEnable _asbp_game_instance)
    (Actor|SetLifeSpan 99999.0)))

(event EventActorBeginOverlap
  (params (OtherActor :type Actor%20Object%20Reference)))

(event EventTick
  (params (DeltaSeconds :type Float%20%28single-precision%29))
  (Transformation|AddLocalRotation (Variables|Default|GetScene2) (Math|Rotator|MakeRotator 0.0 0.0 (* DeltaSeconds 5e+02)) false false))

(fn ConstructionScript)